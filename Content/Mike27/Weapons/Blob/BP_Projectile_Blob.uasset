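; Blob projectile that sticks to the first surface it hits and exposes itself as an active disabler with its collision and attached component.
; On impact it stops projectile movement, snaps its sphere onto the hit surface and pins it there with a physics constraint while simulating physics.
; A safety timer destroys it after launch, replaced on attach by an optional one-time timed lifespan.
; Construction tints its point light from the material's emissive color.
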(event OnProjectileCollision(BP_ProjectileComponent)
  (params (Inpact :type Hit%20Result%20Structure))
  (Utilities|IsValid (Variables|Config|GetAttachedComponent)
    (:Is%20Not%20Valid
      (if (!= self (.hitactor Inpact))
        (Config|AttachtoComponentSurface (.hitcomponent Inpact) (.impactpoint Inpact) (.impactnormal Inpact) "Death")))))

(event Custom|Death
  (Utilities|Time|ClearandInvalidateTimerbyHandle (Variables|Config|GetDeathTimerHandle))
  (if (not (Game|IsActorBeingDestroyed))
    (Actor|DestroyActor)))

(event EventBeginPlay
  ;[1 1 1] Resetter after life duration
  (|CallParentFunction)
  (if (not (Class|KismetSystemLibrary|TimerExistsHandle (Variables|Config|GetDeathTimerHandle)))
    (bind _returnvalue (Utilities|Time|SetTimerbyEvent (delegate Custom|Death) (Variables|Config|GetSecurityLifeDuration)))
    (Variables|Config|SetDeathTimerHandle _returnvalue)))

(event EventEndPlay
  (params (EndPlayReason :type EEndPlayReason%20Enum :default "Destroyed"))
  (Utilities|Time|ClearandInvalidateTimerbyHandle (Variables|Config|GetDeathTimerHandle)))

(fn ConstructionScript
  (bind _returnvalue (Rendering|Material|CreateDynamicMaterialInstance (Variables|Default|GetStaticMesh) 0 (Variables|Config|GetMaterialSet) "None" :!class /Script/Engine.PrimitiveComponent))
  (bind _returnvalue_2 (Rendering|Material|GetVectorParameterValue _returnvalue "Emissive" :!class /Script/Engine.MaterialInstanceDynamic))
  (Rendering|Components|Light|SetLightColor (Variables|Config|GetPointLight) _returnvalue_2 true))

(fn AttachtoComponentSurface
  (params (OtherComp :type Primitive%20Component%20Object%20Reference%20%28by%20ref%29) (ImpactPoint :type Vector) (HitNormal :type Vector) (FunctionName :type String))
  (bind _bp_projectilecomponent (Variables|Default|GetBP_ProjectileComponent))
  (Utilities|Time|ClearandInvalidateTimerbyHandle (Variables|Config|GetDeathTimerHandle))
  (bind _output_get (Variables|Config|SetAttachedComponent OtherComp))
  (Variables|/Game/Mike27/Core/Behaviours/BP_ProjectileComponent.BP_ProjectileComponent_C|SetbDisableNoise (Variables|Default|GetBP_ProjectileComponent) true)
  (Components|Activation|Deactivate (Variables|Default|GetProjectileMovement))
  (Physics|SetPhysicsLinearVelocity _bp_projectilecomponent "0, 0, 0" false "None")
  (Transformation|SetWorldLocation _bp_projectilecomponent (+ (.OutPointOnBody (Collision|GetClosestPointonCollision _output_get ImpactPoint "None")) (* HitNormal (Components|Sphere|GetScaledSphereRadius (Variables|Default|GetBP_ProjectileComponent)))) false true)
  (Physics|SetSimulatePhysics (Variables|Default|GetBP_ProjectileComponent) true)
  (Class|PhysicsConstraintComponent|SetConstrainedComponents (Variables|Config|GetPhysicsConstraint) (Variables|Config|GetAttachedComponent) "None" (Variables|Default|GetBP_ProjectileComponent) "None")
  (if (and (Variables|Config|GetbFirstTime) (Variables|Config|GetbUseTimedAttachDuration))
    (Variables|Config|SetbFirstTime (not (Variables|Config|GetbFirstTime)))
    (Utilities|Time|ClearandInvalidateTimerbyHandle (Variables|Config|GetDeathTimerHandle))
    (bind _returnvalue (Utilities|Time|SetTimerbyFunctionName self FunctionName (Variables|Config|GetLifeDuration)))
    (Variables|Config|SetDeathTimerHandle _returnvalue)
    (return)
    (else
      (return))))

(fn GetAttachedComponent
  (return (Variables|Config|GetAttachedComponent)))

(fn GetDisablerInfo
  (return (Variables|Default|GetBP_ProjectileComponent) (Config|GetAttachedComponent) true))
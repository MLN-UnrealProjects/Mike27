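; Grappling hook projectile that flies at a configured speed, carries the end of a cable and sticks to what it hits.
; On impact it disables collision and attaches to the hit component, keeping its world transform.
; A lifetime timer, or a Tick check on distance from the cable's origin, halts its flight.
; SetCable moves the cable end onto the hook, and EndPlay clears it and detaches the actor.
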(event Custom|StopProjectile
  (Utilities|Time|ClearandInvalidateTimerbyHandle (Variables|Config|GetLifeTimerHandle))
  (Game|Components|ProjectileMovement|StopSimulating (Variables|Default|GetProjectileMovement) (Collision|MakeHitResult false false 0.0 0.0 "0, 0, 0" "0, 0, 0" "0,0,1" "0,0,1" 0 0))
  (Actor|Tick|SetActorTickEnabled false))

(event Custom|OnStopped
  (params (Impact :type Hit%20Result%20Structure))
  (bind (_bblockinghit _binitialoverlap _time _distance _location _impactpoint _normal _impactnormal _physmat _hitactor _hitcomponent) (Collision|BreakHitResult Impact))
  (if (!= self _hitactor)
    (Utilities|IsValid _hitcomponent
      (:Is%20Valid
        (Collision|SetCollisionEnabled (Variables|Default|GetBP_ProjectileComponent) "NoCollision")
        (CallFunction|ReleaseConstrainedBody)
        (Transformation|AttachComponentToComponent _hitcomponent "None" "KeepWorld" "KeepWorld" "KeepWorld" false)))))

(event Custom|ReleaseConstrainedBody
  (Transformation|DetachFromActor "KeepWorld" "KeepWorld" "KeepWorld"))

(event EventBeginPlay
  (EventDispatchers|AssignOnProjectileStopped (delegate Custom|OnStopped))
  (|CallParentFunction)
  (Utilities|Time|ClearandInvalidateTimerbyHandle (Variables|Config|GetLifeTimerHandle))
  (bind _returnvalue (Utilities|Time|SetTimerbyEvent (delegate Custom|StopProjectile) (Variables|Config|GetMaxLifeTime)))
  (Variables|Config|SetLifeTimerHandle _returnvalue))

(event Collision|EventActorBeginOverlap
  (params (OtherActor :type Actor%20Object%20Reference))
  (|CallParentFunction OtherActor) ; This node is disabled and will not be called.\nDrag off pins to build functionality.
)

(event EventEndPlay
  (params (EndPlayReason :type EEndPlayReason%20Enum :default "Destroyed"))
  (Config|SetCable)
  (CallFunction|ReleaseConstrainedBody))

(event EventTick
  (params (DeltaSeconds :type Float%20%28single-precision%29))
  (bind _cable (Variables|Config|GetCable))
  (|CallParentFunction DeltaSeconds)
  (Utilities|IsValid _cable
    (:Is%20Valid
      (if (> (Math|Vector|VectorLength (- (Transformation|GetWorldLocation _cable) (Transformation|GetActorLocation))) (Variables|Config|GetMaxDistance))
        (CallFunction|StopProjectile)))))

(fn ConstructionScript
  (|CallParentFunction)
  (Variables|/Script/Engine.ProjectileMovementComponent|SetInitialSpeed (Variables|Default|GetProjectileMovement) (Variables|Config|GetHookSpeed)))

(fn OnProjStopped
  (params (Impact :type Hit%20Result%20Structure%20%28by%20ref%29))
  (|CallParentFunction Impact)
  (Utilities|Time|ClearandInvalidateTimerbyHandle (Variables|Config|GetLifeTimerHandle))
  (return))

(fn SetCable
  (params (Cable :type Cable%20Component%20Object%20Reference))
  (Utilities|IsValid (Variables|Config|GetCable)
    (:Is%20Valid
      (Class|CableComponent|SetAttachEndto (Variables|Config|GetCable) 0 "None" "None"))
    (:Is%20Not%20Valid
      _))
  (bind _output_get (Variables|Config|SetCable Cable))
  (Utilities|IsValid _output_get
    (:Is%20Valid
      (Class|CableComponent|SetAttachEndto _output_get self "None" "None")
      (Variables|/Script/CableComponent.CableComponent|SetEndLocation _output_get "0, 0, 0"))
    (:Is%20Not%20Valid
      _))
  (return))

(fn GetCable
  (return (Variables|Config|GetCable)))
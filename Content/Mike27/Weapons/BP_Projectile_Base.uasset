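; Base projectile Blueprint that handles impacts through its ProjectileMovement and BPProjectileComponent.
; With native collision events, component collisions stop movement and fire the stop notifications, while movement stops optionally call the component's Hit.
; Otherwise, movement stops fire those notifications and always call Hit.
; OnProjStopped is an empty hook alongside the OnProjectileStopped dispatch, and SetNoiseTag sets the component's Tag.
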(event OnProjectileStop(ProjectileMovement)
  (params (ImpactResult :type Hit%20Result%20Structure%20%28by%20ref%29))
  (bind _bp_projectilecomponent (Variables|Config|GetBP_ProjectileComponent))
  (if (Variables|/Game/Mike27/Core/Behaviours/BP_ProjectileComponent.BP_ProjectileComponent_C|GetbUseNativeCollisionEvents _bp_projectilecomponent)
    (if (Variables|Config|GetbCallHitWithNativeCollEnabled)
      (Default|Hit _bp_projectilecomponent ImpactResult :!label _label))
    (else
      (Config|OnProjStopped ImpactResult)
      (Default|CallOnProjectileStopped ImpactResult)
      (goto _label))))

(event OnProjectileCollision(BP_ProjectileComponent)
  (params (Inpact :type Hit%20Result%20Structure))
  (bind _projectilemovement (Variables|Config|GetProjectileMovement))
  (if (Variables|/Game/Mike27/Core/Behaviours/BP_ProjectileComponent.BP_ProjectileComponent_C|GetbUseNativeCollisionEvents (Variables|Config|GetBP_ProjectileComponent))
    (if (Utilities|IsValid (Variables|/Script/Engine.MovementComponent|GetUpdatedComponent _projectilemovement))
      (Game|Components|ProjectileMovement|StopSimulating _projectilemovement Inpact))
    (Config|OnProjStopped Inpact)
    (Default|CallOnProjectileStopped Inpact)))

(fn ConstructionScript)

(fn SetNoiseTag
  (params (Tag :type Name :default "None"))
  (Variables|/Game/Mike27/Core/Behaviours/BP_ProjectileComponent.BP_ProjectileComponent_C|SetTag (Variables|Config|GetBP_ProjectileComponent) Tag)
  (return))

(fn OnProjStopped
  (params (Impact :type Hit%20Result%20Structure%20%28by%20ref%29))
  (return))
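; Spawned electric arc effect that runs from the actor to a destination and destroys itself when finished.
; Spawn reads an arc struct, then builds a spline mesh with a dynamic noise material, attached sound, colored point light and impact particles.
; A Countdown timeline at randomized play rate animates opacity, rise and dissipation, flickers the light and cuts light and particles on an event.
; Gated Tick can update moving endpoints.
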(event Custom|Spawn
  (params (ArcStruct :type F%20Arc%20Values%20Structure))
  (Config|ArcStructExtraction ArcStruct)
  (Config|SetArcLifetime)
  (Config|SetSpline)
  (Config|SetAudio)
  (Config|SetLight)
  (Config|SetParticles)
  (SplineMesh|SetStartandEnd (Variables|Default|GetSpline) "0, 0, 0" "0, 0,1.000000" (Variables|Default|GetLocalDestination) "0, 0,1.000000" true :!class /Script/Engine.SplineMeshComponent)
  (Rendering|Material|SetVectorParameterValue (Variables|Default|GetArcMat) "BiasVector" (Math|Conversions|ToLinearColor(Vector) (* "0, 0,1.000000" 0.5)) :!class /Script/Engine.MaterialInstanceDynamic)
  (|HandlerFinishArcs))

(fn ConstructionScript)

(fn ArcStructExtraction
  (params (ArcValues :type F%20Arc%20Values%20Structure))
  (bind (_boltcolor _dest _noisescale _noisespeed) (Utilities|Struct|BreakFArcValues ArcValues))
  (Utilities|FlowControl|Sequence
    (:then_0
      (Variables|Default|SetNewColor _boltcolor))
    (:then_1
      (Variables|Default|SetLocalDestination _dest))
    (:then_2
      (Variables|Default|SetArc%20Noise _noisescale))
    (:then_3
      (Variables|Default|SetNoise%20Speed _noisespeed))
    (:then_4
      (return))))

(fn SetArcLifetime
  (Components|Timeline|SetPlayRate (Variables|Default|GetCountdown) (Math|Float|SelectFloat 2.0 (Math|Random|RandomFloatinRange 3.0 6.0) (> (Math|Random|RandomFloatinRange 0.0 1.0) 0.9))) ; This will increase the play speed for the effect if its a branch.
  (return))

(fn SetSpline
  (bind _returnvalue (AddComponent|AddSplineMeshComponent false))
  (Variables|Default|SetSpline _returnvalue)
  (bind _returnvalue_2 (Rendering|Material|CreateDynamicMaterialInstance _returnvalue 0 0 "None" :!class /Script/Engine.PrimitiveComponent))
  (bind _output_get (Variables|Default|SetArcMat _returnvalue_2))
  (Rendering|Material|SetVectorParameterValue _output_get "RandomOffset" (Utilities|RandomColor) :!class /Script/Engine.MaterialInstanceDynamic)
  (Rendering|Material|SetVectorParameterValue _output_get "Color" (Variables|Default|GetNewColor) :!class /Script/Engine.MaterialInstanceDynamic)
  (Rendering|Material|SetScalarParameterValue (Variables|Default|GetArcMat) "Scale" (Variables|Default|GetArc%20Noise) :!class /Script/Engine.MaterialInstanceDynamic)
  (Rendering|Material|SetScalarParameterValue (Variables|Default|GetArcMat) "Speed" (Variables|Default|GetNoise%20Speed) :!class /Script/Engine.MaterialInstanceDynamic))

(fn SetAudio
  (Audio|SpawnSoundAttached (Variables|Default|GetArc%20Sounds) (Variables|Default|GetSpline) "None" "0, 0, 0" "0, 0, 0" "KeepRelativeOffset" true (Math|Random|RandomFloatinRange 0.5 0.9) 1.0 (Math|Random|RandomFloatinRange 0.0 25.0) 0 0)
  (return))

(fn SetLight
  (bind _returnvalue (AddComponent|AddPointLightComponent false (Math|Conversions|ToTransform(Vector) "0, 0, 0")))
  (bind _output_get (Variables|Default|SetArcLight _returnvalue))
  (Rendering|Components|Light|SetLightColor _output_get (Variables|Default|GetNewColor) true)
  (return))

(fn SetParticles
  (bind _arc_impact_end (Variables|Default|GetArc%20Impact%20End))
  (bind _newcolor (Variables|Default|GetNewColor))
  (bind (_r _g _b _a) (Math|Color|BreakColor _newcolor))
  (Transformation|SetWorldTransform (Variables|Default|GetArc%20Impact%20End) (Math|Transform|MakeTransform (+ "0, 0, 0" (Transformation|GetActorLocation)) (Math|Rotator|MakeRotfromX (Variables|Default|GetLocalDestination))) false false)
  (Effects|Components|ParticleSystem|SetVectorParameter _arc_impact_end "Color" (* (Math|Vector|MakeVector _r _g _b) _a))
  (Components|Activation|Activate _arc_impact_end false)
  (return))

(event Custom|SetMoving
  (bind _spline (Variables|Default|GetSpline))
  (Utilities|FlowControl|Gate true) ; enters at Open
)

(event Custom|StopMoving
  (bind _spline (Variables|Default|GetSpline))
  (Utilities|FlowControl|Gate true) ; enters at Close
)

(event EventTick
  (params (DeltaSeconds :type Float%20%28single-precision%29))
  (bind _spline (Variables|Default|GetSpline))
  (if (Variables|Default|GetbAllowAnyTick)
    (if (Variables|Default|GetbTimeToDie)
      (Variables|Default|SetbAllowAnyTick false)
      (Utilities|FlowControl|Delay 0.5)
      (Actor|DestroyActor)
      (elif (not (Variables|Default|GetCustomPos))
        (Utilities|FlowControl|Gate true
          (:Exit
            (SplineMesh|SetStartandEnd _spline (- (Transformation|GetActorLocation) (Transformation|GetWorldLocation _spline)) "0, 0, 0" (.EndPos (|Inputs)) "0, 0,1.000000" true :!class /Script/Engine.SplineMeshComponent)))))))
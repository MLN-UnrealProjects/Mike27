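; BP_DoorTrigger is a placeable trigger that checks whether the player has picked up an object before reporting a door as open.
; On overlap with its collision component, it reads the PickedObject flag from BP_PlayerController via BP_TruePlayer.
; When set, it clears the flag and removes top-level WBP_MainObject widgets; otherwise it prints a refusal.
; The door result is only printed text, with no door movement here.
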(event OnComponentBeginOverlap(CollisionComponent)
  (params (OverlappedComponent :type Primitive%20Component%20Object%20Reference) (OtherActor :type Actor%20Object%20Reference) (OtherComp :type Primitive%20Component%20Object%20Reference) (OtherBodyIndex :type Integer) (bFromSweep :type Boolean) (SweepResult :type Hit%20Result%20Structure%20%28by%20ref%29))
  (bind _asbp_true_player (Utilities|Casting|CastToBP_TruePlayer OtherActor))
  (bind _asbp_player_controller (Utilities|Casting|CastToBP_PlayerController (Pawn|GetController _asbp_true_player)))
  (if (Variables|/Game/Mike27/Characters/Player/BP_PlayerController.BP_PlayerController_C|GetbPickedObject _asbp_player_controller)
    (CallFunction|CustomPrintString "The door is open now" true true "(R=0.000000,G=0.000000,B=1.000000,A=1.000000)" 2.0)
    (Variables|/Game/Mike27/Characters/Player/BP_PlayerController.BP_PlayerController_C|SetbPickedObject _asbp_player_controller false)
    (bind _foundwidgets (Widget|GetAllWidgetsOfClass "/Game/Mike27/UI/WBP_MainObject.WBP_MainObject_C" true))
    (Widget|RemovefromParent _foundwidgets)
    (CallFunction|CustomPrintString "Picked object is false" true true "(R=0.000000,G=0.000000,B=1.000000,A=1.000000)" 2.0)
    (else
      (CallFunction|CustomPrintString "You can't open the door" true true "(R=0.000000,G=0.000000,B=1.000000,A=1.000000)" 2.0))))

(event EventBeginPlay)

(event Collision|EventActorBeginOverlap
  (params (OtherActor :type Actor%20Object%20Reference)))

(event EventTick
  (params (DeltaSeconds :type Float%20%28single-precision%29)))

(fn ConstructionScript)
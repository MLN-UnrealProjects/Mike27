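; Player start placeable that creates a checkpoint at its own location when play begins.
; On BeginPlay it spawns a BP_Checkpoint at the actor's transform and sets that transform as the checkpoint's spawn point.
; It then registers the checkpoint with its CheckpointContainer, falling back to the first BP_Checkpoint_Container found in the level if the reference is not valid.
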(event EventBeginPlay
  (bind _returnvalue (Transformation|GetActorTransform))
  (bind _returnvalue_2 (Game|SpawnActorfromClass "/Game/Mike27/Placeables/BP_Checkpoint.BP_Checkpoint_C" _returnvalue "Undefined" 0 0))
  (bind _output_get (Variables|Config|SetCheckpointSpawned _returnvalue_2))
  (Default|SetSpawnPoint _output_get _returnvalue)
  (Utilities|IsValid (Variables|Config|GetCheckpointContainer)
    (:Is%20Valid
      (Default|AddCheckpoint (Variables|Config|GetCheckpointContainer) _output_get))
    (:Is%20Not%20Valid
      (bind _outactors (Actor|GetAllActorsOfClass "/Game/Mike27/Placeables/BP_Checkpoint_Container.BP_Checkpoint_Container_C"))
      (if (> (Utilities|Array|Length _outactors) 0)
        (bind _output_get_2 (Variables|Config|SetCheckpointContainer (Utilities|Array|Get(acopy) _outactors)))
        (Default|AddCheckpoint _output_get_2 (Variables|Config|GetCheckpointSpawned))))))

(fn ConstructionScript
  (|CallParentFunction))
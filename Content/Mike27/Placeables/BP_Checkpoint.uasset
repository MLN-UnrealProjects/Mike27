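; BP_Checkpoint is a placeable checkpoint actor that acts as a thin wrapper around its checkpoint component, which holds the state and spawn point.
; On BeginPlay it runs the parent logic, then, if a custom spawn point is enabled, passes the SpawnLocation world transform to that component.
; IsCollected and SetSpawnPoint expose the component's state check and spawn-point setter on the actor.
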(event EventBeginPlay
  (|CallParentFunction)
  (if (Variables|Config|GetbUseCustomSpawnPoint)
    (Config|SetSpawnPoint (Transformation|GetWorldTransform (Variables|Config|GetSpawnLocation)))))

(fn ConstructionScript)

(fn IsCollected
  (return (Utilities|Enum|Equal(Enum) (Default|GetCheckpointState (Variables|Config|GetBP_CheckpointComponent)) "NewEnumerator1")))

(fn SetSpawnPoint
  (params (WorldSpawnPoint :type Transform))
  (Default|SetSpawnPoint (Variables|Config|GetBP_CheckpointComponent) WorldSpawnPoint)
  (return))
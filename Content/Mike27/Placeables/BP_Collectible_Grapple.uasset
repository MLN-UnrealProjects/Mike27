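; BP_Collectible_Grapple is a collectible placeable that unlocks the grapple ability for the player.
; It extends a parent collectible, calling the parent logic first in each event.
; Both OnCollected and OnLoaded set GrappleActive on the current Mike character, so the ability is granted on pickup and on load.
; If no valid character exists, both events print an error message instead.
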(event EventBeginPlay
  (|CallParentFunction))

(event EventOnLoaded
  (bind _asbp_player_character (CallFunction|GetCurrentMikeCharacter))
  (|CallParentFunction)
  (Utilities|IsValid _asbp_player_character
    (:Is%20Valid
      (Variables|/Game/Mike27/Core/Characters/Player/BP_PlayerCharacter.BP_PlayerCharacter_C|SetbGrappleActive _asbp_player_character true))
    (:Is%20Not%20Valid
      (CallFunction|CustomPrintString "Player instance could not be found!" true true "(R=0.000000,G=0.000000,B=1.000000,A=1.000000)" 2.0))))

(event EventOnCollected
  (bind _asbp_player_character (CallFunction|GetCurrentMikeCharacter))
  (|CallParentFunction)
  (Utilities|IsValid _asbp_player_character
    (:Is%20Valid
      (Variables|/Game/Mike27/Core/Characters/Player/BP_PlayerCharacter.BP_PlayerCharacter_C|SetbGrappleActive _asbp_player_character true))
    (:Is%20Not%20Valid
      (CallFunction|CustomPrintString "Player instance could not be found!" true true "(R=0.000000,G=0.000000,B=1.000000,A=1.000000)" 2.0))))

(fn ConstructionScript
  (|CallParentFunction))
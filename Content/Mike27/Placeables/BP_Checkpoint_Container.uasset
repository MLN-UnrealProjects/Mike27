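; Placeable checkpoint container that keeps a list of checkpoints and tracks which one is current.
; On BeginPlay it either finds every BP_Checkpoint in the level or uses its existing list, then binds to each checkpoint component's collected event.
; Collected checkpoints become current, and a change fires OnNewCheckpointCollected, which also drives a debug print.
; It also supports adding, removing and releasing checkpoints, and unbinds on EndPlay.
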(event Custom|DEBUG_OnCheckpointCollected
  (params (NewCheckpoint :type BP%20Checkpoint%20Component%20Object%20Reference))
  (CallFunction|CustomPrintString (Utilities|String|Append "New current checkpoint: " (Utilities|GetDisplayName (Components|GetOwner NewCheckpoint))) true true "(R=0.000000,G=0.000000,B=1.000000,A=1.000000)" 2.0))

(event Custom|ReleaseAllCheckpoints
  (for _array_element (Variables|Config|GetCheckpoints)
    (Default|ReleaseCheckpoint (Variables|/Game/Mike27/Placeables/BP_Checkpoint.BP_Checkpoint_C|GetBP_CheckpointComponent _array_element))))

(event Custom|OnCheckpointCollected
  (params (Checkpoint :type BP%20Checkpoint%20Component%20Object%20Reference))
  (Config|SetCurrentCheckpoint Checkpoint))

(event Custom|UnbindCheckpoints
  (for _array_element (Variables|Config|GetCheckpoints)
    (EventDispatchers|UnbindEventfromOnCheckpointCollected (Variables|/Game/Mike27/Placeables/BP_Checkpoint.BP_Checkpoint_C|GetBP_CheckpointComponent _array_element) (delegate Custom|OnCheckpointCollected))
    (EventDispatchers|UnbindEventfromOnNewCheckpointCollected (delegate Custom|DEBUG_OnCheckpointCollected))))

(event Custom|BindCheckpoints
  (for _array_element (Variables|Config|GetCheckpoints)
    (EventDispatchers|BindEventtoOnCheckpointCollected (Variables|/Game/Mike27/Placeables/BP_Checkpoint.BP_Checkpoint_C|GetBP_CheckpointComponent _array_element) (delegate Custom|OnCheckpointCollected))
    (EventDispatchers|BindEventtoOnNewCheckpointCollected (delegate Custom|DEBUG_OnCheckpointCollected))))

(event Custom|AddCheckpoint
  (params (Checkpoint :type BP%20Checkpoint%20Object%20Reference))
  (Utilities|Array|AddUnique (Variables|Config|GetCheckpoints) Checkpoint)
  (if (Default|IsCollected Checkpoint)
    (Config|SetCurrentCheckpoint (Variables|/Game/Mike27/Placeables/BP_Checkpoint.BP_Checkpoint_C|GetBP_CheckpointComponent Checkpoint))))

(event Custom|RemoveCheckpoint
  (params (Checkpoint :type BP%20Checkpoint%20Object%20Reference))
  (Utilities|Array|RemoveItem (Variables|Config|GetCheckpoints) Checkpoint))

(event EventBeginPlay
  (if (Variables|Config|GetbFindAllCheckpointsAtStart)
    (Config|FindAllCheckpoints)
    (else
      (CallFunction|BindCheckpoints))))

(event EventEndPlay
  (params (EndPlayReason :type EEndPlayReason%20Enum :default "Destroyed"))
  (CallFunction|UnbindCheckpoints))

(fn ConstructionScript)

(fn GetCurrentCheckpoint
  (return (Variables|Config|GetCurrentCheckpoint)))

(fn FindAllCheckpoints
  (CallFunction|UnbindCheckpoints)
  (Utilities|Array|Clear (Variables|Config|GetCheckpoints))
  (bind _outactors (Actor|GetAllActorsOfClass "/Game/Mike27/Placeables/BP_Checkpoint.BP_Checkpoint_C"))
  (bind _output_get (Variables|Config|SetCheckpoints _outactors))
  (CallFunction|BindCheckpoints)
  (for _array_element _output_get
    (switch Utilities|FlowControl|Switch|SwitchonECheckpointStatus (Default|GetCheckpointState (Variables|/Game/Mike27/Placeables/BP_Checkpoint.BP_Checkpoint_C|GetBP_CheckpointComponent _array_element))
      (:NewEnumerator0
        (Default|CallOnCheckpointsFindOver :!label _label)
        (return))
      (:NewEnumerator1
        (Config|SetCurrentCheckpoint (Variables|/Game/Mike27/Placeables/BP_Checkpoint.BP_Checkpoint_C|GetBP_CheckpointComponent _array_element)))
      (:NewEnumerator2
        (goto _label))))
  (Default|CallOnCheckpointsFindOver)
  (return))

(fn SetCurrentCheckpoint
  (params (Newcheckpoint :type BP%20Checkpoint%20Component%20Object%20Reference))
  (if (not (== Newcheckpoint (Variables|Config|GetCurrentCheckpoint)))
    (Default|CallOnNewCheckpointCollected Newcheckpoint)
    (Variables|Config|SetCurrentCheckpoint Newcheckpoint)))
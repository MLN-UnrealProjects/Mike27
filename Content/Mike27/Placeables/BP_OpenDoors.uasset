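; BP_OpenDoors is a pickup that opens small doors when the player character overlaps its sphere.
; On overlap it sets PickedObject on the player controller, plays a collection sound, shows the WBP_MainObject widget and destroys itself.
; It then calls Open on the first two BP_Door_Small actors returned by GetAllActorsOfClass, so the doors are chosen by array index rather than by direct reference.
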(event OnComponentBeginOverlap(Sphere)
  (params (OverlappedComponent :type Primitive%20Component%20Object%20Reference) (OtherActor :type Actor%20Object%20Reference) (OtherComp :type Primitive%20Component%20Object%20Reference) (OtherBodyIndex :type Integer) (bFromSweep :type Boolean) (SweepResult :type Hit%20Result%20Structure%20%28by%20ref%29))
  (bind _asbp_player_character (Utilities|Casting|CastToBP_PlayerCharacter OtherActor))
  (bind _asbp_player_controller (Utilities|Casting|CastToBP_PlayerController (Pawn|GetController _asbp_player_character)))
  (Variables|/Game/Mike27/Characters/Player/BP_PlayerController.BP_PlayerController_C|SetbPickedObject _asbp_player_controller true)
  (CallFunction|CustomPrintString "Picked object is true" true true "(R=0.000000,G=0.000000,B=1.000000,A=1.000000)" 2.0)
  ;[1 1 1] Eventually add a sound
  (Audio|PlaySoundatLocation (Variables|Config|GetCollectedSound) (Transformation|GetActorLocation) "0, 0, 0" 1.0 1.0 0.0 0 0 0)
  (bind _returnvalue (UserInterface|CreateWidget "/Game/Mike27/UI/WBP_MainObject.WBP_MainObject_C" _asbp_player_controller))
  (UserInterface|Viewport|AddtoViewport _returnvalue 0)
  (Actor|DestroyActor)
  (bind _outactors (Actor|GetAllActorsOfClass "/Game/Blueprints/BP_Door_Small.BP_Door_Small_C"))
  (bind _asbp_door_small (Utilities|Casting|CastToBP_Door_Small (Utilities|Array|Get(acopy) _outactors)))
  (Default|Open _asbp_door_small)
  (bind _outactors_2 (Actor|GetAllActorsOfClass "/Game/Blueprints/BP_Door_Small.BP_Door_Small_C"))
  (bind _asbp_door_small_2 (Utilities|Casting|CastToBP_Door_Small (Utilities|Array|Get(acopy) _outactors_2 1)))
  (Default|Open _asbp_door_small_2))

(event EventBeginPlay)

(event Collision|EventActorBeginOverlap
  (params (OtherActor :type Actor%20Object%20Reference)))

(event EventTick
  (params (DeltaSeconds :type Float%20%28single-precision%29)))

(fn ConstructionScript)
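; BP_PlayerStart_Gadgets is a placeable, apparently a player start, that sets which gadgets the Mike character has active in a level.
; On BeginPlay it copies its grapple and blob flags onto the current Mike character.
; If the character does not exist yet, it enables Tick and retries each frame, printing a warning until it applies the flags, then disables ticking.
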(event EventTick
  (params (DeltaSeconds :type Float%20%28single-precision%29))
  (bind _asbp_player_character (CallFunction|GetCurrentMikeCharacter))
  (|CallParentFunction DeltaSeconds)
  (Utilities|IsValid _asbp_player_character
    (:Is%20Valid
      (Variables|/Game/Mike27/Core/Characters/Player/BP_PlayerCharacter.BP_PlayerCharacter_C|SetbGrappleActive _asbp_player_character (Variables|Config|GetbIsGrappleActive))
      (Variables|/Game/Mike27/Core/Characters/Player/BP_PlayerCharacter.BP_PlayerCharacter_C|SetbBlobActive _asbp_player_character (Variables|Config|GetbIsBlobActive))
      (Actor|Tick|SetActorTickEnabled false))
    (:Is%20Not%20Valid
      (CallFunction|CustomPrintString "Player characther not found!" true true "(R=0.000000,G=0.000000,B=1.000000,A=1.000000)" 2.0))))

(event EventBeginPlay
  (bind _asbp_player_character (CallFunction|GetCurrentMikeCharacter))
  (|CallParentFunction)
  (Utilities|IsValid _asbp_player_character
    (:Is%20Valid
      (Variables|/Game/Mike27/Core/Characters/Player/BP_PlayerCharacter.BP_PlayerCharacter_C|SetbGrappleActive _asbp_player_character (Variables|Config|GetbIsGrappleActive))
      (Variables|/Game/Mike27/Core/Characters/Player/BP_PlayerCharacter.BP_PlayerCharacter_C|SetbBlobActive _asbp_player_character (Variables|Config|GetbIsBlobActive)))
    (:Is%20Not%20Valid
      (Actor|Tick|SetActorTickEnabled true))))

(fn ConstructionScript
  (|CallParentFunction))
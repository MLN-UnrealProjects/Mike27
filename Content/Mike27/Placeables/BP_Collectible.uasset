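; Base collectible placeable that is picked up when something overlaps its Cube component.
; If ShouldBeSaved is set, it passes itself to BP_Gamemode_Mike_Base's SaveCollectibles, otherwise it calls OnCollected, then destroys itself.
; A failed gamemode cast only prints an error and leaves the actor in place.
; The construction script defaults an empty Name to the object name, and OnLoaded and OnCollected are empty functions.
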(event OnComponentBeginOverlap(Cube)
  (params (OverlappedComponent :type Primitive%20Component%20Object%20Reference) (OtherActor :type Actor%20Object%20Reference) (OtherComp :type Primitive%20Component%20Object%20Reference) (OtherBodyIndex :type Integer) (bFromSweep :type Boolean) (SweepResult :type Hit%20Result%20Structure%20%28by%20ref%29))
  (if (Variables|Config|GetbShouldBeSaved)
    (bind _asbp_gamemode_mike_base (Utilities|Casting|CastToBP_Gamemode_Mike_Base (Game|GetGameMode))
      (:then
        (Default|SaveCollectibles _asbp_gamemode_mike_base self)
        (if (not (Game|IsActorBeingDestroyed)) :!label _label
          (Actor|DestroyActor)))
      (:CastFailed
        (CallFunction|CustomPrintString "Not valid gamemode type" true true "(R=0.000000,G=0.000000,B=1.000000,A=1.000000)" 2.0)))
    (else
      (Config|OnCollected)
      (goto _label))))

(fn ConstructionScript
  (if (>= 0 (Utilities|String|Len (Variables|Config|GetName)))
    (Variables|Config|SetName (Utilities|GetObjectName self))))

(fn OnLoaded
  (return))

(fn OnCollected
  (return))
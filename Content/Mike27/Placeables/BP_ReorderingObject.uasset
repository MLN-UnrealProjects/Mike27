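; BP_ReorderingObject is a placeable that shows particle effects while its Reordering component is moving it to a reorder destination.
; When reordering starts, it activates its own ParticleSystem and spawns a copy at the destination, which follows any destination change.
; On completion, interruption or failure, StopEffects deactivates both and destroys the spawned copy, or its owning actor if one exists.
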(event OnReordered(Reordering)
  (CallFunction|StopEffects))

(event OnReorderDestinationChanged(Reordering)
  (params (OldReorderDestination :type Transform) (NewReorderDestination :type Transform))
  (bind _particleatoriginallocation (Variables|Default|GetParticleAtOriginalLocation))
  (Utilities|IsValid _particleatoriginallocation
    (:Is%20Valid
      (Transformation|SetWorldTransform _particleatoriginallocation NewReorderDestination false true))))

(event OnReorderInterrupted(Reordering)
  (CallFunction|StopEffects))

(event OnReorderFailed(Reordering)
  (CallFunction|StopEffects))

(event OnReordering(Reordering)
  (params (ReorderDestination :type Transform))
  (bind (_location _rotation _scale) (Math|Transform|BreakTransform ReorderDestination))
  (bind _particlesystem (Variables|Default|GetParticleSystem))
  (bind _template (Variables|/Script/Engine.ParticleSystemComponent|GetTemplate _particlesystem))
  (CallFunction|StopEffects)
  (Utilities|IsValid _template
    (:Is%20Valid
      (bind _returnvalue (Effects|SpawnEmitteratLocation _template _location _rotation _scale false))
      (bind _output_get (Variables|Default|SetParticleAtOriginalLocation _returnvalue))
      (Components|Activation|SetActive _output_get true false))
    (:Is%20Not%20Valid
      _))
  (Components|Activation|SetActive (Variables|Default|GetParticleSystem) true false))

(event Custom|StopEffects
  (Utilities|IsValid (Variables|Default|GetParticleAtOriginalLocation)
    (:Is%20Valid
      (Components|Activation|SetActive (Variables|Default|GetParticleAtOriginalLocation) false true)
      (Utilities|IsValid (Components|GetOwner (Variables|Default|GetParticleAtOriginalLocation))
        (:Is%20Valid
          (Actor|DestroyActor (Components|GetOwner (Variables|Default|GetParticleAtOriginalLocation))))
        (:Is%20Not%20Valid
          (Components|DestroyComponent (Variables|Default|GetParticleAtOriginalLocation)))))
    (:Is%20Not%20Valid
      _))
  (Components|Activation|SetActive (Variables|Default|GetParticleSystem) false true)
  (Variables|Default|SetParticleAtOriginalLocation 0))

(fn ConstructionScript)
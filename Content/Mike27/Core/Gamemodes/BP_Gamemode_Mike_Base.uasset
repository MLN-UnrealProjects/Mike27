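; Base game mode that tracks collectibles and persists them through a BP_SaveCollectibles save game.
; On BeginPlay it creates a collectible widget, left off the viewport, loads or creates the save, then destroys placed BP_Collectible actors whose names are already saved.
; SaveCollectibles records new pickups by name and triggers their OnCollected.
; Both paths feed images to the widget and the queryable Collectibles set, though restored entries get an empty name.
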(event EventBeginPlay
  (Utilities|FlowControl|Sequence
    (:then_0
      (bind _returnvalue (UserInterface|CreateWidget "/Game/Mike27/UI/WBP_Collectible.WBP_Collectible_C"))
      ;[1 1 1] connect if need visible collectibles in game
      (bind _output_get (Variables|Config|SetCollectibleWidget _returnvalue)))
    (:then_1
      (Config|LoadCollectibles)
      (Utilities|IsValid (Variables|Config|GetCollectibleSave)
        (:Is%20Valid
          _)
        (:Is%20Not%20Valid
          (bind _returnvalue_2 (SaveGame|CreateSaveGameObject "/Game/Mike27/Core/Engine/BP_SaveCollectibles.BP_SaveCollectibles_C"))
          (bind _output_get_2 (Variables|Config|SetCollectibleSave _returnvalue_2))
          (bind _returnvalue_3 (Default|SetSlotInfo _output_get_2 (Variables|Config|GetCollectablesSaveSlot) (Variables|Config|GetCollectablesUserIndex)))
          (if _returnvalue_3
            _
            (else
              (CallFunction|CustomPrintString "Failed to initialize and save collectables Savegame" true true "(R=0.000000,G=0.000000,B=1.000000,A=1.000000)" 2.0)))))
      (Config|DeleteExistingCollectibles))))

(fn ConstructionScript)

(fn SaveCollectibles
  (params (Collectible :type BP%20Collectible%20Object%20Reference))
  (bind _name (Variables|/Game/Mike27/Placeables/BP_Collectible.BP_Collectible_C|GetName Collectible))
  (bind _returnvalue (Default|Add (Variables|Config|GetCollectibleSave) _name))
  (if _returnvalue
    (Default|OnCollected Collectible)
    (Config|AddCollectibletoUI (Variables|/Game/Mike27/Placeables/BP_Collectible.BP_Collectible_C|GetImage Collectible) _name)
    (else
      (CallFunction|CustomPrintString "Failed to save collected collectable" true true "(R=0.000000,G=0.000000,B=1.000000,A=1.000000)" 2.0)))
  (return))

(fn LoadCollectibles
  (bind _returnvalue (SaveGame|LoadGamefromSlot (Variables|Config|GetCollectablesSaveSlot) (Variables|Config|GetCollectablesUserIndex)))
  (bind _asbp_save_collectibles (Utilities|Casting|CastToBP_SaveCollectibles _returnvalue)
    (:then
      (Variables|Config|SetCollectibleSave _asbp_save_collectibles))
    (:CastFailed
      (CallFunction|CustomPrintString "Invalid collectable save type" true true "(R=0.000000,G=0.000000,B=1.000000,A=1.000000)" 2.0)))
  (return))

(fn DebugResetCollectibles
  (bind _returnvalue (Default|Clear (Variables|Config|GetCollectibleSave)))
  (return _returnvalue))

(fn DeleteExistingCollectibles
  (bind _outactors (Actor|GetAllActorsOfClass "/Game/Mike27/Placeables/BP_Collectible.BP_Collectible_C"))
  (bind _output_get (LocalVariables|SetExistingCollectables _outactors))
  (for _array_element _output_get
    (if (Default|Contains (Variables|Config|GetCollectibleSave) (Variables|/Game/Mike27/Placeables/BP_Collectible.BP_Collectible_C|GetName _array_element))
      (Default|OnLoaded _array_element)
      (Config|AddCollectibletoUI (Variables|/Game/Mike27/Placeables/BP_Collectible.BP_Collectible_C|GetImage _array_element))
      (if (not (Game|IsActorBeingDestroyed _array_element))
        (Actor|DestroyActor _array_element))))
  (return))

(fn AddCollectibletoUI
  (params (Image :type Texture%20Object%20Reference) (Name :type String))
  (Utilities|IsValid Image
    (:Is%20Valid
      (Default|AddCollectible (Variables|Config|GetCollectibleWidget) Image)
      (Config|AddtoCollectibles Name Image))
    (:Is%20Not%20Valid
      _))
  (return))

(fn AddtoCollectibles
  (params (Name :type String) (Image :type Texture%20Object%20Reference))
  (Utilities|Set|Add (Variables|Default|GetCollectibles) (Utilities|Struct|MakeFCollectible Name Image)))

(fn GetAllCollectibles
  (bind _result (Utilities|Set|ToArray (Variables|Default|GetCollectibles)))
  (return _result))
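; Checkpoint component that is collected when an actor with the target tag hits or overlaps it.
; On first collection it snapshots the BP_PlayerCharacter's health, shrink percentage (rounded if growth is binary) and camera depth-of-field method, then broadcasts OnCheckpointCollected.
; ReleaseCheckpoint resets that state on BeginPlay or on demand and broadcasts the release.
; Getters expose the saved values and a spawn point, which defaults to the owner's transform unless overridden.
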(event Custom|ReleaseCheckpoint
  (Variables|Config|SetStatus "NewEnumerator2")
  (Variables|Config|SetShrinkPercentage 0.0)
  (Variables|Config|SetHealth 9.223372036854776e+18)
  (Variables|Config|SetMethod "DOFM_BokehDOF")
  (Default|CallOnCheckpointReleased))

(event Custom|OnHit
  (params (HitComponent :type Primitive%20Component%20Object%20Reference) (OtherActor :type Actor%20Object%20Reference) (OtherComp :type Primitive%20Component%20Object%20Reference) (NormalImpulse :type Vector) (Hit :type Hit%20Result%20Structure%20%28by%20ref%29))
  (Config|OnCollision OtherActor))

(event Custom|OnBeginOverlap
  (params (OverlappedComponent :type Primitive%20Component%20Object%20Reference) (OtherActor :type Actor%20Object%20Reference) (OtherComp :type Primitive%20Component%20Object%20Reference) (OtherBodyIndex :type Integer) (bFromSweep :type Boolean) (SweepResult :type Hit%20Result%20Structure%20%28by%20ref%29))
  (Config|OnCollision OtherActor))

(event EventBeginPlay
  (CallFunction|ReleaseCheckpoint)
  (EventDispatchers|BindEventtoOnComponentHit (delegate Custom|OnHit))
  (EventDispatchers|BindEventtoOnComponentBeginOverlap (delegate Custom|OnBeginOverlap)))

(event EventEndPlay
  (params (EndPlayReason :type EEndPlayReason%20Enum :default "Destroyed"))
  (EventDispatchers|UnbindEventfromOnComponentHit (delegate Custom|OnHit))
  (EventDispatchers|UnbindEventfromOnComponentBeginOverlap (delegate Custom|OnBeginOverlap)))

(fn OnCollision
  (params (CollidedActor :type Actor%20Object%20Reference))
  (if (Actor|ActorHasTag CollidedActor (Variables|Config|GetTargetTag))
    (switch Utilities|FlowControl|Switch|SwitchonECheckpointStatus (Variables|Config|GetStatus)
      (:NewEnumerator0
        _)
      (:NewEnumerator1
        _)
      (:NewEnumerator2
        (Variables|Config|SetStatus "NewEnumerator1")
        (bind _asbp_player_character (Utilities|Casting|CastToBP_PlayerCharacter CollidedActor)
          (:then
            (if (Default|IsGrowingEffectBinary _asbp_player_character)
              (Variables|Config|SetShrinkPercentage (Math|Conversions|ToFloat(Integer) (Math|Float|Round (Default|GetShrinkingPercentage _asbp_player_character))))
              (else
                (Variables|Config|SetShrinkPercentage (Default|GetShrinkingPercentage _asbp_player_character))))
            (Variables|Config|SetHealth (Default|GetCurrentHealth _asbp_player_character))
            ;[1 1 1] Se non viene fatto questo break-make c'è la possibilità che venga portato nel checkpoint anche i valori del material post-process
            (Variables|Config|SetMethod (Utilities|Struct|BreakPostProcessSettings (Variables|/Script/Engine.CameraComponent|GetPostProcessSettings (Variables|/Game/Mike27/Core/Characters/Player/BP_PlayerCharacter.BP_PlayerCharacter_C|GetCamera _asbp_player_character)))))
          (:CastFailed
            (Variables|Config|SetShrinkPercentage 0.0)
            (Variables|Config|SetHealth 8.023796054858138e+18)
            (Variables|Config|SetMethod "DOFM_BokehDOF")))
        (Default|CallOnCheckpointCollected self)
        (return true)))
    (return false)
    (else
      (return false))))

(fn GetCheckpointState
  (return (Variables|Config|GetStatus)))

(fn GetShrinkPercentageatCheckpoint
  (return (Variables|Config|GetShrinkPercentage)))

(fn GetHealthatCheckpoint
  (return (Variables|Config|GetHealth)))

(fn GetSpawnPoint
  (if (Variables|Config|GetbSpawnPointOverride)
    (return (Variables|Config|GetOverrideSpawnPoint))
    (else
      (return (Transformation|GetActorTransform (Components|GetOwner))))))

(fn SetSpawnPoint
  (params (WorldSpawnPoint :type Transform))
  (Variables|Config|SetOverrideSpawnPoint WorldSpawnPoint)
  (Variables|Config|SetbSpawnPointOverride true)
  (return))

(fn GetMethodDOFatCheckpoint
  (return (Variables|Config|GetMethod)))
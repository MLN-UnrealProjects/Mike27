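; Health component that tracks current and maximum health for its owning actor and signals damage, death and revival.
; It binds to the owner's any-damage event, subtracting damage and firing OnDamage only while health stays above zero.
; All changes go through SetCurrentHealth, which clamps the value and fires OnDeath or OnRevive on zero crossings.
; Maximum health can change with current health clamped or its percentage preserved.
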(event Custom|SetMaxHealth
  (params (NewMaxHealth :type Float%20%28single-precision%29))
  (Variables|Config|SetMaxHealth NewMaxHealth)
  (Config|SetCurrentHealth (Config|GetCurrentHealth)))

(event Custom|OnTakeAnyDamage
  (params (DamagedActor :type Actor%20Object%20Reference) (Damage :type Float%20%28single-precision%29) (DamageType :type Damage%20Type%20Object%20Reference) (InstigatedBy :type Controller%20Object%20Reference) (DamageCauser :type Actor%20Object%20Reference))
  (Config|SetCurrentHealth (- (Config|GetCurrentHealth) Damage))
  (if (> (Config|GetCurrentHealth) 0.0)
    (Default|CallOnDamage DamagedActor Damage DamageType InstigatedBy DamageCauser)))

(event EventBeginPlay
  (if (Variables|Config|GetbStartAtMaxHealth)
    (Config|SetCurrentHealth (Variables|Config|GetMaxHealth)))
  (EventDispatchers|BindEventtoOnTakeAnyDamage (Components|GetOwner) (delegate Custom|OnTakeAnyDamage)))

(event EventEndPlay
  (params (EndPlayReason :type EEndPlayReason%20Enum :default "Destroyed"))
  (EventDispatchers|BindEventtoOnTakeAnyDamage (Components|GetOwner) (delegate Custom|OnTakeAnyDamage)))

(fn GetCurrentHealth
  (return (Math|Float|Clamp(Float) (Variables|Config|GetCurrentHealth) 0.0 (Variables|Config|GetMaxHealth))))

(fn GetCurrentHealthNormalized
  (return (/ (Config|GetCurrentHealth) (Variables|Config|GetMaxHealth))))

(fn SetMaxHealthMantainingHealthPercentage
  (params (NewMaxHealth :type Float%20%28single-precision%29))
  (LocalVariables|SetHealthPercentage (Config|GetCurrentHealthNormalized))
  (bind _output_get (Variables|Config|SetMaxHealth NewMaxHealth))
  (Config|SetCurrentHealth (* _output_get (LocalVariables|GetHealthPercentage)))
  (return))

(fn SetCurrentHealth
  (params (NewCurrentHealth :type Float%20%28single-precision%29))
  (bind _currenthealth (Config|GetCurrentHealth))
  (if (or (> NewCurrentHealth _currenthealth) (> _currenthealth 0.0))
    (LocalVariables|SetPrevHealth (Config|GetCurrentHealth))
    (bind _output_get (Variables|Config|SetCurrentHealth (Math|Float|Clamp(Float) NewCurrentHealth 0.0 (Variables|Config|GetMaxHealth))))
    (if (and (<= _output_get 0.0) (> (LocalVariables|GetPrevHealth) 0.0))
      (Default|CallOnDeath)
      (return)
      (elif (and (<= (LocalVariables|GetPrevHealth) 0.0) (> (Config|GetCurrentHealth) 0.0))
        (Default|CallOnRevive)
        (return)
        (else
          (return))))
    (else
      (return))))

(fn IsAlive
  (return (> (Config|GetCurrentHealth) 0.0)))
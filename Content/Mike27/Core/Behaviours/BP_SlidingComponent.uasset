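; Character component that detects sliding on too-steep floors and lets the character jump out of a slide.
; Sliding means Falling while an offset capsule overlap below finds a valid floor type; walkable floor angle sets the slide threshold.
; OnJumped launches with the stored velocity if a minimum-speed check passes, then starts a cooldown timer.
; Tick, enabled only for velocity limiting or debug, clamps slide speed and refreshes that stored velocity when limiting.
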(event Custom|OnJumped
  (bind _lastvelocity (Variables|Config|GetLastVelocity))
  (if (Config|Stats|IsJumpAllowed false)
    (Character|LaunchCharacter (Variables|Config|GetCharacter) (Math|Vector|MakeVector (.x _lastvelocity) (.y _lastvelocity) (.z _lastvelocity)) true false)
    (CallFunction|DisableJump)))

(event Custom|EnableJump
  (Utilities|Time|ClearandInvalidateTimerbyHandle (Variables|Config|GetJumpCooldownHandle))
  (Variables|Config|SetbJumpEnabled true))

(event Custom|DisableJump
  (Variables|Config|SetbJumpEnabled false)
  (bind _returnvalue (Utilities|Time|SetTimerbyEvent (delegate Custom|EnableJump) (Variables|Config|Stats|GetJumpCooldown)))
  (Variables|Config|SetJumpCooldownHandle _returnvalue))

(event EventBeginPlay
  (CallFunction|EnableJump)
  (Config|CheckTickEnableValidity))

(event EventTick
  (params (DeltaSeconds :type Float%20%28single-precision%29))
  (bind _character (Variables|Config|GetCharacter))
  (bind _charactermovement (Variables|/Script/Engine.Character|GetCharacterMovement _character))
  (Config|CheckTickEnableValidity)
  (if (Config|Stats|GetLimitSlideVelocityEnabled)
    (if (Config|Detection|IsSliding true)
      (Variables|/Script/Engine.MovementComponent|SetVelocity _charactermovement (Math|Vector|ClampVectorSize (Variables|/Script/Engine.MovementComponent|GetVelocity _charactermovement) 0.0 (Variables|Config|Stats|GetMaxSlidingVelocity)))))
  (if (Config|Debug|GetDebugEnabled)
    (CallFunction|CustomPrintString (Utilities|String|Append "Is sliding " (Utilities|String|ToString(Boolean) (Config|Detection|IsSliding false)) ", can jump: " (Utilities|String|ToString(Boolean) (Config|Stats|IsJumpAllowed false))) true true "(R=0.000000,G=0.000000,B=1.000000,A=1.000000)" 2.0)))

(fn IsSliding
  (params (bUpdateLastVelocity :type Boolean))
  (bind _character (Variables|Config|GetCharacter))
  (bind _character_2 (Variables|Config|GetCharacter))
  (bind _returnvalue (Transformation|GetActorLocation _character))
  (bind _capsulecomponent (Variables|/Script/Engine.Character|GetCapsuleComponent _character))
  (bind (_outradius _outhalfheight) (Components|Capsule|GetScaledCapsuleSize _capsulecomponent))
  (Utilities|IsValid _character_2
    (:Is%20Valid
      (if bUpdateLastVelocity
        (Variables|Config|SetLastVelocity (Variables|/Script/Engine.MovementComponent|GetVelocity (Variables|/Script/Engine.Character|GetCharacterMovement (Variables|Config|GetCharacter)))))
      (if (Utilities|Enum|Equal(Enum) (Variables|/Script/Engine.CharacterMovementComponent|GetMovementMode (Variables|/Script/Engine.Character|GetCharacterMovement _character_2)) "MOVE_Falling")
        (bind _returnvalue_2 (Class|KismetSystemLibrary|CapsuleOverlapComponents (Math|Vector|MakeVector (.x _returnvalue) (.y _returnvalue) (- (.z _returnvalue) (* _outhalfheight (Variables|Config|GetSizeMultiplier)))) _outradius _outhalfheight (Variables|Config|Detection|GetValidSlidingFloors) (Variables|Config|Detection|GetClassFilter) (Variables|Config|Detection|GetActorsToIgnore)))
        (return _returnvalue_2)
        (else
          _)))
    (:Is%20Not%20Valid
      _))
  (return false))

(fn Initialize
  (params (Character :type Character%20Object%20Reference))
  (Utilities|Array|RemoveItem (Variables|Config|Detection|GetActorsToIgnore) Character)
  (bind _output_get (Variables|Config|SetCharacter Character))
  (Utilities|Array|AddUnique (Variables|Config|Detection|GetActorsToIgnore) _output_get)
  (CallFunction|EnableJump)
  (return))

(fn GetMinimumAngleforSlide
  (bind _character (Variables|Config|GetCharacter))
  (Utilities|IsValid _character
    (:Is%20Valid
      (return (Class|CharacterMovementComponent|GetWalkableFloorAngle (Variables|/Script/Engine.Character|GetCharacterMovement _character))))
    (:Is%20Not%20Valid
      (return 0.0))))

(fn SetMinimumAngleforSlide
  (params (MinAngle :type Float%20%28single-precision%29))
  (bind _character (Variables|Config|GetCharacter))
  (Utilities|IsValid _character
    (:Is%20Valid
      (Pawn|Components|CharacterMovement|SetWalkableFloorAngle (Variables|/Script/Engine.Character|GetCharacterMovement _character) MinAngle))
    (:Is%20Not%20Valid
      _))
  (return))

(fn IsJumpAllowed
  (params (bUpdateLastVelocity :type Boolean))
  (if (Config|Stats|IsJumpDisabled)
    (return false)
    (else
      (return (Config|Detection|IsSliding bUpdateLastVelocity)))))

(fn GetCooldownInfo
  (bind _jumpcooldownhandle (Variables|Config|GetJumpCooldownHandle))
  (bind (_outtimeleft _outtimeelapsed _returnvalue) (Class|MikeBlueprintFunctionLibrary|IsTimerValid _jumpcooldownhandle))
  (return _outtimeelapsed _outtimeleft _returnvalue))

(fn GetNormalizedVelocityRequirement
  (bind _velocity (Config|Stats|GetCurrentCharacterVelocity))
  (bind _minvelocityrequiredforjump (Variables|Config|Stats|GetMinVelocityRequiredForJump))
  (bind _returnvalue (>= _velocity _minvelocityrequiredforjump))
  (Utilities|IsValid (Variables|Config|GetCharacter)
    (:Is%20Valid
      (if (Math|Float|NearlyEqual(Float) (Variables|Config|Stats|GetMinVelocityRequiredForJump) 0.0 1e-06)
        (return (select _returnvalue 1.0 0.0) _returnvalue)
        (else
          (return (Math|Float|Clamp(Float) (/ (Config|Stats|GetCurrentCharacterVelocity) (Variables|Config|Stats|GetMinVelocityRequiredForJump))) _returnvalue))))
    (:Is%20Not%20Valid
      (return 0.0 false))))

(fn GetCurrentCharacterVelocity
  (bind _character (Variables|Config|GetCharacter))
  (bind _charactermovement (Variables|/Script/Engine.Character|GetCharacterMovement _character))
  (bind _velocity (Variables|/Script/Engine.MovementComponent|GetVelocity _charactermovement))
  (Utilities|IsValid (Variables|Config|GetCharacter)
    (:Is%20Valid
      (if (Variables|Config|Stats|GetbCheckOnlyZVelocity)
        (return (Math|Float|Absolute(Float) (.z _velocity)))
        (else
          (return (Math|Vector|VectorLength (Math|Vector|MakeVector (.x _velocity) (.y _velocity) (.z _velocity)))))))
    (:Is%20Not%20Valid
      (return 0.0))))

(fn IsJumpDisabled
  (Utilities|IsValid (Variables|Config|GetCharacter)
    (:Is%20Valid
      (if (Math|Boolean|ANDBoolean (Variables|Config|Stats|GetbCanJumpWhenSliding) (Variables|Config|GetbJumpEnabled) (Utilities|Enum|Equal(Enum) "MOVE_Falling" (Variables|/Script/Engine.CharacterMovementComponent|GetMovementMode (Variables|/Script/Engine.Character|GetCharacterMovement (Variables|Config|GetCharacter)))))
        (return (not (.bGreater (Config|Stats|GetNormalizedVelocityRequirement))))
        (else
          (return true))))
    (:Is%20Not%20Valid
      (return true))))

(fn SetDebugEnabled
  (params (bEnabled :type Boolean))
  (Variables|Config|Debug|SetbDebugEnabled bEnabled)
  (Config|CheckTickEnableValidity)
  (return))

(fn SetLimitSlideVelocityEnabled
  (params (bEnabled :type Boolean))
  (Variables|Config|Stats|SetbLimitSlidingVelocity bEnabled)
  (Config|CheckTickEnableValidity)
  (return))

(fn CheckTickEnableValidity
  (Components|Tick|SetComponentTickEnabled (or (Variables|Config|Stats|GetbLimitSlidingVelocity) (Variables|Config|Debug|GetbDebugEnabled)))
  (return))

(fn GetDebugEnabled
  (return (Variables|Config|Debug|GetbDebugEnabled)))

(fn GetLimitSlideVelocityEnabled
  (return (and (Utilities|IsValid (Variables|Config|GetCharacter)) (Variables|Config|Stats|GetbLimitSlidingVelocity))))
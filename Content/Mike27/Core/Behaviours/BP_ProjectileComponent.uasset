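; Projectile collision component that turns impacts into damage, sound and optional AI noise, then notifies listeners and can destroy its actor.
; It takes the shooter from the projectile's owner, with getters and overrides for owner and instigator controller.
; Optional native hit and overlap bindings feed a shared Hit function, with overlaps ignoring the shooter.
; The audio component can be auto-found on the shooter at start.
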(event Custom|OnHit
  (params (HitComponent :type Primitive%20Component%20Object%20Reference) (OtherActor :type Actor%20Object%20Reference) (OtherComp :type Primitive%20Component%20Object%20Reference) (NormalImpulse :type Vector) (Hit :type Hit%20Result%20Structure%20%28by%20ref%29))
  (Config|Stats|Hit Hit))

(event Custom|OnBeginOverlap
  (params (OverlappedComponent :type Primitive%20Component%20Object%20Reference) (OtherActor :type Actor%20Object%20Reference) (OtherComp :type Primitive%20Component%20Object%20Reference) (OtherBodyIndex :type Integer) (bFromSweep :type Boolean) (SweepResult :type Hit%20Result%20Structure%20%28by%20ref%29))
  (if (!= OtherActor (Variables|Config|GetOwner))
    (Config|Stats|Hit SweepResult)))

(event EventBeginPlay
  (bind _output_get (Variables|Config|SetOwner (Components|GetOwner (Components|GetOwner))))
  (if (and (not (Utilities|IsValid (Variables|Config|Sound|GetAudio))) (Variables|Config|Sound|GetbSearchAudioComponentAtStart))
    (Variables|Config|Sound|SetAudio (Actor|GetComponentbyClass _output_get "/Script/Engine.AudioComponent")))
  (bind _aspawn (Utilities|Casting|CastToPawn _output_get)
    (:then
      (Variables|Config|SetInstigator (Pawn|GetController _aspawn)))
    (:CastFailed
      _))
  (if (Variables|Config|Stats|GetbUseNativeCollisionEvents)
    (EventDispatchers|AssignOnComponentHit (delegate Custom|OnHit))
    (EventDispatchers|AssignOnComponentBeginOverlap (delegate Custom|OnBeginOverlap))))

(event EventEndPlay
  (params (EndPlayReason :type EEndPlayReason%20Enum :default "Destroyed"))
  (if (Variables|Config|Stats|GetbUseNativeCollisionEvents)
    (EventDispatchers|UnbindEventfromOnComponentHit (delegate Custom|OnHit))
    (EventDispatchers|UnbindEventfromOnComponentBeginOverlap (delegate Custom|OnBeginOverlap))))

(fn Hit
  (params (Inpact :type Hit%20Result%20Structure%20%28by%20ref%29))
  (bind _hitactor (Collision|BreakHitResult Inpact))
  (bind _returnvalue (Components|GetOwner))
  (Config|Noise|PerformNoise)
  (Utilities|IsValid _hitactor
    (:Is%20Valid
      (Game|Damage|ApplyDamage _hitactor (Variables|Config|Stats|GetBaseDamage) (Variables|Config|GetInstigator) (Components|GetOwner) (Variables|Config|Stats|GetDamageType)))
    (:Is%20Not%20Valid
      _))
  (Default|CallOnProjectileCollision Inpact)
  (if (Variables|Config|Stats|GetbDestroyOnValidHit)
    (Utilities|IsValid _returnvalue
      (:Is%20Valid
        (if (not (Game|IsActorBeingDestroyed _returnvalue))
          (Actor|DestroyActor _returnvalue)))
      (:Is%20Not%20Valid
        _)))
  (return))

(fn PerformNoise
  (if (Variables|Config|Noise|GetbDisableNoise)
    (return)
    (else
      (Class|MikeBlueprintFunctionLibrary|PlaySound (Variables|Config|Sound|GetAudio) (Variables|Config|Sound|GetSound) 0.0 (Variables|Config|Noise|GetbPerformNoiseOnHit) (Transformation|GetWorldLocation) (Variables|Config|Noise|GetLoudness) (Variables|Config|GetOwner) (Variables|Config|Noise|GetMaxRange) (Variables|Config|Noise|GetTag))
      (return))))

(fn GetShooter
  (return (Variables|Config|GetOwner) (Variables|Config|GetInstigator)))

(fn OverrideShooter
  (params (Owner :type Actor%20Object%20Reference) (Instigator :type Controller%20Object%20Reference))
  (Variables|Config|SetOwner Owner)
  (Variables|Config|SetInstigator Instigator)
  (return))
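; Actor component that gives a character a sprint, raising walk speed and acceleration while it moves forward.
; StartSprint caches the CharacterMovement base stats and enables Tick, whose enabled state doubles as the sprint-active flag.
; Each tick scales both stats through IncrementalValue using the cosine of the forward movement angle, restoring them outside the angle tolerance.
; StopSprint or disabling restores the cached values, and getters expose base and boosted stats.
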(event Custom|StartSprint
  (bind _character (Variables|Config|GetCharacter))
  (bind _charactermovement (Variables|/Script/Engine.Character|GetCharacterMovement _character))
  (if (Config|GetEnabled)
    (if (not (Config|IsSprintActive))
      (Utilities|IsValid _character
        (:Is%20Valid
          (Config|SetMovementStats (Variables|/Script/Engine.CharacterMovementComponent|GetMaxWalkSpeed _charactermovement) (Variables|/Script/Engine.CharacterMovementComponent|GetMaxAcceleration _charactermovement))
          (Components|Tick|SetComponentTickEnabled true))))))

(event Custom|StopSprint
  (if (Config|IsSprintActive)
    (Components|Tick|SetComponentTickEnabled false)
    (Utilities|IsValid (Variables|Config|GetCharacter)
      (:Is%20Valid
        (Config|SetMovementStatstoCharacter)))))

(event Custom|Initialize
  (params (Character :type Character%20Object%20Reference) (bEnable :type Boolean))
  (bind _output_get (Variables|Config|SetCharacter Character))
  (Utilities|IsValid _output_get
    (:Is%20Valid
      (Config|SetMovementStats (Variables|/Script/Engine.CharacterMovementComponent|GetMaxWalkSpeed (Variables|/Script/Engine.Character|GetCharacterMovement _output_get)) (Variables|/Script/Engine.CharacterMovementComponent|GetMaxAcceleration (Variables|/Script/Engine.Character|GetCharacterMovement _output_get))))
    (:Is%20Not%20Valid
      _))
  (Config|SetEnabled bEnable)
  (CallFunction|StopSprint))

(event EventTick
  (params (DeltaSeconds :type Float%20%28single-precision%29))
  (bind (_dot _bmovingforward) (Config|IsMovingForward))
  (bind _character (Variables|Config|GetCharacter))
  (bind _charactermovement (Variables|/Script/Engine.Character|GetCharacterMovement _character))
  (Utilities|IsValid (Variables|Config|GetCharacter)
    (:Is%20Valid
      ;[1 1 1] Character movemente values updated based on if the character is moving forward and the deviation between character forward and movement direction
      (if _bmovingforward
        (Variables|/Script/Engine.CharacterMovementComponent|SetMaxWalkSpeed _charactermovement (Class|MikeBlueprintFunctionLibrary|IncrementalValue (Variables|Config|GetOriginalSpeed) (Variables|Config|GetSpeedMultiplierIncrement) _dot))
        (Variables|/Script/Engine.CharacterMovementComponent|SetMaxAcceleration _charactermovement (Class|MikeBlueprintFunctionLibrary|IncrementalValue (Variables|Config|GetOriginalAcceleration) (Variables|Config|GetAccelerationMultiplierIncrement) _dot))
        (else
          (Config|SetMovementStatstoCharacter))))
    (:Is%20Not%20Valid
      (CallFunction|StopSprint))))

(fn IsMovingForward
  (bind _forwardangletollerance (Variables|Config|GetForwardAngleTollerance))
  (bind _character (Variables|Config|GetCharacter))
  (bind _returnvalue (Transformation|GetActorForwardVector _character))
  (bind _returnvalue_2 (Transformation|GetActorRightVector _character))
  (bind _charactermovement (Variables|/Script/Engine.Character|GetCharacterMovement _character))
  (bind _velocity (Variables|/Script/Engine.MovementComponent|GetVelocity _charactermovement))
  (bind (_outforwardangle _outrightangle _boutismovingright _returnvalue_3) (Class|MikeBlueprintFunctionLibrary|IsMovingForwardXY _forwardangletollerance 9e+01 _returnvalue _returnvalue_2 _velocity))
  (Utilities|IsValid (Variables|Config|GetCharacter)
    (:Is%20Valid
      (return (Math|Trig|Cos(Degrees) _outforwardangle) _returnvalue_3))
    (:Is%20Not%20Valid
      (return 0.0 false))))

(fn SetMovementStatstoCharacter
  (bind _character (Variables|Config|GetCharacter))
  (bind _charactermovement (Variables|/Script/Engine.Character|GetCharacterMovement _character))
  (Variables|/Script/Engine.CharacterMovementComponent|SetMaxWalkSpeed _charactermovement (Variables|Config|GetOriginalSpeed))
  (Variables|/Script/Engine.CharacterMovementComponent|SetMaxAcceleration _charactermovement (Variables|Config|GetOriginalAcceleration))
  (return))

(fn IsSprintActive
  (return (Class|ActorComponent|IsComponentTickEnabled)))

(fn SetMovementStats
  (params (NewOriginalMaxWalkSpeed :type Float%20%28single-precision%29) (NewOriginalMaxAcceleration :type Float%20%28single-precision%29))
  (Variables|Config|SetOriginalSpeed NewOriginalMaxWalkSpeed)
  (Variables|Config|SetOriginalAcceleration NewOriginalMaxAcceleration)
  (return))

(fn GetMovementStats
  (return (Variables|Config|GetOriginalSpeed) (Variables|Config|GetOriginalAcceleration)))

(fn SetEnabled
  (params (bEnabled :type Boolean))
  (bind _output_get (Variables|Config|SetbEnabled bEnabled))
  (if _output_get
    _
    (else
      (CallFunction|StopSprint)))
  (return))

(fn GetEnabled
  (return (Variables|Config|GetbEnabled)))

(fn GetMaxSpeed
  (params (DefaultSpeedIfError :type Float%20%28single-precision%29))
  (bind _character (Variables|Config|GetCharacter))
  (if (Config|IsSprintActive)
    (LocalVariables|SetSpeed (Variables|Config|GetOriginalSpeed) :!label _label)
    (else
      (Utilities|IsValid _character
        (:Is%20Valid
          (LocalVariables|SetSpeed (Variables|/Script/Engine.CharacterMovementComponent|GetMaxWalkSpeed (Variables|/Script/Engine.Character|GetCharacterMovement _character))))
        (:Is%20Not%20Valid
          (goto _label)))))
  (if (Math|Float|NearlyEqual(Float) (Class|MikeBlueprintFunctionLibrary|IncrementalValue (LocalVariables|GetSpeed) (Variables|Config|GetSpeedMultiplierIncrement) 0.0) 0.0 1e-06)
    (return DefaultSpeedIfError)
    (else
      (return (Class|MikeBlueprintFunctionLibrary|IncrementalValue (LocalVariables|GetSpeed) (Variables|Config|GetSpeedMultiplierIncrement) 0.0)))))

(fn GetMaxAcceleration
  (return (Class|MikeBlueprintFunctionLibrary|IncrementalValue (Variables|Config|GetOriginalAcceleration) (Variables|Config|GetAccelerationMultiplierIncrement) 0.0)))
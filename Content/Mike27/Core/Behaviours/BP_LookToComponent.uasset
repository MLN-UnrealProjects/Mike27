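; Actor component that turns an assigned scene component to face a target component, a location, or a direction given as a velocity.
; Each tick it finds a focus point, optionally the target actor's bounds center, and builds an offset look-at rotation.
; It interpolates at constant speed on axes allowed by a roll/pitch/yaw mask.
; A tolerance check fires focused and unfocused events, and ticking follows owner validity when the owner is set.
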(event EventTick
  (params (DeltaSeconds :type Float%20%28single-precision%29))
  (bind _owner (Config|GetOwnerComponent))
  (bind (_target _focus) (Config|GetTargetRotation DeltaSeconds))
  (Utilities|IsValid _owner
    (:Is%20Valid
      (Transformation|SetWorldRotation _owner _target false (Variables|Config|GetbTeleport))
      (Config|UpdateFocusedStatus _focus))
    (:Is%20Not%20Valid
      (Config|SetOwnerComponent))))

(fn GetFocusLocation
  (bind (_target _targetlocation _buselocationasvelocity) (Config|GetTargetData))
  (bind _owner (Config|GetOwnerComponent))
  (bind _maskrotator (Config|GetRawRotationMask))
  (bind _returnvalue (Components|GetOwner _target))
  (bind (_x _y _z) (Math|Vector|BreakVector _targetlocation))
  (bind (_center _extents _returnvalue_2) (Class|MikeBlueprintFunctionLibrary|GetActorBoundsCenter _returnvalue true))
  (bind _returnvalue_3 (* _z (.yaw _maskrotator)))
  (bind _returnvalue_4 (* _x (.roll _maskrotator)))
  (bind _returnvalue_5 (* _y (.pitch _maskrotator)))
  (bind _returnvalue_6 (Math|Vector|MakeVector _returnvalue_4 _returnvalue_5 _returnvalue_3))
  (Utilities|IsValid _target
    (:Is%20Valid
      (if (Variables|Config|GetbFocusToTargetActorCenter)
        (if _returnvalue_2
          (return _center)
          (else
            _)))
      (return (Transformation|GetWorldLocation _target)))
    (:Is%20Not%20Valid
      (if _buselocationasvelocity
        (if (> (Math|Vector|VectorLength _returnvalue_6) (Variables|Config|GetVelocityTollerance))
          (LocalVariables|SetDirection (Math|Vector|Normalize _returnvalue_6))
          (else
            (Utilities|IsValid _owner
              (:Is%20Valid
                (LocalVariables|SetDirection (Math|Vector|GetForwardVector _owner)))
              (:Is%20Not%20Valid
                _))))
        (return (+ (LocalVariables|GetDirection) (.ReturnValue (Config|GetStartLocation))))
        (else
          (return _targetlocation))))))

(fn GetFocusRotation
  (bind (_returnvalue _bvalid) (Config|GetStartLocation))
  (bind _target (Config|GetFocusLocation))
  (bind _maskrotator (Config|GetRawRotationMask))
  (bind _returnvalue_2 (Math|Rotator|FindLookatRotation _returnvalue _target))
  (return (Math|Rotator|CombineRotators (Variables|Config|GetPreRotationOffset) (Math|Rotator|MakeRotator (* (.roll _returnvalue_2) (.roll _maskrotator)) (* (.pitch _returnvalue_2) (.pitch _maskrotator)) (* (.yaw _returnvalue_2) (.yaw _maskrotator)))) _bvalid))

(fn GetOwnerComponent
  (return (Variables|Config|GetOwner)))

(fn SetOwnerComponent
  (params (Owner :type Scene%20Component%20Object%20Reference))
  (bind _owner (Config|GetOwnerComponent))
  (if (!= Owner _owner)
    (bind _output_get (Variables|Config|SetOwner Owner))
    (Components|Tick|SetComponentTickEnabled (Utilities|IsValid _output_get))
    (Config|UpdateFocusedStatus (.Rot (Config|GetFocusRotation)))
    (return)
    (else
      (Components|Tick|SetComponentTickEnabled (Utilities|IsValid _owner))
      (return))))

(fn SetRotationMask
  (params (bAllowRoll :type Boolean) (bAllowPitch :type Boolean) (bAllowYaw :type Boolean))
  (Config|SetRawRotationMask (Math|Rotator|MakeRotator (Math|Conversions|ToFloat(Boolean) bAllowRoll) (Math|Conversions|ToFloat(Boolean) bAllowPitch) (Math|Conversions|ToFloat(Boolean) bAllowYaw)))
  (return))

(fn SetTarget
  (params (Target :type Scene%20Component%20Object%20Reference))
  (Variables|Config|SetTarget Target)
  (return))

(fn SetTargetLocation
  (params (TargetLocation :type Vector) (bLocAsVelocity :type Boolean))
  (Config|SetTarget)
  (Variables|Config|SetbUseLocationAsVelocity bLocAsVelocity)
  (Variables|Config|SetTargetLocation TargetLocation)
  (return))

(fn GetTargetData
  (return (Variables|Config|GetTarget) (Variables|Config|GetTargetLocation) (Variables|Config|GetbUseLocationAsVelocity)))

(fn SetData
  (params (TargetLocation :type Vector) (Target :type Scene%20Component%20Object%20Reference) (Owner :type Scene%20Component%20Object%20Reference) (bLocationAsVelocity :type Boolean))
  (Config|SetTargetLocation TargetLocation bLocationAsVelocity)
  (Config|SetTarget Target)
  (Config|SetOwnerComponent Owner)
  (return))

(fn GetRotationMask
  (bind _maskrotator (Config|GetRawRotationMask))
  (return (Math|Float|NearlyEqual(Float) (.roll _maskrotator) 1.0 1e-06) (Math|Float|NearlyEqual(Float) (.pitch _maskrotator) 1.0 1e-06) (Math|Float|NearlyEqual(Float) (.yaw _maskrotator) 1.0 1e-06)))

(fn GetRawRotationMask
  (return (Variables|Config|GetMaskRotator)))

(fn SetRawRotationMask
  (params (MaskRotator :type Rotator))
  (Variables|Config|SetMaskRotator (Math|Rotator|MakeRotator (Math|Conversions|ToFloat(Integer) (Math|Float|Round (Math|Float|Clamp(Float) (.roll MaskRotator)))) (Math|Conversions|ToFloat(Integer) (Math|Float|Round (Math|Float|Clamp(Float) (.pitch MaskRotator)))) (Math|Conversions|ToFloat(Integer) (Math|Float|Round (Math|Float|Clamp(Float) (.yaw MaskRotator))))))
  (return))

(fn GetTargetRotation
  (params (Deltatime :type Float%20%28single-precision%29))
  (bind _owner (Config|GetOwnerComponent))
  (bind _rot (Config|GetFocusRotation))
  (bind (_brollallowed _bpitchallowed _byawallowed) (Config|GetRotationMask))
  (bind _rotationspeed (Variables|Config|GetRotationSpeed))
  (bind _returnvalue (Transformation|GetWorldRotation _owner))
  (bind (_roll _pitch _yaw) (Math|Rotator|BreakRotator _returnvalue))
  (bind _returnvalue_2 (Class|KismetMathLibrary|RInterptoConstant _returnvalue _rot Deltatime _rotationspeed))
  (Utilities|IsValid _owner
    (:Is%20Valid
      (return (Math|Rotator|MakeRotator (select _brollallowed (.roll _returnvalue_2) _roll) (select _bpitchallowed (.pitch _returnvalue_2) _pitch) (select _byawallowed (.yaw _returnvalue_2) _yaw)) _rot))
    (:Is%20Not%20Valid
      (return "0, 0, 0" _rot))))

(fn IsTargetFocused
  (return (Variables|Config|GetbFocused)))

(fn UpdateFocusedStatus
  (params (Target :type Rotator))
  (bind _owner (Config|GetOwnerComponent))
  (Utilities|IsValid _owner
    (:Is%20Valid
      (Config|SetTargetFocused (Math|Rotator|Equal(Rotator) (Transformation|GetWorldRotation _owner) Target (Variables|Config|GetFocusTollerance))))
    (:Is%20Not%20Valid
      (Config|SetTargetFocused false)))
  (return))

(fn GetStartLocation
  (bind _owner (Config|GetOwnerComponent))
  (Utilities|IsValid _owner
    (:Is%20Valid
      (return (select (Variables|Config|GetbUseOwnerComponentAsStartLocation) (Transformation|GetWorldLocation _owner) (Variables|Config|GetStartLocation)) true))
    (:Is%20Not%20Valid
      (return "0, 0, 0" false))))

(fn SetTargetFocused
  (params (bFocused :type Boolean))
  (if (Math|Boolean|NotEqual(Boolean) bFocused (Config|IsTargetFocused))
    (bind _output_get (Variables|Config|SetbFocused bFocused))
    (if _output_get
      (Default|CallOnTargetFocused)
      (else
        (Default|CallOnTargetUnfocused)))
    (return)
    (else
      (return))))

(fn IsEnabled
  (return (Class|ActorComponent|IsComponentTickEnabled)))
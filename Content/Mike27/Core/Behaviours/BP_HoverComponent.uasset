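; Hover component that floats a target scene component, by default the owner's root, within a height band above ground.
; A looping timer traces down by line or bounds-sized multi-sphere with slope filtering, then accelerates clamped vertical velocity toward mid-band using a signed-square curve, or downward without ground.
; Tick applies that velocity as a swept world Z offset, without physics forces.
; Tick and timer pause when the target is invalid.
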(event Custom|OnCheckGround
  (bind (_distance _alpha _bvalid) (Config|GetCurrentHoveringHeightData))
  (Config|SetCurrentHoveringVelocity (Config|GetNewExpectedVelocity (Config|TranformDistanceAlpha _alpha _bvalid))))

(event Custom|RestartGroundCheckTimer
  (params (Interval :type Float%20%28single-precision%29))
  (Utilities|Time|ClearandInvalidateTimerbyHandle (Variables|Config|GetGroundCheckHandle))
  (bind _returnvalue (Utilities|Time|SetTimerbyEvent (delegate Custom|OnCheckGround) Interval true))
  (Variables|Config|SetEffectiveGroundCheckTimeStep Interval)
  (Variables|Config|SetGroundCheckHandle _returnvalue)
  (if (Class|ActorComponent|IsComponentTickEnabled)
    (Utilities|Time|UnpauseTimerbyHandle (Variables|Config|GetGroundCheckHandle))
    (else
      (Utilities|Time|PauseTimerbyHandle (Variables|Config|GetGroundCheckHandle)))))

(event EventBeginPlay
  (CallFunction|RestartGroundCheckTimer (Variables|Config|GetGroundCheckInterval))
  (Utilities|IsValid (Config|GetSceneComponent)
    (:Is%20Not%20Valid
      (Config|SetSceneComponent (Variables|/Script/Engine.Actor|GetRootComponent (Components|GetOwner))))))

(event EventTick
  (params (DeltaSeconds :type Float%20%28single-precision%29))
  (Utilities|IsValid (Config|GetSceneComponent)
    (:Is%20Valid
      (Transformation|AddWorldOffset (Config|GetSceneComponent) (Math|Vector|MakeVector 0.0 0.0 (* DeltaSeconds (Config|GetCurrentHoveringVelocity))) true false))
    (:Is%20Not%20Valid
      (Config|SetSceneComponent))))

(fn SetSceneComponent
  (params (PrimitiveComponent :type Scene%20Component%20Object%20Reference))
  (bind _groundcheckhandle (Variables|Config|GetGroundCheckHandle))
  (if (!= PrimitiveComponent (Config|GetSceneComponent))
    (Config|ResetHoveringVelocity)
    (bind _output_get (Variables|Config|SetSceneComponent PrimitiveComponent)))
  (Utilities|IsValid _output_get
    (:Is%20Valid
      (Components|Tick|SetComponentTickEnabled true)
      (Utilities|Time|UnpauseTimerbyHandle _groundcheckhandle))
    (:Is%20Not%20Valid
      (Components|Tick|SetComponentTickEnabled false)
      (Utilities|Time|PauseTimerbyHandle _groundcheckhandle)))
  (return))

(fn GetSceneComponent
  (return (Variables|Config|GetSceneComponent)))

(fn GetCurrentHoveringHeightData
  (Utilities|IsValid (Config|GetSceneComponent)
    (:Is%20Valid
      (bind (_hitdistance _bvalid) (Config|PerformTrace))
      (return _hitdistance (Class|MikeBlueprintFunctionLibrary|FastLinearConversion (Class|MikeBlueprintFunctionLibrary|InverseInterpolation _hitdistance (Variables|Config|GetMinDistanceFromGround) (Variables|Config|GetMaxDistanceFromGround)) 0.0 1.0 -1.0 1.0) _bvalid))
    (:Is%20Not%20Valid
      (return 0.0 0.0 false))))

(fn GetCurrentHoveringVelocity
  (return (Variables|Config|GetVelocity)))

(fn SetCurrentHoveringVelocity
  (params (NewVelocity :type Float%20%28single-precision%29))
  (bind _maxabsolutevelocity (Variables|Config|GetMaxAbsoluteVelocity))
  (Variables|Config|SetVelocity (Math|Float|Clamp(Float) NewVelocity (* -1.0 _maxabsolutevelocity) _maxabsolutevelocity))
  (return))

(fn GetGroundCheckIntervalTimerInfo
  (bind _groundcheckhandle (Variables|Config|GetGroundCheckHandle))
  (bind (_outtimeleft _outtimeelapsed _returnvalue) (Class|MikeBlueprintFunctionLibrary|IsTimerValid _groundcheckhandle))
  (return _outtimeleft _outtimeelapsed _returnvalue))

(fn ResetHoveringVelocity
  (Config|SetCurrentHoveringVelocity 0.0)
  (return))

(fn SetGroundCheckInterval
  (params (Interval :type Float%20%28single-precision%29))
  (CallFunction|RestartGroundCheckTimer Interval)
  (return))

(fn GetGroundCheckInterval
  (return (Variables|Config|GetEffectiveGroundCheckTimeStep)))

(fn GetNewExpectedVelocity
  (params (Alpha :type Float%20%28single-precision%29))
  (return (+ (Config|GetCurrentHoveringVelocity) (* Alpha (Variables|Config|GetHoveringAcceleration) (Config|GetGroundCheckInterval)))))

(fn TranformDistanceAlpha
  (params (Alpha :type Float%20%28single-precision%29) (bValidAlpha :type Boolean))
  (bind _returnvalue (Math|Float|Clamp(Float) Alpha -1.0))
  (if bValidAlpha
    (return (* (* (Math|Float|Sign(Float) _returnvalue) (Math|Float|Power _returnvalue 2.0)) -1.0))
    (else
      (return -1.0))))

(fn PerformTrace
  (bind _returnvalue (Transformation|GetWorldLocation))
  (bind _returnvalue_2 (Transformation|GetWorldLocation))
  (bind _component (Config|GetSceneComponent))
  (bind _returnvalue_3 (Components|GetOwner _component))
  (bind (_origin _boxextent) (Collision|GetActorBounds _returnvalue_3 true))
  (bind _returnvalue_4 (Math|Vector|MakeVector (.x _origin) (.y _origin) (.z _returnvalue_2)))
  (Utilities|IsValid _component
    (:Is%20Valid
      (if (Variables|Config|GetbSimpleTrace)
        (bind (_outhit _returnvalue_5) (Collision|LineTraceByChannel _returnvalue (- _returnvalue (Math|Vector|MakeVector 0.0 0.0 (Variables|Config|GetMaxDistanceFromGround))) "TraceTypeQuery1" false 0 (Variables|Config|GetTraceDebugMode)))
        (return (.distance _outhit) _returnvalue_5)
        (else
          (bind (_outhits _returnvalue_6) (Collision|MultiSphereTraceByChannel _returnvalue_4 (- _returnvalue_4 (Math|Vector|MakeVector 0.0 0.0 (Variables|Config|GetMaxDistanceFromGround))) (* (Math|Vector|VectorLength _boxextent) (Variables|Config|GetTraceSizeMultiplier)) "TraceTypeQuery1" false 0 (Variables|Config|GetTraceDebugMode)))
          (if _returnvalue_6
            (LocalVariables|SetSelfUp (Math|Vector|GetUpVector))
            (for _array_element _outhits
              (if (Math|Boolean|ANDBoolean (< (.distance _array_element) (LocalVariables|GetLastDistance)) (<= (Class|MikeBlueprintFunctionLibrary|GetAngleDegrees (LocalVariables|GetSelfUp) (.normal _array_element)) (Variables|Config|GetGroundAngleThreshold)) (Utilities|IsValid (.hitactor _array_element)))
                (LocalVariables|SetLastDistance (.distance _array_element))
                (LocalVariables|SetbValidDistance true)))
            (return (LocalVariables|GetLastDistance) (LocalVariables|GetbValidDistance))
            (else
              (return 0.0 false))))))
    (:Is%20Not%20Valid
      (return 0.0 false))))

(fn IsEnabled
  (return (Class|ActorComponent|IsComponentTickEnabled)))
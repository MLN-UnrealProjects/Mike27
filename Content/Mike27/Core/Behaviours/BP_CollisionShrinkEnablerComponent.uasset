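; Component that switches collision on a list of collision components according to how shrunk the current Mike character is.
; A looping timer, optionally auto-started and restarted on new-player events, tests whether the shrinking percentage lies within a min/max range.
; Each entry receives its own enabled or disabled collision type, and invalid entries are removed in reverse index order.
; A missing player or character stops the timer and unbinds the event.
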(event Custom|InternalActivateTimer
  (params (NewPlayer :type Controller%20Object%20Reference) (OldPlayer :type Controller%20Object%20Reference))
  (Utilities|IsValid NewPlayer
    (:Is%20Valid
      (Utilities|Time|ClearandInvalidateTimerbyHandle (Variables|Config|GetIntervalTimerHandle))
      (bind _returnvalue (Utilities|Time|SetTimerbyEvent (delegate Custom|CheckPlayerShrink) (Variables|Config|GetCheckInterval) true))
      (Variables|Config|SetIntervalTimerHandle _returnvalue))
    (:Is%20Not%20Valid
      (CallFunction|DisableInterval))))

(event Custom|CheckPlayerShrink
  (Config|UpdateCollisionEnableStatus))

(event Custom|DisableInterval
  (Utilities|Time|ClearandInvalidateTimerbyHandle (Variables|Config|GetIntervalTimerHandle))
  (if (Variables|Config|GetbEventBinded)
    (Variables|Config|SetbEventBinded (not (Variables|Config|GetbEventBinded)))
    (EventDispatchers|UnbindEventfromOnNewPlayer (CallFunction|GetMikeGameInstance) (delegate Custom|InternalActivateTimer))))

(event Custom|RestartInterval
  (if (Variables|Config|GetbEventBinded)
    _
    (else
      (Variables|Config|SetbEventBinded (not (Variables|Config|GetbEventBinded)))
      (EventDispatchers|BindEventtoOnNewPlayer (CallFunction|GetMikeGameInstance) (delegate Custom|InternalActivateTimer))))
  (Utilities|IsValid (CallFunction|GetCurrentMikeCharacter)
    (:Is%20Valid
      (CallFunction|InternalActivateTimer (CallFunction|GetCurrentPlayer)))))

(event EventBeginPlay
  (if (Variables|Config|GetbAutoActivateInterval)
    (CallFunction|RestartInterval)))

(fn GetIntervalTimerInfo
  (bind _intervaltimerhandle (Variables|Config|GetIntervalTimerHandle))
  (bind (_outtimeleft _outtimeelapsed _returnvalue) (Class|MikeBlueprintFunctionLibrary|IsTimerValid _intervaltimerhandle))
  (return _outtimeleft _outtimeelapsed _returnvalue))

(fn UpdateCollisionEnableStatus
  (bind _asbp_player_character (CallFunction|GetCurrentMikeCharacter))
  (Utilities|IsValid _asbp_player_character
    (:Is%20Valid
      (LocalVariables|SetbEnable (Math|Float|InRange(Float) (Default|GetShrinkingPercentage _asbp_player_character) (Variables|Config|GetMinPercentageEnabler) (Variables|Config|GetMaxPercentageEnabler)))
      (for (_array_element _array_index) (Variables|Config|GetCollisions)
        (Utilities|IsValid (.collision _array_element)
          (:Is%20Valid
            (Collision|SetCollisionEnabled (.collision _array_element) (select (LocalVariables|GetbEnable) (.enabledtype _array_element) (.disabledtype _array_element))))
          (:Is%20Not%20Valid
            (Utilities|Array|Add (LocalVariables|GetIndexesToRemove) _array_index))))
      (bind _arrayelement (Utilities|Array|ReverseforEachLoop (LocalVariables|GetIndexesToRemove))
        (:LoopBody
          (Utilities|Array|RemoveIndex (Variables|Config|GetCollisions) _arrayelement))
        (:Completed
          (return))))
    (:Is%20Not%20Valid
      (CallFunction|DisableInterval)
      (return))))
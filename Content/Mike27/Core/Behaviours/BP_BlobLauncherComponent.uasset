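; Blob launcher component that fires size-dependent projectiles with a limited pool of charges.
; It follows player changes and listens to the character's size changes to switch projectile type and scale at a shrink threshold.
; Live projectiles are tracked, each returning a charge when destroyed, and all are destroyed on EndPlay.
; Optional dynamic recycling destroys the oldest projectile when firing empty, once a fire-rate timer started on emptying has expired.
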(event Custom|OnNoAmmoLeft
  ;[1 1 1] Custom Refill charges
  (Utilities|Time|ClearandInvalidateTimerbyHandle (Variables|Config|GetPseudoFirerateHandler))
  (bind _returnvalue (Utilities|Time|SetTimerbyEvent (delegate Custom|OnPseudoFirerateOver) (Variables|Default|GetFireRate)))
  (Variables|Config|SetPseudoFirerateHandler _returnvalue))

(event Custom|OnPseudoFirerateOver
  ;[1 1 1] Custom Refill charges
  (Utilities|Time|ClearandInvalidateTimerbyHandle (Variables|Config|GetPseudoFirerateHandler)))

(event Custom|BindBullet
  (params (Bullet :type BP%20Projectile%20Base%20Object%20Reference))
  ;[1 1 1] Custom Refill charges
  (Utilities|Array|Add (Variables|Config|GetActiveProjectiles) Bullet)
  (Game|BindEventtoOnDestroyed Bullet (delegate Custom|AddCharge)))

(event Custom|AddCharge
  (params (DestroyedActor :type Actor%20Object%20Reference))
  ;[1 1 1] Custom Refill charges
  (bind _returnvalue (Utilities|Array|RemoveItem (Variables|Config|GetActiveProjectiles) DestroyedActor))
  (if _returnvalue
    (CallFunction|SetCurrentAmmo (+ 1 (CallFunction|GetCurrentAmmoLeft)) false)))

(event Custom|BindPlayer
  (params (Player :type BP%20Player%20Character%20Object%20Reference))
  ;[1 1 1] Set correct projectile to spawn
  (Utilities|IsValid Player
    (:Is%20Valid
      (EventDispatchers|BindEventtoOnSizeChanging Player (delegate Custom|SetProjectileToUse))
      (CallFunction|SetProjectiletoUse Player))))

(event Custom|UnbindPlayer
  (params (Player :type BP%20Player%20Character%20Object%20Reference))
  ;[1 1 1] Set correct projectile to spawn
  (Utilities|IsValid Player
    (:Is%20Valid
      (EventDispatchers|UnbindEventfromOnSizeChanging Player (delegate Custom|SetProjectileToUse)))))

(event Custom|Setup
  (params (NewPlayer :type Controller%20Object%20Reference) (OldPlayer :type Controller%20Object%20Reference))
  ;[1 1 1] Custom Refill charges
  (bind _asbp_player_character (Utilities|CasttoChar OldPlayer)
    (:Valid
      (CallFunction|UnbindPlayer _asbp_player_character))
    (:Invalid
      _))
  (bind _asbp_player_character_2 (Utilities|CasttoChar NewPlayer)
    (:Valid
      (CallFunction|BindPlayer _asbp_player_character_2))))

(event Custom|SetProjectileToUse
  (params (Character :type BP%20Player%20Character%20Object%20Reference))
  ;[1 1 1] Set correct projectile to spawn
  (if (>= (Default|GetShrinkingPercentage Character) (Variables|Config|Shrink|GetShrinkSwitchPercentage))
    (Variables|Default|SetProjectileType (Variables|Config|Shrink|GetShrunkProjectileType))
    (Variables|Default|SetProjectileScale (Variables|Config|Shrink|GetShrinkProjectileScale))
    (else
      (Variables|Default|SetProjectileType (Variables|Config|Shrink|GetGrownProjectileType))
      (Variables|Default|SetProjectileScale (Variables|Config|Shrink|GetGrownProjectileScale)))))

(event EventFire
  (params (Audio :type Audio%20Component%20Object%20Reference))
  ;[1 1 1] Custom Refill charges
  (if (Variables|Config|Shrink|GetbUseDynamicChargeRecycle)
    (Config|VerifyAvailableProjectiles))
  (|CallParentFunction Audio))

(event EventBeginPlay
  ;[1 1 1] Custom Refill charges
  (|CallParentFunction)
  (EventDispatchers|AssignOnEmptiedMagazine (delegate Custom|OnNoAmmoLeft))
  (EventDispatchers|BindEventtoOnShoot (delegate Custom|BindBullet))
  (EventDispatchers|BindEventtoOnNewPlayer (CallFunction|GetMikeGameInstance) (delegate Custom|Setup))
  (CallFunction|BindPlayer (CallFunction|GetCurrentMikeCharacter)))

(event EventEndPlay
  (params (EndPlayReason :type EEndPlayReason%20Enum :default "Destroyed"))
  ;[1 1 1] Custom Refill charges
  (|CallParentFunction EndPlayReason)
  (EventDispatchers|UnbindEventfromOnShoot (delegate Custom|BindBullet))
  (bind _asbp_player_character (Utilities|CasttoChar (CallFunction|GetCurrentPlayer))
    (:Valid
      (CallFunction|UnbindPlayer _asbp_player_character))
    (:Invalid
      _))
  (EventDispatchers|UnbindEventfromOnNewPlayer (CallFunction|GetMikeGameInstance) (delegate Custom|Setup))
  (bind _arrayelement (Utilities|Array|ReverseforEachLoop (Variables|Config|GetActiveProjectiles))
    (:LoopBody
      (Utilities|IsValid _arrayelement
        (:Is%20Valid
          (if (not (Game|IsActorBeingDestroyed _arrayelement))
            (Actor|DestroyActor _arrayelement)))))))

(fn VerifyAvailableProjectiles
  (bind _activeprojectiles (Variables|Config|GetActiveProjectiles))
  (if (Math|Boolean|ORBoolean (> (CallFunction|GetCurrentAmmoLeft) 0) (Class|KismetSystemLibrary|TimerExistsHandle (Variables|Config|GetPseudoFirerateHandler)) (<= (Utilities|Array|Length _activeprojectiles) 0))
    (return)
    (else
      (bind _output_get (LocalVariables|SetProjectileToRecycle (Utilities|Array|Get(acopy) _activeprojectiles)))
      (CallFunction|AddCharge _output_get)
      (Actor|DestroyActor _output_get)
      (return))))
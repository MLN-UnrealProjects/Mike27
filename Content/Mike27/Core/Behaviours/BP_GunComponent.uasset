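; Gun scene component that spawns projectiles from its own transform, with magazine ammo, sound and noise on each shot.
; A state machine (Ready, WaitDelay, WaitFirerate, Reloading, Empty) gates firing and reloading, using timers for fire delay, fire rate and reload.
; Reloading cancels a pending shot or pauses the fire-rate timer, which resumes if reloading is interrupted.
; Ammo setters clamp values and update state; dispatchers report shot, reload and empty-magazine events.
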(event Custom|Fire
  (params (Audio :type Audio%20Component%20Object%20Reference))
  (Variables|Config|SetAudioComponent Audio)
  (switch Utilities|FlowControl|Switch|SwitchonEGunStatus (Variables|Config|GetState)
    (:NewEnumerator0
      (if (Variables|Config|Stats|GetbAutoReloading)
        (CallFunction|Reload)))
    (:NewEnumerator2
      (if (Variables|Config|Stats|GetbUseDelay)
        (Variables|Config|SetState "NewEnumerator5")
        (Utilities|Time|ClearandInvalidateTimerbyHandle (Variables|Config|GetDelayTimer))
        (bind _returnvalue (Utilities|Time|SetTimerbyEvent (delegate Custom|ShootProjectile) (Variables|Config|Stats|GetFireDelay)))
        (Variables|Config|SetDelayTimer _returnvalue)
        (else
          (CallFunction|ShootProjectile))))))

(event Custom|Reload
  (bind (_ammoleft _maxammo) (Config|Stats|GetAmmoState))
  (switch Utilities|FlowControl|Switch|SwitchonEGunStatus (Variables|Config|GetState)
    (:NewEnumerator0
      _)
    (:NewEnumerator4
      (Utilities|Time|PauseTimerbyHandle (Variables|Config|GetFirerateTimer)))
    (:NewEnumerator2
      _)
    (:NewEnumerator5
      (Utilities|Time|ClearandInvalidateTimerbyHandle (Variables|Config|GetDelayTimer))))
  (if (!= _ammoleft _maxammo)
    (Variables|Config|SetState "NewEnumerator1")
    (Default|CallOnStartReloading)
    (Utilities|Time|ClearandInvalidateTimerbyHandle (Variables|Config|GetReloadingTimer))
    (bind _returnvalue (Utilities|Time|SetTimerbyEvent (delegate Custom|FillAmmo) (Variables|Config|Stats|GetReloadTime)))
    (Variables|Config|SetReloadingTimer _returnvalue)))

(event Custom|FillAmmo
  (Config|Stats|SetCurrentAmmo (Config|Stats|GetMaxAmmo) false)
  (Variables|Config|SetState "NewEnumerator2")
  (Default|CallOnReloaded))

(event Custom|InterruptReloading
  (switch Utilities|FlowControl|Switch|SwitchonEGunStatus (Variables|Config|GetState)
    (:NewEnumerator1
      (Utilities|Time|ClearandInvalidateTimerbyHandle (Variables|Config|GetReloadingTimer))
      (Default|CallOnReloadInterrupted)
      (if (Class|KismetSystemLibrary|IsTimerPausedHandle (Variables|Config|GetFirerateTimer))
        (Variables|Config|SetState "NewEnumerator4")
        (Utilities|Time|UnpauseTimerbyHandle (Variables|Config|GetFirerateTimer))
        (elif (<= (Config|Stats|GetCurrentAmmoLeft) 0)
          (Variables|Config|SetState "NewEnumerator0")
          (else
            (Variables|Config|SetState "NewEnumerator2")))))))

(event Custom|StartFirerateDelay
  (Variables|Config|SetState "NewEnumerator4")
  (Utilities|Time|ClearandInvalidateTimerbyHandle (Variables|Config|GetFirerateTimer))
  (bind _returnvalue (Utilities|Time|SetTimerbyEvent (delegate Custom|ShotReady) (Variables|Config|Stats|GetFireRate)))
  (Variables|Config|SetFirerateTimer _returnvalue))

(event Custom|ShotReady
  (Variables|Config|SetState "NewEnumerator2")
  (Default|CallOnFirerateOver))

(event Custom|ShootProjectile
  (bind _returnvalue (Components|GetOwner))
  (bind _returnvalue_2 (Transformation|GetWorldTransform))
  (Class|MikeBlueprintFunctionLibrary|PlaySound (Variables|Config|GetAudioComponent) (Variables|Config|Audio|GetSound) 0.0 (Variables|Config|Noise|GetbPerformNoise) (Transformation|GetWorldLocation) (Variables|Config|Noise|GetLoudness) (Components|GetOwner) (Variables|Config|Noise|GetMaxRange) (Variables|Config|Noise|GetTag))
  (bind _returnvalue_3 (Game|SpawnActorfromClass (Variables|Config|Stats|Projectile|GetProjectileType) (Math|Transform|MakeTransform (.location _returnvalue_2) (.rotation _returnvalue_2) (select (Variables|Config|Stats|GetbUseProjectileScale) (Variables|Config|Stats|Projectile|GetProjectileScale) (.scale _returnvalue_2))) "AlwaysSpawn" _returnvalue (.AsPawn (Utilities|Casting|CastToPawn _returnvalue))))
  (Utilities|IsValid _returnvalue_3
    (:Is%20Valid
      (Default|SetNoiseTag _returnvalue_3 (Variables|Config|Noise|GetTag))
      (Default|CallOnShoot _returnvalue_3)
      (Config|Stats|SetCurrentAmmo (- (Config|Stats|GetCurrentAmmoLeft) 1) false)
      (if (not (<= (Config|Stats|GetCurrentAmmoLeft) 0))
        (CallFunction|StartFirerateDelay :!label _label)))
    (:Is%20Not%20Valid
      (goto _label))))

(event EventBeginPlay
  (CallFunction|FillAmmo))

(fn GetCurrentState
  (return (Variables|Config|GetState)))

(fn GetCurrentAmmoLeft
  (return (Variables|Config|GetCurrentAmmo)))

(fn GetReloadingTimerInfo
  (bind _reloadingtimer (Variables|Config|GetReloadingTimer))
  (bind (_outtimeleft _outtimeelapsed _returnvalue) (Class|MikeBlueprintFunctionLibrary|IsTimerValid _reloadingtimer))
  (return _outtimeelapsed _outtimeleft _returnvalue (Utilities|Enum|Equal(Enum) (Variables|Config|GetState) "NewEnumerator1")))

(fn GetFirerateTimerInfo
  (bind _fireratetimer (Variables|Config|GetFirerateTimer))
  (bind (_outtimeleft _outtimeelapsed _returnvalue) (Class|MikeBlueprintFunctionLibrary|IsTimerValid _fireratetimer))
  (return _outtimeelapsed _outtimeleft _returnvalue (Utilities|Enum|Equal(Enum) (Variables|Config|GetState) "NewEnumerator4")))

(fn GetDelayTimerInfo
  (bind _delaytimer (Variables|Config|GetDelayTimer))
  (bind (_outtimeleft _outtimeelapsed _returnvalue) (Class|MikeBlueprintFunctionLibrary|IsTimerValid _delaytimer))
  (return _outtimeelapsed _outtimeleft _returnvalue (Utilities|Enum|Equal(Enum) (Variables|Config|GetState) "NewEnumerator5")))

(fn SetCurrentAmmo
  (params (CurrentAmmo :type Integer) (bUseFirerateIfPReviouslyEmpty :type Boolean))
  (LocalVariables|SetPreviousAmmo (Config|Stats|GetCurrentAmmoLeft))
  (bind _output_get (Variables|Config|SetCurrentAmmo (Math|Integer|Clamp(Integer) CurrentAmmo 0 (Config|Stats|GetMaxAmmo))))
  (if (> _output_get 0)
    (switch Utilities|FlowControl|Switch|SwitchonEGunStatus (Variables|Config|GetState)
      (:NewEnumerator0
        _)
      (:NewEnumerator1
        (Utilities|Time|ClearandInvalidateTimerbyHandle (Variables|Config|GetReloadingTimer)))
      (:NewEnumerator4
        (return))
      (:NewEnumerator2
        (return))
      (:NewEnumerator5
        (return)))
    (if (and bUseFirerateIfPReviouslyEmpty (<= (LocalVariables|GetPreviousAmmo) 0))
      (CallFunction|StartFirerateDelay)
      (else
        (Variables|Config|SetState "NewEnumerator2")))
    (return)
    (else
      (Default|CallOnEmptiedMagazine)
      (switch Utilities|FlowControl|Switch|SwitchonEGunStatus (Variables|Config|GetState)
        (:NewEnumerator0
          (if (Variables|Config|Stats|GetbAutoReloading) :!label _label
            _
            (else
              (Variables|Config|SetState "NewEnumerator0" :!label _label_2)
              (return))))
        (:NewEnumerator1
          (Utilities|Time|ClearandInvalidateTimerbyHandle (Variables|Config|GetReloadingTimer))
          (goto _label))
        (:NewEnumerator4
          (Utilities|Time|ClearandInvalidateTimerbyHandle (Variables|Config|GetFirerateTimer))
          (goto _label_2))
        (:NewEnumerator2
          (goto _label_2))
        (:NewEnumerator5
          (Utilities|Time|ClearandInvalidateTimerbyHandle (Variables|Config|GetDelayTimer))
          (goto _label_2)))
      (Utilities|FlowControl|Sequence
        (:then_0
          (Variables|Config|SetState "NewEnumerator0"))
        (:then_1
          (CallFunction|Reload)
          (return))))))

(fn GetAmmoState
  (return (Config|Stats|GetCurrentAmmoLeft) (Config|Stats|GetMaxAmmo)))

(fn GetMaxAmmo
  (return (Variables|Config|Stats|GetMaxAmmo)))

(fn SetMaxAmmo
  (params (MaxAmmo :type Integer))
  (Variables|Config|Stats|SetMaxAmmo MaxAmmo)
  (if (< (Config|Stats|GetMaxAmmo) (Config|Stats|GetCurrentAmmoLeft))
    (Config|Stats|SetCurrentAmmo (Config|Stats|GetMaxAmmo) false))
  (return))
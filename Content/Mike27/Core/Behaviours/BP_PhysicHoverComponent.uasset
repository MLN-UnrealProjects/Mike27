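; BP_PhysicHoverComponent is a scene component that makes its owner's physics primitive hover above surfaces.
; It defaults to the owner's root primitive and enables physics simulation on it.
; Each tick, it sphere-traces down from the component's height at the primitive's bounds center, using a bounds-based radius.
; A hit applies force along the surface normal, fading linearly with distance, while linear and angular damping are reapplied every tick.
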(event EventBeginPlay
  ;[1 1 1] Activate the physics on the object that implement this component
  (Utilities|IsValid (Config|GetPrimitiveComponent)
    (:Is%20Not%20Valid
      (Config|SetPrimitiveComponent (.AsPrimitive%20Component (Utilities|Casting|CastToPrimitiveComponent (Variables|/Script/Engine.Actor|GetRootComponent (Components|GetOwner))))))))

(event EventTick
  (params (DeltaSeconds :type Float%20%28single-precision%29))
  (bind _component (Config|GetPrimitiveComponent))
  (bind _component_2 (Config|GetPrimitiveComponent))
  (bind _returnvalue (Transformation|GetWorldLocation))
  (bind (_origin _boxextent _sphereradius) (Collision|GetComponentBounds _component))
  (bind _returnvalue_2 (Math|Vector|MakeVector (.x _origin) (.y _origin) (.z _returnvalue)))
  ;[1 1 1] Z of this scene component is used to determine trace starting height
  (bind (_outhit _returnvalue_3) (Collision|SphereTraceForObjects _returnvalue_2 (- _returnvalue_2 (Math|Vector|MakeVector 0.0 0.0 (Variables|Config|GetTraceLength))) (- _sphereradius 37.0) (Variables|Config|GetObjects) false 0 (Variables|Config|GetTraceDebugMode)))
  (if _returnvalue_3
    (Physics|AddForce (Config|GetPrimitiveComponent) (Config|GetHoveringForce (.Location (Collision|BreakHitResult _outhit)) (.ImpactNormal (Collision|BreakHitResult _outhit))) "None" false))
  (Class|PrimitiveComponent|SetLinearDamping _component_2 (Variables|Config|GetLinearDamping))
  (Class|PrimitiveComponent|SetAngularDamping _component_2 (Variables|Config|GetAngularDamping)))

(fn SetPrimitiveComponent
  (params (PrimitiveComponent :type Primitive%20Component%20Object%20Reference))
  (bind _output_get (Variables|Config|SetActorPrimitiveComponent PrimitiveComponent))
  (Utilities|IsValid _output_get
    (:Is%20Valid
      (Physics|SetSimulatePhysics _output_get true)
      (Components|Tick|SetComponentTickEnabled true))
    (:Is%20Not%20Valid
      (Components|Tick|SetComponentTickEnabled false)))
  (return))

(fn GetPrimitiveComponent
  (return (Variables|Config|GetActorPrimitiveComponent)))

(fn GetHoveringForce
  (params (HitLocation :type Vector) (HitNormal :type Vector))
  (bind _component (Config|GetPrimitiveComponent))
  (Utilities|IsValid _component
    (:Is%20Valid
      (return (* HitNormal (Math|Float|Lerp (Variables|Config|GetHoverForce) 0.0 (/ (Math|Vector|VectorLength (- HitLocation (Transformation|GetWorldLocation _component))) (Variables|Config|GetTraceLength))))))
    (:Is%20Not%20Valid
      (return "0, 0, 0"))))
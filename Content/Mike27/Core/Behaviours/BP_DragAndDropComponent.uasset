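; Actor component that lets its owner pick up, carry and drop physics objects along the forward axis of a supplied transform.
; Drag line-traces for a movable, simulating component within mass limit and grabs it with a supplied PhysicsHandle.
; Tick, enabled only while dragging, holds it at its grab distance and drops it when too far, too heavy or references are invalid.
; It also drops when the object's ReorderingComponent fires OnPreReordered.
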(event Custom|Drag
  (bind _transform (Variables|Config|GetTransform))
  (bind _dragignore (Variables|Config|Detection|GetDragIgnore))
  (Utilities|IsValidStatus
    (:Valid
      (if (Config|Stats|IsDraggingObject)
        (CallFunction|Drop))
      (bind (_outhitresult _returnvalue) (Class|MikeBlueprintFunctionLibrary|SimpleBlockingLineTraceSingleforObjects (Transformation|GetWorldLocation _transform) (Math|Vector|GetForwardVector _transform) (Variables|Config|Stats|GetPickupDistance) (Variables|Config|Detection|GetBlockingObjects) (Variables|Config|Detection|GetDraggableObjects) (Variables|Config|Detection|GetbTraceComplex) _dragignore _dragignore (Components|GetOwner)))
      (if _returnvalue
        (Utilities|ProcessLinetrace (.hitcomponent _outhitresult)
          (:ValidPickup
            (Config|Stats|PickupObject (.hitcomponent _outhitresult))
            (Default|CallOnPickedUp (Variables|Config|GetDraggedObject))))))))

(event Custom|Drop
  (bind _reordeable (Config|Stats|GetDraggedObjectReordeableComponent))
  ;[1 1 1] Release pickup if there is one, disable component
  (Utilities|IsValid (Variables|Config|GetDraggedObject)
    (:Is%20Valid
      (Physics|Components|PhysicsHandle|ReleaseComponent (Variables|Config|GetPhysicsHandle))
      (Utilities|IsValid _reordeable
        (:Is%20Valid
          (CallFunction|UnbindReordeableObject _reordeable))
        (:Is%20Not%20Valid
          _))
      (Default|CallOnDropped (Variables|Config|GetDraggedObject)))
    (:Is%20Not%20Valid
      _))
  (Variables|Config|SetDraggedObject 0)
  (Components|Tick|SetComponentTickEnabled false))

(event Custom|Initialize
  (params (Transform :type Scene%20Component%20Object%20Reference) (PhysicsHandle :type Physics%20Handle%20Component%20Object%20Reference))
  ;[1 1 1] Initialization, drops current pickup if there is one
  (CallFunction|Drop)
  (Variables|Config|SetTransform Transform)
  (Variables|Config|SetPhysicsHandle PhysicsHandle))

(event Custom|BindReordeableObject
  (params (Reordering :type Reordering%20Component%20Object%20Reference))
  (EventDispatchers|BindEventtoOnPreReordered Reordering (delegate Custom|Drop)))

(event Custom|UnbindReordeableObject
  (params (Reordeable :type Reordering%20Component%20Object%20Reference))
  (EventDispatchers|UnbindEventfromOnPreReordered Reordeable (delegate Custom|Drop)))

(event EventTick
  (params (DeltaSeconds :type Float%20%28single-precision%29))
  ;[1 1 1] If component has no longer valid refs disable component
  (Utilities|IsValidStatus
    (:Valid
      (Utilities|IsValid (Variables|Config|GetDraggedObject)
        (:Is%20Valid
          ;[1 1 1] Update pickup position throught physic handle
          (Physics|Components|PhysicsHandle|SetTargetLocation (Variables|Config|GetPhysicsHandle) (Config|Stats|GetNewPickupPosition (Variables|Config|GetObjectDistance)))
          ;[1 1 1] Drop pickup if it is no longer draggable
          (if (not (Config|Stats|IsPickupDraggable))
            (CallFunction|Drop)))
        (:Is%20Not%20Valid
          (CallFunction|Drop :!label _label))))
    (:Invalid
      (goto _label))))

(event EventBeginPlay
  ;[1 1 1] Make sure component is disabled initially
  (CallFunction|Drop))

(fn IsDraggingObject
  (return (Class|ActorComponent|IsComponentTickEnabled)))

(fn GetDraggedObject
  (return (Variables|Config|GetDraggedObject)))

(fn GetDraggedObjectDistance
  (return (Math|Vector|VectorLength (- (Transformation|GetWorldLocation (Variables|Config|GetDraggedObject)) (Transformation|GetWorldLocation (Variables|Config|GetTransform))))))

(fn GetNewPickupPosition
  (params (Distance :type Float%20%28single-precision%29))
  (bind _transform (Variables|Config|GetTransform))
  (return (+ (Transformation|GetWorldLocation _transform) (* (Math|Vector|GetForwardVector _transform) Distance))))

(fn IsPickupDraggable
  (return (not (or (> (Config|Detection|GetDraggedObjectDistance) (Variables|Config|Stats|GetBreakDistance)) (> (Physics|GetMass (Variables|Config|GetDraggedObject)) (Variables|Config|Stats|GetMaxDraggableMass))))))

(fn GetLineTracePoints
  (bind _transform (Variables|Config|GetTransform))
  (bind _returnvalue (Transformation|GetWorldLocation _transform))
  (return _returnvalue (+ _returnvalue (* (Math|Vector|GetForwardVector _transform) (Variables|Config|Stats|GetPickupDistance)))))

(fn PickupObject
  (params (DraggedObject :type Primitive%20Component%20Object%20Reference))
  (bind _reordeable (Config|Stats|GetDraggedObjectReordeableComponent))
  (bind _output_get (Variables|Config|SetDraggedObject DraggedObject))
  (Physics|Components|PhysicsHandle|GrabComponentatLocationwithRotation (Variables|Config|GetPhysicsHandle) _output_get "None" (Transformation|GetWorldLocation _output_get) (Transformation|GetWorldRotation _output_get))
  (Components|Tick|SetComponentTickEnabled true)
  (Variables|Config|SetObjectDistance (Config|Detection|GetDraggedObjectDistance))
  (Utilities|IsValid _reordeable
    (:Is%20Valid
      (CallFunction|BindReordeableObject _reordeable))
    (:Is%20Not%20Valid
      _))
  (return))

(fn GetDraggedObjectReordeableComponent
  (bind _draggedobject (Variables|Config|GetDraggedObject))
  (Utilities|IsValid _draggedobject
    (:Is%20Valid
      (return (Actor|GetComponentbyClass (Components|GetOwner _draggedobject) "/Script/Mike27.ReorderingComponent")))
    (:Is%20Not%20Valid
      (return 0))))
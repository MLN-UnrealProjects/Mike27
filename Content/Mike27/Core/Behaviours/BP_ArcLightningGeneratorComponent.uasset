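; Scene component that generates lightning arcs from its world location toward a destination actor.
; StartArcing spawns a BP_SpawnedArc at the component's transform and passes it an FArcValues struct of colour, noise settings and destination offset.
; The struct is built before SetDestinationArc refreshes that relative offset, so it reads the previously stored value.
; SetDestinationActor only accepts a new target while the current one is invalid.
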(event Custom|StartArcing
  (bind _returnvalue (Game|SpawnActorfromClass "/Game/Mike27/Weapons/Arc/BP_SpawnedArc.BP_SpawnedArc_C" (Transformation|GetWorldTransform) "Undefined" (Components|GetOwner) 0))
  (bind _arcstructout (Config|SetArcStruct))
  (Config|SetDestinationArc)
  (Default|Spawn _returnvalue _arcstructout))

(fn SetArcStruct
  (return (Utilities|Struct|MakeFArcValues (Variables|Default|GetArcColor) (Variables|Default|GetPassalong_D) (Variables|Default|GetArc%20Noise%20Scale) (Variables|Default|GetArc%20Noise%20Speed))))

(fn SetDestinationArc
  (Variables|Default|SetPassalong_D (- (Transformation|GetActorLocation (Variables|Default|GetDestination%20Object)) (Transformation|GetWorldLocation)))
  (return))

(fn SetDestinationActor
  (params (DestinationActor :type Actor%20Object%20Reference))
  (Utilities|IsValid (Variables|Default|GetDestination%20Object)
    (:Is%20Not%20Valid
      (Variables|Default|SetDestination%20Object DestinationActor)
      (return))))
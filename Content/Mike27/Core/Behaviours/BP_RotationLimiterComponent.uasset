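; Actor component that keeps a chosen scene component's relative rotation within configurable local min and max angles.
; Each tick it writes the clamped rotation back to the target, with limits optionally combined with a stored base rotation.
; SetLimitingComponent assigns the target and base rotation and enables ticking only while the target is valid; a lost target gets cleared, switching ticking off.
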(event EventTick
  (params (DeltaSeconds :type Float%20%28single-precision%29))
  (bind _transform (Variables|Config|GetTransform))
  (Utilities|IsValid _transform
    (:Is%20Valid
      (Transformation|SetRelativeRotation _transform (Config|GetClampedRotation) false false))
    (:Is%20Not%20Valid
      (Config|SetLimitingComponent "0, 0, 0"))))

(fn SetLimitingComponent
  (params (BaseRotation :type Rotator) (Component :type Scene%20Component%20Object%20Reference))
  (Variables|Config|SetBaseRotation BaseRotation)
  (bind _output_get (Variables|Config|SetTransform Component))
  (Components|Tick|SetComponentTickEnabled (Utilities|IsValid _output_get))
  (return))

(fn GetLimitingComponent
  (return (Variables|Config|GetTransform) (Variables|Config|GetBaseRotation)))

(fn GetClampedRotation
  (Utilities|IsValid (Variables|Config|GetTransform)
    (:Is%20Valid
      (if (Variables|Config|GetbUseBaseRotation)
        (LocalVariables|SetMaxRot (Math|Rotator|CombineRotators (Variables|Config|GetBaseRotation) (Variables|Config|GetMaxLocalRotation)))
        (LocalVariables|SetMinRot (Math|Rotator|CombineRotators (Variables|Config|GetBaseRotation) (Variables|Config|GetMinLocalRotation)))
        (else
          (LocalVariables|SetMaxRot (Variables|Config|GetMaxLocalRotation))
          (LocalVariables|SetMinRot (Variables|Config|GetMinLocalRotation))))
      (return (Class|MikeBlueprintFunctionLibrary|ClampAngles (Variables|/Script/Engine.SceneComponent|GetRelativeRotation (Variables|Config|GetTransform)) (LocalVariables|GetMinRot) (LocalVariables|GetMaxRot))))
    (:Is%20Not%20Valid
      (return "0, 0, 0"))))
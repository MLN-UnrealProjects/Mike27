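; Trigger component that loads a level when an overlap begins on it and unloads it when the overlap ends.
; It uses either a named streaming level or a level instance spawned at the origin, with optional blocking.
; Pending and loaded flags guard requests, queuing an opposite load or unload until the current operation completes.
; Completion handlers update state, fire OnLoaded or OnUnloaded, then run any queued request.
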(event Custom|OnBeginOverlap
  (params (OverlappedComponent :type Primitive%20Component%20Object%20Reference) (OtherActor :type Actor%20Object%20Reference) (OtherComp :type Primitive%20Component%20Object%20Reference) (OtherBodyIndex :type Integer) (bFromSweep :type Boolean) (SweepResult :type Hit%20Result%20Structure%20%28by%20ref%29))
  (if (or (Config|IsPendingOperation) (Config|IsLoaded))
    (bind _output_get (Variables|Config|SetbLoadLevel (Config|IsUnloading)))
    (if _output_get
      (Variables|Config|SetbUnloadLevel false))
    (else
      (Variables|Config|SetbPendingRequest true)
      (CallFunction|LoadLevel))))

(event Custom|OnEndOverlap
  (params (OverlappedComponent :type Primitive%20Component%20Object%20Reference) (OtherActor :type Actor%20Object%20Reference) (OtherComp :type Primitive%20Component%20Object%20Reference) (OtherBodyIndex :type Integer))
  (if (and (not (Config|IsPendingOperation)) (Config|IsLoaded))
    (Variables|Config|SetbPendingRequest true)
    (CallFunction|UnloadLevel)
    (else
      (bind _output_get (Variables|Config|SetbUnloadLevel (Config|IsLoading)))
      (if _output_get
        (Variables|Config|SetbLoadLevel false)))))

(event Custom|OnLevelLoaded
  (Default|CallOnLoaded self)
  (Variables|Config|SetbPendingRequest false)
  (Variables|Config|SetbLoaded true)
  (CallFunction|CustomPrintString "Load complete" true true "(R=0.000000,G=0.000000,B=1.000000,A=1.000000)" 2.0)
  (if (Variables|Config|GetbUnloadLevel)
    (CallFunction|UnloadLevel))
  (Variables|Config|SetbLoadLevel false)
  (Variables|Config|SetbUnloadLevel false))

(event Custom|OnLevelUnloaded
  (Default|CallOnUnloaded self)
  (Variables|Config|SetbPendingRequest false)
  (Variables|Config|SetbLoaded false)
  (Utilities|IsValid (Variables|Config|GetLoadedLevel)
    (:Is%20Valid
      (EventDispatchers|UnbindEventfromOnLevelLoaded (Variables|Config|GetLoadedLevel) (delegate Custom|OnLevelLoaded))
      (EventDispatchers|UnbindEventfromOnLevelUnloaded (Variables|Config|GetLoadedLevel) (delegate Custom|OnLevelUnloaded))
      (Variables|Config|SetLoadedLevel 0))
    (:Is%20Not%20Valid
      _))
  (CallFunction|CustomPrintString "Unload complete" true true "(R=0.000000,G=0.000000,B=1.000000,A=1.000000)" 2.0)
  (if (Variables|Config|GetbLoadLevel)
    (CallFunction|LoadLevel))
  (Variables|Config|SetbLoadLevel false)
  (Variables|Config|SetbUnloadLevel false))

(event Custom|UnloadLevel
  (if (Variables|Config|GetbUseStream)
    (Game|UnloadStreamLevel(byName) (Variables|Config|GetLevelName) (Variables|Config|GetbBlocking))
    (CallFunction|OnLevelUnloaded)
    (else
      (Variables|/Script/Engine.LevelStreaming|SetbShouldBeLoaded (Variables|Config|GetLoadedLevel) false))))

(event Custom|LoadLevel
  (if (Variables|Config|GetbUseStream)
    (Game|LoadStreamLevel(byName) (Variables|Config|GetLevelName) true (Variables|Config|GetbBlocking))
    (CallFunction|OnLevelLoaded)
    (else
      (bind (_boutsuccess _returnvalue) (Class|LevelStreamingDynamic|LoadLevelInstancebySoftObjectPtr (Variables|Config|GetLevelInstance) "0, 0, 0" "0, 0, 0"))
      (bind _output_get (Variables|Config|SetLoadedLevel _returnvalue))
      (if _boutsuccess
        (bind _output_get_2 (Variables|/Script/Engine.LevelStreaming|SetbShouldBlockOnLoad _output_get (Variables|Config|GetbBlocking)))
        (Variables|/Script/Engine.LevelStreaming|SetbShouldBlockOnUnload _output_get _output_get_2)
        (EventDispatchers|AssignOnLevelLoaded (Variables|Config|GetLoadedLevel) (delegate Custom|OnLevelLoaded))
        (EventDispatchers|BindEventtoOnLevelUnloaded (Variables|Config|GetLoadedLevel) (delegate Custom|OnLevelUnloaded))
        (else
          (Variables|Config|SetbLoaded false)
          (Variables|Config|SetbPendingRequest false))))))

(event EventBeginPlay
  (Config|Reset)
  (EventDispatchers|AssignOnComponentBeginOverlap (delegate Custom|OnBeginOverlap))
  (EventDispatchers|BindEventtoOnComponentEndOverlap (delegate Custom|OnEndOverlap)))

(event EventEndPlay
  (params (EndPlayReason :type EEndPlayReason%20Enum :default "Destroyed"))
  (EventDispatchers|UnbindEventfromOnComponentBeginOverlap (delegate Custom|OnBeginOverlap))
  (EventDispatchers|UnbindEventfromOnComponentEndOverlap (delegate Custom|OnEndOverlap)))

(fn IsLoaded
  (return (Variables|Config|GetbLoaded)))

(fn IsPendingOperation
  (return (Variables|Config|GetbPendingRequest)))

(fn IsLoading
  (return (and (not (Config|IsLoaded)) (Config|IsPendingOperation))))

(fn IsUnloading
  (return (and (Config|IsLoaded) (Config|IsPendingOperation))))

(fn Reset
  (Variables|Config|SetLoadedLevel 0)
  (Variables|Config|SetbLoaded false)
  (Variables|Config|SetbPendingRequest false)
  (Variables|Config|SetbLoadLevel false)
  (Variables|Config|SetbUnloadLevel false)
  (return))
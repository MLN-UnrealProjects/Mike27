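; Component that smoothly shrinks and grows a scene collision component, with start and interrupt sounds that can emit noise.
; Tick advances a timer that lerps scale between max and min, firing size-change callbacks.
; Overlapped shrink volumes are tracked, and the highest priority one clamps the range or disables commands.
; Capsule overlap tests block growth, either per tick or upfront in ImmediateCollisionGrowth mode, which snaps collision to max and scales registered transforms gradually.
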(event Custom|Shrink
  ;[1 1 1] Shrinking Command
  (if (not (.bdisableshrinkgrow (Config|Stats|GetCurrentShrinkVolumeLimits)))
    (Variables|Stats|SetStatus "NewEnumerator0")
    (Components|Tick|SetComponentTickEnabled true)
    (Class|MikeBlueprintFunctionLibrary|PlaySound (Variables|Stats|GetAudioEffect) (Variables|Config|Audio|GetShrinkEffect) 0.0 (Variables|Config|Noise|GetbPerformNoise) (Transformation|GetWorldLocation (Variables|Stats|GetSceneCollisionRef)) (Variables|Config|Noise|GetLoudness) (Variables|Stats|GetInstigator) (Variables|Config|Noise|GetMaxRange) (Variables|Config|Noise|GetTag))))

(event Custom|Grow
  (bind _maxscale (Config|Stats|GetMaxScale))
  (bind (_position _radius _halfheight) (Config|Stats|GetCapsuleStats _maxscale))
  ;[1 1 1] Growing Command
  (if (not (.bdisableshrinkgrow (Config|Stats|GetCurrentShrinkVolumeLimits)))
    (if (Variables|Config|Stats|GetbImmediateCollisionGrowth)
      (bind _boverlap (Config|Detection|CheckCapsuleOverlapping _position _radius _halfheight (Variables|Config|Detection|GetValidCollisions) (Variables|Config|Detection|GetComponentClassFilter) (Variables|Config|Detection|GetActorsToIgnore)))
      (if _boverlap
        (CallFunction|InterruptShrinkGrow true)
        (else
          (Transformation|SetWorldTransform (Variables|Stats|GetSceneCollisionRef) (Math|Transform|MakeTransform _position (Transformation|GetWorldRotation (Variables|Stats|GetSceneCollisionRef)) (Config|Stats|GetMaxScale)) false true)
          (Variables|Stats|SetStatus "NewEnumerator1" :!label _label)
          (Components|Tick|SetComponentTickEnabled true)
          (Class|MikeBlueprintFunctionLibrary|PlaySound (Variables|Stats|GetAudioEffect) (Variables|Config|Audio|GetGrowEffect) 0.0 (Variables|Config|Noise|GetbPerformNoise) (Transformation|GetWorldLocation (Variables|Stats|GetSceneCollisionRef)) (Variables|Config|Noise|GetLoudness) (Variables|Stats|GetInstigator) (Variables|Config|Noise|GetMaxRange) (Variables|Config|Noise|GetTag))))
      (else
        (goto _label)))))

(event Custom|ToggleShrinkGrow
  ;[1 1 1] Single input shrink grow
  (if (>= (Config|Stats|GetShrinkPercentage) 0.5)
    (CallFunction|Grow)
    (else
      (CallFunction|Shrink))))

(event Custom|RemoveCurrentVolume
  (Variables|Detection|SetCurrentShrinkVolume 0))

(event Custom|BindCollisionEvents
  (bind _scenecollisionref (Variables|Stats|GetSceneCollisionRef))
  (Utilities|IsValid _scenecollisionref
    (:Is%20Valid
      (Collision|BindEventtoOnComponentBeginOverlap _scenecollisionref (delegate Custom|OnBeginOverlap))
      (Collision|BindEventtoOnComponentEndOverlap _scenecollisionref (delegate Custom|OnEndOverlap))
      (Utilities|Array|AddUnique (Variables|Config|Detection|GetActorsToIgnore) (Components|GetOwner _scenecollisionref)))))

(event Custom|Initialize
  (params (Transform :type Primitive%20Component%20Object%20Reference) (ShrinkEffect :type Audio%20Component%20Object%20Reference) (NoiseInstigator :type Actor%20Object%20Reference) (Transforms :type Array%20of%20Scene%20Component%20Object%20References) (MaxScale :type Vector :default "1.000000,1.000000,1.000000"))
  ;[1 1 1] Initialization
  (Config|Detection|ClearTransforms)
  (Config|Noise|SetNoiseInstigator NoiseInstigator)
  (CallFunction|UnbindCollisionEvents)
  (Config|Audio|SetSoundComponent ShrinkEffect)
  (Variables|Stats|SetSceneCollisionRef Transform)
  (Config|Stats|SetMaxScale MaxScale)
  (Variables|Stats|SetTimer 0.0)
  (CallFunction|RemoveCurrentVolume)
  (CallFunction|InterruptShrinkGrow false)
  (CallFunction|BindCollisionEvents)
  (for _array_element Transforms
    (Config|Detection|AddTransform _array_element)))

(event Custom|InterruptShrinkGrow
  (params (bPlaySound :type Boolean))
  ;[1 1 1] Stop grow/shrink command
  (Variables|Stats|SetStatus "NewEnumerator2")
  (Components|Tick|SetComponentTickEnabled false)
  (if bPlaySound
    (Class|MikeBlueprintFunctionLibrary|PlaySound (Variables|Stats|GetAudioEffect) (Variables|Config|Audio|GetInterruptEffect) 0.0 (Variables|Config|Noise|GetbPerformNoise) (Transformation|GetWorldLocation (Variables|Stats|GetSceneCollisionRef)) (Variables|Config|Noise|GetLoudness) (Variables|Stats|GetInstigator) (Variables|Config|Noise|GetMaxRange) (Variables|Config|Noise|GetTag)))
  (Default|CallOnInterrupted))

(event Custom|UnbindCollisionEvents
  (bind _scenecollisionref (Variables|Stats|GetSceneCollisionRef))
  (Utilities|IsValid _scenecollisionref
    (:Is%20Valid
      (Collision|UnbindEventfromOnComponentBeginOverlap _scenecollisionref (delegate Custom|OnBeginOverlap))
      (Collision|UnbindEventfromOnComponentEndOverlap _scenecollisionref (delegate Custom|OnEndOverlap))
      (Utilities|Array|RemoveItem (Variables|Config|Detection|GetActorsToIgnore) (Components|GetOwner _scenecollisionref)))))

(event Custom|SetCurrentShrinkVolume
  (params (Volume :type BP%20Shrink%20Volume%20Component%20Object%20Reference))
  (bind _data (Config|Stats|GetCurrentShrinkVolumeLimits))
  (Utilities|IsValid Volume
    (:Is%20Valid
      (if (>= (.priority (Variables|/Game/Mike27/Core/Behaviours/BP_ShrinkVolumeComponent.BP_ShrinkVolumeComponent_C|GetData Volume)) (.priority (Config|Stats|GetCurrentShrinkVolumeLimits)))
        (Variables|Detection|SetCurrentShrinkVolume Volume)
        (Config|Stats|SetShrinkPercentage (Math|Float|Clamp(Float) (Config|Stats|GetShrinkPercentage) (.minshrinkpercentage _data) (.maxshrinkpercentage _data)))))))

(event Custom|OnBeginOverlap
  (params (OverlappedComponent :type Primitive%20Component%20Object%20Reference) (OtherActor :type Actor%20Object%20Reference) (OtherComp :type Primitive%20Component%20Object%20Reference) (OtherBodyIndex :type Integer) (bFromSweep :type Boolean) (SweepResult :type Hit%20Result%20Structure%20%28by%20ref%29))
  (bind _asbp_shrink_volume_component (Utilities|Casting|CastToBP_ShrinkVolumeComponent OtherComp))
  (CallFunction|AddShrinkVolume _asbp_shrink_volume_component))

(event Custom|OnEndOverlap
  (params (OverlappedComponent :type Primitive%20Component%20Object%20Reference) (OtherActor :type Actor%20Object%20Reference) (OtherComp :type Primitive%20Component%20Object%20Reference) (OtherBodyIndex :type Integer))
  (bind _asbp_shrink_volume_component (Utilities|Casting|CastToBP_ShrinkVolumeComponent OtherComp))
  (Config|Stats|RemoveShrinkVolume _asbp_shrink_volume_component))

(event Custom|AddShrinkVolume
  (params (ShrinkVolume :type BP%20Shrink%20Volume%20Component%20Object%20Reference%20%28by%20ref%29))
  (bind _returnvalue (Utilities|Array|AddUnique (Variables|Detection|GetActiveShrinkVolumes) ShrinkVolume))
  (if (>= _returnvalue 0)
    (CallFunction|SetCurrentShrinkVolume ShrinkVolume)))

(event EventTick
  (params (DeltaSeconds :type Float%20%28single-precision%29))
  ;[1 1 1] Grow/Shrink update logic
  (CallFunction|UpdateTImer DeltaSeconds)
  (Config|Stats|SetActorScale)
  (Default|CallOnSizeChange DeltaSeconds (Variables|Stats|GetStatus)))

(fn UpdateTimer
  (params (DeltaTime :type Float%20%28single-precision%29))
  (bind _data (Config|Stats|GetCurrentShrinkVolumeLimits))
  (bind _data_2 (Config|Stats|GetCurrentShrinkVolumeLimits))
  (bind _scale (Config|Stats|GetActorTargetScale))
  (bind _duration (Variables|Config|Stats|GetDuration))
  (bind _duration_2 (Variables|Config|Stats|GetDuration))
  (bind (_position _radius _halfheight) (Config|Stats|GetCapsuleStats _scale))
  (bind _returnvalue (* _duration_2 (.maxshrinkpercentage _data)))
  (bind _returnvalue_2 (* (.minshrinkpercentage _data_2) _duration))
  (LocalVariables|SetInitialTimer (Variables|Stats|GetTimer))
  (switch Utilities|FlowControl|Switch|SwitchonEShrinkingStatus (Variables|Stats|GetStatus)
    (:NewEnumerator0
      (Variables|Stats|SetTimer (Math|Float|Clamp(Float) (+ (Variables|Stats|GetTimer) DeltaTime) (* (.minshrinkpercentage _data) _duration_2) _returnvalue))
      (if (Math|Float|NearlyEqual(Float) _returnvalue (Variables|Stats|GetTimer) 1e-06)
        _
        (else
          (return))))
    (:NewEnumerator1
      (Variables|Stats|SetTimer (Math|Float|Clamp(Float) (- (Variables|Stats|GetTimer) DeltaTime) _returnvalue_2 (* _duration (.maxshrinkpercentage _data_2))))
      (if (Variables|Config|Stats|GetbImmediateCollisionGrowth)
        (if (Math|Float|NearlyEqual(Float) (Variables|Stats|GetTimer) _returnvalue_2 1e-06) :!label _label
          _
          (else
            (return)))
        (else
          (bind _boverlap (Config|Detection|CheckCapsuleOverlapping _position _radius _halfheight (Variables|Config|Detection|GetValidCollisions) (Variables|Config|Detection|GetComponentClassFilter) (Variables|Config|Detection|GetActorsToIgnore)))
          (if _boverlap
            (Variables|Stats|SetTimer (LocalVariables|GetInitialTimer))
            (else
              (goto _label)))))))
  (CallFunction|InterruptShrinkGrow true)
  (return))

(fn GetShrinkPercentage
  (return (/ (Variables|Stats|GetTimer) (Variables|Config|Stats|GetDuration))))

(fn GetActorTargetScale
  (return (Math|Vector|Lerp(Vector) (Config|Stats|GetMaxScale) (Variables|Config|Stats|GetMinScale) (Config|Stats|GetShrinkPercentage))))

(fn GetStatus
  (return (Variables|Stats|GetStatus)))

(fn SetShrinkPercentage
  (params (Alpha :type Float%20%28single-precision%29))
  (Variables|Stats|SetTimer (* (Math|Float|Clamp(Float) Alpha) (Variables|Config|Stats|GetDuration)))
  (Config|Stats|SetActorScale)
  (CallFunction|InterruptShrinkGrow false)
  (Default|CallOnSizeChange 0.0 (Variables|Stats|GetStatus))
  (return))

(fn GetCurrentShrinkVolumeLimits
  (Utilities|IsValid (Variables|Detection|GetCurrentShrinkVolume)
    (:Is%20Valid
      (return (Variables|/Game/Mike27/Core/Behaviours/BP_ShrinkVolumeComponent.BP_ShrinkVolumeComponent_C|GetData (Variables|Detection|GetCurrentShrinkVolume))))
    (:Is%20Not%20Valid
      (return (Utilities|Struct|MakeFShrinkVolumeData 1.0 false 0.0 -2147483648)))))

(fn RemoveShrinkVolume
  (params (Volume :type BP%20Shrink%20Volume%20Component%20Object%20Reference))
  (Utilities|IsValid Volume
    (:Is%20Valid
      (Utilities|Array|RemoveItem (Variables|Detection|GetActiveShrinkVolumes) Volume)
      (if (== Volume (Variables|Detection|GetCurrentShrinkVolume))
        (CallFunction|RemoveCurrentVolume)
        (LocalVariables|SetHigherPriorityVolume 0)
        (for _array_element (Variables|Detection|GetActiveShrinkVolumes)
          (Utilities|IsValid (LocalVariables|GetHigherPriorityVolume)
            (:Is%20Valid
              (if (>= (.priority (Variables|/Game/Mike27/Core/Behaviours/BP_ShrinkVolumeComponent.BP_ShrinkVolumeComponent_C|GetData _array_element)) (.priority (Variables|/Game/Mike27/Core/Behaviours/BP_ShrinkVolumeComponent.BP_ShrinkVolumeComponent_C|GetData (LocalVariables|GetHigherPriorityVolume))))
                (LocalVariables|SetHigherPriorityVolume _array_element)))
            (:Is%20Not%20Valid
              (LocalVariables|SetHigherPriorityVolume _array_element))))
        (CallFunction|SetCurrentShrinkVolume (LocalVariables|GetHigherPriorityVolume))
        (return)
        (else
          _)))
    (:Is%20Not%20Valid
      _))
  (return))

(fn SetActorScale
  (switch Utilities|FlowControl|Switch|SwitchonEShrinkingStatus (Variables|Stats|GetStatus)
    (:NewEnumerator0
      _)
    (:NewEnumerator1
      (if (Variables|Config|Stats|GetbImmediateCollisionGrowth)
        (for _array_element (Variables|Detection|GetTransforms)
          (Transformation|SetRelativeScale3D _array_element (/ (Config|Stats|GetActorTargetScale) (Config|Stats|GetMaxScale))))
        (return)
        (else
          _)))
    (:NewEnumerator2
      _))
  (Transformation|SetRelativeScale3D (Variables|Stats|GetSceneCollisionRef) (Config|Stats|GetActorTargetScale))
  (return))

(fn CheckCapsuleOverlapping
  (params (Position :type Vector%20%28by%20ref%29) (Radius :type Float%20%28single-precision%29) (HalfHeight :type Float%20%28single-precision%29) (ValidCollisions :type Array%20of%20EObjectTypeQuery%20Enums :default "ObjectTypeQuery1") (ComponentClassFilter :type Object%20Class%20Reference) (ActorsToIgnore :type Array%20of%20Actor%20Object%20References) (MaxOverlaps :type Integer))
  (bind _outcomponents (Class|KismetSystemLibrary|CapsuleOverlapComponents Position Radius HalfHeight ValidCollisions ComponentClassFilter ActorsToIgnore))
  (return (> (Utilities|Array|Length _outcomponents) MaxOverlaps)))

(fn GetCapsuleStats
  (params (TargetScale :type Vector))
  (bind _ascapsule_collision (Utilities|Casting|CastToCapsuleComponent (Variables|Stats|GetSceneCollisionRef))
    (:then
      (return (+ (Transformation|GetWorldLocation _ascapsule_collision) (Math|Vector|MakeVector 0.0 0.0 (- (* (Components|Capsule|GetUnscaledCapsuleHalfHeight _ascapsule_collision) (.y TargetScale)) (Components|Capsule|GetScaledCapsuleHalfHeight _ascapsule_collision)))) (* (Class|CapsuleComponent|GetUnscaledCapsuleRadius _ascapsule_collision) (.x TargetScale)) (* (Components|Capsule|GetUnscaledCapsuleHalfHeight _ascapsule_collision) (.y TargetScale))))
    (:CastFailed
      (return "0, 0, 0" 0.0 0.0))))

(fn SetSoundComponent
  (params (Component :type Audio%20Component%20Object%20Reference))
  (Utilities|IsValid (Variables|Stats|GetAudioEffect)
    (:Is%20Valid
      (Audio|Components|Audio|Stop (Variables|Stats|GetAudioEffect)))
    (:Is%20Not%20Valid
      _))
  (bind _output_get (Variables|Stats|SetAudioEffect Component))
  (Utilities|IsValid _output_get
    (:Is%20Valid
      (Audio|Components|Audio|Stop _output_get))
    (:Is%20Not%20Valid
      _))
  (return))

(fn SetNoiseInstigator
  (params (Instigator :type Actor%20Object%20Reference))
  (Variables|Stats|SetInstigator Instigator)
  (return))

(fn GetSoundComponent
  (return (Variables|Stats|GetAudioEffect)))

(fn GetNoiseInstigator
  (return (Variables|Stats|GetInstigator)))

(fn AddTransform
  (params (Transform :type Scene%20Component%20Object%20Reference%20%28by%20ref%29))
  (Utilities|IsValid Transform
    (:Is%20Valid
      (Utilities|Array|AddUnique (Variables|Detection|GetTransforms) Transform))
    (:Is%20Not%20Valid
      _))
  (return))

(fn RemoveTransform
  (params (Transform :type Scene%20Component%20Object%20Reference%20%28by%20ref%29))
  (Utilities|Array|RemoveItem (Variables|Detection|GetTransforms) Transform)
  (return))

(fn ClearTransforms
  (Utilities|Array|Clear (Variables|Detection|GetTransforms))
  (return))

(fn SetMaxScale
  (params (MaxScale :type Vector))
  (Variables|Stats|SetMaxScale MaxScale)
  (Config|Stats|SetShrinkPercentage (Config|Stats|GetShrinkPercentage))
  (return))

(fn GetMaxScale
  (return (Variables|Stats|GetMaxScale)))
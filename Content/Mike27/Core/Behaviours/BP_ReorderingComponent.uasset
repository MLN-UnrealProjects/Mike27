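; BP_ReorderingComponent is a physics-simulating component that periodically teleports a physics root, itself by default, back to its saved transform.
; A cooldown timer triggers Reordering, then a delay timer triggers Reorder, which briefly disables physics to teleport and restarts the cooldown.
; A fallback duration prevents infinite loops when both delays are zero.
; Callbacks report each phase, interruption and failure, while helper functions expose both timers' states.
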(event Custom|SaveInitialPosition
  (params (PhysicRoot :type Primitive%20Component%20Object%20Reference))
  (bind _output_get (Variables|Config|SetPhysicRoot PhysicRoot))
  (Variables|Config|SetOriginalTransform (Transformation|GetWorldTransform _output_get)))

(event Custom|Reorder
  (if (> (.OutTimeLeft (Config|IsReordering)) 0.0)
    (Default|CallOnReorderInterrupted))
  (if (Class|MikeBlueprintFunctionLibrary|IsPhysicActive (Variables|Config|GetPhysicRoot) (Utilities|Name|MakeLiteralName "None"))
    (Default|CallOnPreReordered)
    (Physics|SetSimulatePhysics (Variables|Config|GetPhysicRoot) false)
    (Transformation|SetWorldTransform (Variables|Config|GetPhysicRoot) (Variables|Config|GetOriginalTransform) false true)
    (Physics|SetSimulatePhysics (Variables|Config|GetPhysicRoot) true)
    (Default|CallOnReordered)
    (else
      (Default|CallOnReorderedFailed)))
  (CallFunction|RestartCooldown))

(event Custom|Reordering
  (Default|CallOnReordering (Variables|Config|GetOriginalTransform))
  ;[1 1 1] To avoid infinite loop
  (if (and (<= (Variables|Config|GetReorderingDuration) 0.0) (<= (Variables|Config|GetTimerIntervall) 0.0))
    (Variables|Config|SetReorderingDuration (Variables|Config|GetDefaultReorderingDuration)))
  (Utilities|Time|ClearandInvalidateTimerbyHandle (Variables|Config|GetDelayTimerHandle))
  (if (>= 0.0 (Variables|Config|GetReorderingDuration))
    (CallFunction|Reorder)
    (else
      (bind _returnvalue (Utilities|Time|SetTimerbyEvent (delegate Custom|Reorder) (Variables|Config|GetReorderingDuration)))
      (Variables|Config|SetDelayTimerHandle _returnvalue))))

(event Custom|RestartCooldown
  (bind _timerintervall (Variables|Config|GetTimerIntervall))
  (Utilities|Time|ClearandInvalidateTimerbyHandle (Variables|Config|GetCooldownTimerHandle))
  (if (>= 0.0 _timerintervall)
    (CallFunction|Reordering)
    (else
      (bind _returnvalue (Utilities|Time|SetTimerbyEvent (delegate Custom|Reordering) _timerintervall))
      (Variables|Config|SetCooldownTimerHandle _returnvalue))))

(event EventBeginPlay
  (Transformation|SetMobility "Movable")
  (Physics|SetSimulatePhysics true)
  (if (Variables|Config|GetbUseDefaultMass)
    (Class|PrimitiveComponent|SetMassOverrideinKg "None" (Variables|Config|GetDefaultMass) true))
  (if (Variables|Config|GetbSavePositionAtBeginPlay)
    (CallFunction|SaveInitialPosition self)
    (CallFunction|RestartCooldown)))

(fn IsReordering
  (bind _delaytimerhandle (Variables|Config|GetDelayTimerHandle))
  (bind (_outtimeleft _outtimeelapsed _returnvalue) (Class|MikeBlueprintFunctionLibrary|IsTimerValid _delaytimerhandle))
  (return _returnvalue _outtimeleft _outtimeelapsed))

(fn InonCooldown
  (bind _cooldowntimerhandle (Variables|Config|GetCooldownTimerHandle))
  (bind (_outtimeleft _outtimeelapsed _returnvalue) (Class|MikeBlueprintFunctionLibrary|IsTimerValid _cooldowntimerhandle))
  (return _returnvalue _outtimeleft _outtimeelapsed))
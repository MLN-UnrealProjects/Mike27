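; Player controller that registers itself as the single current player, destroys duplicates, and respawns the pawn at the current checkpoint.
; DoRespawn starts a timer unless one is pending; on expiry it spawns a same-class pawn at the checkpoint, possesses it, passes it the old pawn to reset, then destroys that.
; Caches the checkpoint container, exposes checkpoint health, shrink and depth-of-field data, and has debug inputs for releasing checkpoints and resetting collectibles.
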(event Custom|OnExecuteRespawn
  (Config|ExecuteRespawn))

(event EventBeginPlay
  (Utilities|IsValid (CallFunction|GetCurrentPlayer)
    (:Is%20Valid
      (CallFunction|CustomPrintString "Duplicate player controller is going to be destroyed" true true "(R=0.000000,G=0.000000,B=1.000000,A=1.000000)" 2.0)
      (Actor|DestroyActor))
    (:Is%20Not%20Valid
      (CallFunction|SetCurrentPlayer self)
      (Class|MikeBlueprintFunctionLibrary|SetNearClipPlane 0.02)
      (Config|GetCheckpointsContainer)
      (Variables|Config|SetOwnPawn 0))))

(event EventEndPlay
  (params (EndPlayReason :type EEndPlayReason%20Enum :default "Destroyed"))
  (if (== (CallFunction|GetCurrentPlayer) self)
    (CallFunction|SetCurrentPlayer)))

(event EventDoRespawn
  (Utilities|CheckRespawnValidity
    (:Is%20Valid
      (bind _returnvalue (Utilities|Time|SetTimerbyEvent (delegate Custom|OnExecuteRespawn) (Variables|Config|GetRespawnTime)))
      (Variables|Config|SetRespawnTimerHandle _returnvalue))
    (:Not%20Valid
      (CallFunction|CustomPrintString "Respawn not valid" true true "(R=0.000000,G=0.000000,B=1.000000,A=1.000000)" 2.0))))

(event Input|ActionEvents|InputActionDEBUG_ReleaseAllCheckpoints
  (params (Key :type Key%20Structure))
  ;[1 1 1] Only for debug, releases all checkpoints
  (:Pressed
    (Utilities|IsValid (Config|GetCurrentControlledPawn)
      (:Is%20Not%20Valid
        (if true
          (bind _container (Config|GetCheckpointsContainer))
          (Utilities|IsValid _container
            (:Is%20Valid
              (Default|ReleaseAllCheckpoints _container)
              (CallFunction|CustomPrintString "Released checkpoints" true true "(R=0.000000,G=0.000000,B=1.000000,A=1.000000)" 2.0))))))))

(event Input|ActionEvents|InputActionDEBUG_ResetCollectables
  (params (Key :type Key%20Structure))
  ;[1 1 1] Debug: By pressing 1 it resets the saved collectibles
  (:Pressed
    (bind _asbp_gamemode_mike_base (Utilities|Casting|CastToBP_Gamemode_Mike_Base (Game|GetGameMode))
      (:then
        (bind _returnvalue (Default|DebugResetCollectibles _asbp_gamemode_mike_base))
        (if _returnvalue
          (CallFunction|CustomPrintString "Collectables resetted" true true "(R=0.000000,G=0.000000,B=1.000000,A=1.000000)" 2.0)
          (else
            (CallFunction|CustomPrintString "Failed to release collectables." true true "(R=0.000000,G=0.000000,B=1.000000,A=1.000000)" 2.0))))
      (:CastFailed
        (CallFunction|CustomPrintString "Invalid gamemode type" true true "(R=0.000000,G=0.000000,B=1.000000,A=1.000000)" 2.0)))))

(fn ConstructionScript)

(fn GetCheckpointsContainer
  (Utilities|IsValid (Variables|Config|GetCheckpoints)
    (:Is%20Valid
      (return (Variables|Config|GetCheckpoints)))
    (:Is%20Not%20Valid
      (bind _outactors (Actor|GetAllActorsOfClass "/Game/Mike27/Placeables/BP_Checkpoint_Container.BP_Checkpoint_Container_C"))
      (if (> (Utilities|Array|Length _outactors) 0)
        (bind _output_get (Variables|Config|SetCheckpoints (Utilities|Array|Get(acopy) _outactors)))
        (return _output_get)
        (else
          (return (Variables|Config|GetCheckpoints)))))))

(fn ExecuteRespawn
  (bind _controlled (Config|GetCurrentControlledPawn))
  (bind _container (Config|GetCheckpointsContainer))
  (Utilities|IsValid _container
    (:Is%20Valid
      (Utilities|IsValid (Default|GetCurrentCheckpoint (Variables|Config|GetCheckpoints))
        (:Is%20Valid
          (Utilities|IsValid _controlled
            (:Is%20Valid
              (bind _output_get (LocalVariables|SetPrevious _controlled))
              (CallFunction|SetCurrentPlayer)
              (Pawn|UnPossess)
              (bind _returnvalue (Game|SpawnActorfromClass (Utilities|GetClass _output_get) (Default|GetSpawnPoint (Default|GetCurrentCheckpoint (Variables|Config|GetCheckpoints))) "AdjustIfPossibleButAlwaysSpawn" 0 0))
              (Utilities|IsValid _returnvalue
                (:Is%20Valid
                  (Pawn|Possess _returnvalue)
                  (Class|BPIResettable|DoReset(Message) _returnvalue (LocalVariables|GetPrevious))
                  (Actor|DestroyActor (LocalVariables|GetPrevious))
                  (CallFunction|SetCurrentPlayer self)
                  (CallFunction|CustomPrintString "Respawned" true true "(R=0.000000,G=0.000000,B=1.000000,A=1.000000)" 2.0)
                  (return))
                (:Is%20Not%20Valid
                  (CallFunction|CustomPrintString "Failed to spawn new character" true true "(R=0.000000,G=0.000000,B=1.000000,A=1.000000)" 2.0)
                  (return))))
            (:Is%20Not%20Valid
              _)))
        (:Is%20Not%20Valid
          _)))
    (:Is%20Not%20Valid
      _))
  (CallFunction|CustomPrintString "Failed to respawn" true true "(R=0.000000,G=0.000000,B=1.000000,A=1.000000)" 2.0)
  (return))

(fn GetRespawnTimerInfo
  (bind _respawntimerhandle (Variables|Config|GetRespawnTimerHandle))
  (bind (_outtimeleft _outtimeelapsed _returnvalue) (Class|MikeBlueprintFunctionLibrary|IsTimerValid _respawntimerhandle))
  (return _outtimeleft _outtimeelapsed _returnvalue))

(fn GetCurrentControlledPawn
  (bind _returnvalue (Pawn|GetControlledPawn))
  (if (== (Variables|Config|GetOwnPawn) _returnvalue)
    _
    (else
      (Variables|Config|SetOwnPawn _returnvalue)))
  (return (Variables|Config|GetOwnPawn)))

(fn GetRespawnInfo
  (bind _checkpoints (Variables|Config|GetCheckpoints))
  (bind _currentcheckpoint (Default|GetCurrentCheckpoint _checkpoints))
  (Utilities|IsValid _checkpoints
    (:Is%20Valid
      (Utilities|IsValid _currentcheckpoint
        (:Is%20Valid
          (return (Default|GetShrinkPercentageatCheckpoint _currentcheckpoint) (Default|GetHealthatCheckpoint _currentcheckpoint) (Default|GetMethodDOFatCheckpoint _currentcheckpoint) true))
        (:Is%20Not%20Valid
          _)))
    (:Is%20Not%20Valid
      _))
  (return 0.0 0.0 0 false))
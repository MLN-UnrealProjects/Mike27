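; Turret actor that takes its targeting and firing cues from the nearest linked guard AI.
; Each tick it picks the closest AIC_Guard controller from its AIPawn list, pruning invalid entries and rebuilding the controller cache when empty.
; In Chase or Attack it fires, aiming the look-to component at that guard's target if valid.
; In other states it returns to the default forward direction captured at construction and reloads.
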(event EventBeginPlay
  (bind _bp_looktocomponent (Variables|Default|GetBP_LookToComponent))
  (Default|SetRotationMask _bp_looktocomponent false true true)
  (Default|SetData _bp_looktocomponent (CallFunction|GetDefaultPointtoLook) 0 (CallFunction|GetRotableComponent) false))

(event EventTick
  (params (DeltaSeconds :type Float%20%28single-precision%29))
  (bind _closestai (CallFunction|GetClosestAi))
  (bind _bp_looktocomponent (Variables|Default|GetBP_LookToComponent))
  (bind _target (Default|GetTarget _closestai))
  (CallFunction|UpdateClosestController)
  (Utilities|IsValid _closestai
    (:Is%20Valid
      (switch Utilities|FlowControl|Switch|SwitchonEGuardState (Default|GetGuardState _closestai)
        (:NewEnumerator0
          (Default|SetTargetLocation (Variables|Default|GetBP_LookToComponent) (CallFunction|GetDefaultPointtoLook) false :!label _label)
          (Default|Reload (Variables|Default|GetBP_GunComponent)))
        (:NewEnumerator1
          (goto _label))
        (:NewEnumerator2
          (Utilities|IsValid _target :!label _label_2
            (:Is%20Valid
              (Default|SetTarget _bp_looktocomponent (Variables|/Script/Engine.Actor|GetRootComponent _target)))
            (:Is%20Not%20Valid
              (Default|SetTargetLocation _bp_looktocomponent (CallFunction|GetDefaultPointtoLook) false)))
          (Default|Fire (Variables|Default|GetBP_GunComponent) (Variables|Default|GetAudio)))
        (:NewEnumerator3
          (goto _label))
        (:NewEnumerator4
          (goto _label_2))))
    (:Is%20Not%20Valid
      (CallFunction|CustomPrintString "No Valid Attached controller" true true "(R=0.000000,G=0.000000,B=1.000000,A=1.000000)" 2.0))))

(fn ConstructionScript
  (bind _rotable (CallFunction|GetRotableComponent))
  (Variables|/Game/Mike27/Core/Behaviours/BP_LookToComponent.BP_LookToComponent_C|SetPreRotationOffset (Variables|Default|GetBP_LookToComponent) (Transformation|GetWorldRotation _rotable))
  (Variables|Config|SetDefaultLookDirection (Math|Vector|GetForwardVector _rotable)))

(fn RefreshAiControllers
  (Utilities|Array|Clear (Variables|Config|GetAiControllers))
  (for (_array_element _array_index) (Variables|Config|GetAIPawn)
    (Utilities|IsValid _array_element
      (:Is%20Valid
        (bind _asaic_guard (Utilities|Casting|CastToAIC_Guard (Pawn|GetController _array_element)))
        (Utilities|Array|AddUnique (Variables|Config|GetAiControllers) _asaic_guard))
      (:Is%20Not%20Valid
        (Utilities|Array|Add (LocalVariables|GetIndexesToRemove) _array_index))))
  (bind _arrayelement (Utilities|Array|ReverseforEachLoop (LocalVariables|GetIndexesToRemove))
    (:LoopBody
      (Utilities|Array|RemoveIndex (Variables|Config|GetAIPawn) _arrayelement))
    (:Completed
      (return))))

(fn GetDefaultPointtoLook
  (return (+ (Variables|Config|GetDefaultLookDirection) (Transformation|GetWorldLocation (CallFunction|GetRotableComponent)))))

(fn GetRotableComponent
  (return (Variables|Default|GetPivotBarrel)))

(fn GetControllers
  (return (Variables|Config|GetAiControllers)))

(fn UpdateClosestController
  (bind _aicontrollers (Variables|Config|GetAiControllers))
  (Variables|Config|SetClosestAi 0)
  (LocalVariables|SetMyLocation (Transformation|GetActorLocation))
  (if (<= (Utilities|Array|Length _aicontrollers) 0)
    (CallFunction|RefreshAiControllers))
  (for (_array_element _array_index) _aicontrollers
    (Utilities|IsValid _array_element
      (:Is%20Valid
        (Utilities|IsValid (Pawn|GetControlledPawn _array_element)
          (:Is%20Valid
            (if (> (LocalVariables|GetLastDistance) (Math|Vector|VectorLengthSquared (- (Transformation|GetActorLocation (Pawn|GetControlledPawn _array_element)) (LocalVariables|GetMyLocation))))
              (LocalVariables|SetLastDistance (Math|Vector|VectorLengthSquared (- (Transformation|GetActorLocation (Pawn|GetControlledPawn _array_element)) (LocalVariables|GetMyLocation))))
              (Variables|Config|SetClosestAi _array_element)))
          (:Is%20Not%20Valid
            (Utilities|Array|Add (LocalVariables|GetIndexesToRemove) _array_index :!label _label))))
      (:Is%20Not%20Valid
        (goto _label))))
  (bind _arrayelement (Utilities|Array|ReverseforEachLoop (LocalVariables|GetIndexesToRemove))
    (:LoopBody
      (Utilities|Array|RemoveIndex (Variables|Config|GetAiControllers) _arrayelement))
    (:Completed
      (return))))

(fn GetClosestAi
  (return (Variables|Config|GetClosestAi)))
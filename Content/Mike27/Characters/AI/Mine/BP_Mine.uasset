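; Hovering mine pawn that targets players and explodes with radial damage.
; On possession it passes hover and blast settings to AIC_Mine, and its detection sphere sets or clears that controller's player target.
; StartExplosion runs a single, non-restartable ticking fuse, with its timer state exposed through GetExplosionDelayTimerInfo.
; Explode applies damage, hides and disables the mine, emits a noise with the blast sound, and destroys it once audio finishes.
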(event OnComponentBeginOverlap(DetectionRange)
  (params (OverlappedComponent :type Primitive%20Component%20Object%20Reference) (OtherActor :type Actor%20Object%20Reference) (OtherComp :type Primitive%20Component%20Object%20Reference) (OtherBodyIndex :type Integer) (bFromSweep :type Boolean) (SweepResult :type Hit%20Result%20Structure%20%28by%20ref%29))
  (Utilities|IsValid (Variables|Config|GetAIController)
    (:Is%20Valid
      (Utilities|IsValid (Default|GetTarget (Variables|Config|GetAIController))
        (:Is%20Not%20Valid
          (bind _asbp_player_character (Utilities|Casting|CastToBP_PlayerCharacter OtherActor))
          (Default|SetTarget (Variables|Config|GetAIController) _asbp_player_character))))))

(event OnComponentEndOverlap(DetectionRange)
  (params (OverlappedComponent :type Primitive%20Component%20Object%20Reference) (OtherActor :type Actor%20Object%20Reference) (OtherComp :type Primitive%20Component%20Object%20Reference) (OtherBodyIndex :type Integer))
  (Utilities|IsValid (Variables|Config|GetAIController)
    (:Is%20Valid
      (if (== OtherActor (Default|GetTarget (Variables|Config|GetAIController)))
        (Default|SetTarget (Variables|Config|GetAIController))))))

(event Custom|StartExplosion
  (if (not (Class|KismetSystemLibrary|TimerExistsHandle (Variables|Config|GetExplosionDelayTimer)))
    (bind _returnvalue (Utilities|Time|SetTimerbyEvent (delegate Custom|Explode) (Variables|Config|Explosion|GetExplosionDelay)))
    (Variables|Config|SetExplosionDelayTimer _returnvalue)
    (Class|MikeBlueprintFunctionLibrary|PlaySound (Variables|Config|Audio|GetAudio) (Variables|Config|Audio|GetTickingSound) 0.0 false (Math|Vector|MakeVector 0.0 0.0 0.0) 1.0 0 0.0 (Utilities|Name|MakeLiteralName "None"))))

(event Custom|Death
  (if (not (Game|IsActorBeingDestroyed))
    (Actor|DestroyActor)))

(event Custom|Explode
  (bind _self self)
  (bind _staticmesh (Variables|Config|Stats|GetStaticMesh))
  (bind _audio (Variables|Config|Audio|GetAudio))
  (Game|Damage|ApplyRadialDamage (Variables|Config|Explosion|GetDamage) (Transformation|GetActorLocation) (Variables|Config|Explosion|GetExplosionRange) (Variables|Config|Explosion|GetDamageType) 0 _self (AI|GetAIController _self) true (Variables|Config|Explosion|GetDamagePreventionChannels))
  (Rendering|SetVisibility _staticmesh false true)
  (Collision|SetCollisionEnabled _staticmesh "NoCollision")
  (Collision|SetCollisionEnabled (Variables|Config|Stats|GetDetectionRange) "NoCollision")
  (Components|Activation|Deactivate (Variables|Config|Stats|GetFloatingPawnMovement))
  (Class|MikeBlueprintFunctionLibrary|PlaySound _audio (Variables|Config|Audio|GetExplosionSound) 0.0 true (Transformation|GetActorLocation) 1.0 0 0.0 (Utilities|Name|MakeLiteralName "None"))
  (EventDispatchers|BindEventtoOnAudioFinished _audio (delegate Custom|Death)))

(event EventPossessed
  (params (NewController :type Controller%20Object%20Reference))
  (bind _asaic_mine (Utilities|Casting|CastToAIC_Mine NewController)
    (:then
      (bind _output_get (Variables|Config|SetAIController _asaic_mine))
      (Default|SetHoveringLocation _output_get (Transformation|GetActorLocation) (Variables|Config|Stats|GetHoveringHeight))
      (Default|SetExplosionRange _output_get (Variables|Config|Explosion|GetExplosionRange))
      (Variables|/Script/Engine.FloatingPawnMovement|SetMaxSpeed (Variables|Config|Stats|GetFloatingPawnMovement) (Variables|Config|Stats|GetHoveringSpeed))
      (if (Variables|Config|Stats|GetbUseDefaultDetectionRadius)
        (Components|Sphere|SetSphereRadius (Variables|Config|Stats|GetDetectionRange) (Variables|Config|Stats|GetDefaultDetectionRadius) true)))
    (:CastFailed
      (CallFunction|CustomPrintString "Invalid mine controller" true true "(R=0.000000,G=0.000000,B=1.000000,A=1.000000)" 2.0))))

(event EventUnpossessed
  (params (OldController :type Controller%20Object%20Reference))
  (Variables|Config|SetAIController 0))

(fn ConstructionScript)

(fn GetExplosionDelayTimerInfo
  (bind _explosiondelaytimer (Variables|Config|GetExplosionDelayTimer))
  (bind (_outtimeleft _outtimeelapsed _returnvalue) (Class|MikeBlueprintFunctionLibrary|IsTimerValid _explosiondelaytimer))
  (return _outtimeelapsed _outtimeleft _returnvalue))
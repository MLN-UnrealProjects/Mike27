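; AI security camera pawn that pans between waypoints in circular or ping-pong order and tracks targets spotted through sight-only perception.
; Two look-to components split the rotation, yaw on the bottom and pitch on the top, and the controller's focal point follows the bottom's facing.
; While chasing, it alerts predetermined guards, disables player sprint and lowers their acceleration.
; Active disablers attached to it, registered through top-mesh collisions, switch off vision and trigger shock particles.
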(event OnComponentHit(CameraTop)
  (params (HitComponent :type Primitive%20Component%20Object%20Reference) (OtherActor :type Actor%20Object%20Reference) (OtherComp :type Primitive%20Component%20Object%20Reference) (NormalImpulse :type Vector :default "0, 0, 0") (Hit :type Hit%20Result%20Structure%20%28by%20ref%29))
  ;[1 1 1] Disablers Management. TODO: usare trigger davanti a 'sensore' camera invece della mesh della camera per le collisioni con i disabler
  (CallFunction|TryAddAiDisabler OtherActor))

(event OnComponentBeginOverlap(CameraTop)
  (params (OverlappedComponent :type Primitive%20Component%20Object%20Reference) (OtherActor :type Actor%20Object%20Reference) (OtherComp :type Primitive%20Component%20Object%20Reference) (OtherBodyIndex :type Integer) (bFromSweep :type Boolean) (SweepResult :type Hit%20Result%20Structure%20%28by%20ref%29))
  ;[1 1 1] Disablers Management. TODO: usare trigger davanti a 'sensore' camera invece della mesh della camera per le collisioni con i disabler
  (CallFunction|TryAddAiDisabler OtherActor))

(event OnComponentEndOverlap(CameraTop)
  (params (OverlappedComponent :type Primitive%20Component%20Object%20Reference) (OtherActor :type Actor%20Object%20Reference) (OtherComp :type Primitive%20Component%20Object%20Reference) (OtherBodyIndex :type Integer))
  ;[1 1 1] Disablers Management. TODO: usare trigger davanti a 'sensore' camera invece della mesh della camera per le collisioni con i disabler
  (CallFunction|TryRemoveAiDisabler OtherActor))

(event OnComponentHit(CameraBottom)
  (params (HitComponent :type Primitive%20Component%20Object%20Reference) (OtherActor :type Actor%20Object%20Reference) (OtherComp :type Primitive%20Component%20Object%20Reference) (NormalImpulse :type Vector :default "0, 0, 0") (Hit :type Hit%20Result%20Structure%20%28by%20ref%29)))

(event OnComponentBeginOverlap(CameraBottom)
  (params (OverlappedComponent :type Primitive%20Component%20Object%20Reference) (OtherActor :type Actor%20Object%20Reference) (OtherComp :type Primitive%20Component%20Object%20Reference) (OtherBodyIndex :type Integer) (bFromSweep :type Boolean) (SweepResult :type Hit%20Result%20Structure%20%28by%20ref%29)))

(event OnComponentEndOverlap(CameraBottom)
  (params (OverlappedComponent :type Primitive%20Component%20Object%20Reference) (OtherActor :type Actor%20Object%20Reference) (OtherComp :type Primitive%20Component%20Object%20Reference) (OtherBodyIndex :type Integer)))

(event Custom|Patrol
  (params (DeltaTime :type Float%20%28single-precision%29))
  ;[1 1 1] Management of Patrol Wayponts
  (if (== (Utilities|Array|Length (Variables|Config|Stats|GetWaypointsCamera)) 0)
    (Utilities|FlowControl|DoOnce false
      (:Completed
        (CallFunction|CustomPrintString "Please setup the actor in scene for Wayponts of CameraAI" true true "(R=1.000000,G=0.000000,B=0.000000,A=1.000000)" 5.0)))
    (elif (Default|IsTargetFocused (Variables|Default|GetBP_LookToComponentBot))
      (if (Variables|Config|Stats|GetbCircularPatrolPattern)
        (Config|SetNextCircularWaypoint)
        (else
          (Config|SetNextPingPongWaypoint))))))

(event Custom|TryRemoveAiDisabler
  (params (Actor :type Actor%20Object%20Reference%20%28by%20ref%29))
  ;[1 1 1] Disablers Management. TODO: usare trigger davanti a 'sensore' camera invece della mesh della camera per le collisioni con i disabler
  (Utilities|Array|RemoveItem (Variables|Stats|GetDisablers) Actor))

(event Custom|ResetPatrol
  (bind _asbp_player_character (CallFunction|GetCurrentMikeCharacter))
  (bind _sprint (Variables|/Game/Mike27/Core/Characters/Player/BP_PlayerCharacter.BP_PlayerCharacter_C|GetSprint _asbp_player_character))
  ;[1 1 1] Update
  (Utilities|FlowControl|DoOnce false) ; enters at Reset
)

(event Custom|ResetPrintChaseDebug
  (bind _aicontroller_npc (Variables|Stats|GetAIController_NPC))
  (bind _target (Default|GetTarget _aicontroller_npc))
  ;[1 1 1] Update
  (Utilities|FlowControl|DoOnce false) ; enters at Reset
)

(event Custom|ResetPrintPatrolDebug
  (bind _bp_looktocomponentbot (Variables|Default|GetBP_LookToComponentBot))
  (bind _bp_looktocomponenttop (Variables|Default|GetBP_LookToComponentTop))
  (bind _waypointscamera (Variables|Config|Stats|GetWaypointsCamera))
  (bind _returnvalue (Utilities|Array|Length _waypointscamera))
  (bind _returnvalue_2 (> _returnvalue 0))
  ;[1 1 1] Update
  (Utilities|FlowControl|DoOnce false) ; enters at Reset
)

(event Custom|TryAddAiDisabler
  (params (Actor :type Actor%20Object%20Reference%20%28by%20ref%29))
  ;[1 1 1] Disablers Management. TODO: usare trigger davanti a 'sensore' camera invece della mesh della camera per le collisioni con i disabler
  (if (Utilities|DoesObjectImplementInterface Actor "/Game/Mike27/Characters/AI/Common/BPI_AiDisabler.BPI_AiDisabler_C")
    (Utilities|Array|AddUnique (Variables|Stats|GetDisablers) Actor)))

(event EventPossessed
  (params (NewController :type Controller%20Object%20Reference))
  ;[1 1 1] Initialization
  (Config|InitializationControllerSettings NewController)
  (Config|SetAISensing))

(event EventBeginPlay
  (bind _bp_looktocomponentbot (Variables|Default|GetBP_LookToComponentBot))
  (bind _bp_looktocomponenttop (Variables|Default|GetBP_LookToComponentTop))
  ;[1 1 1] Initialization
  (Config|SetCurrentWaypoint)
  (Variables|/Game/Mike27/Core/Behaviours/BP_LookToComponent.BP_LookToComponent_C|SetPreRotationOffset _bp_looktocomponentbot "0, 0, 0")
  (Default|SetRotationMask _bp_looktocomponentbot false false true)
  (Variables|/Game/Mike27/Core/Behaviours/BP_LookToComponent.BP_LookToComponent_C|SetPreRotationOffset _bp_looktocomponenttop (Variables|/Script/Engine.SceneComponent|GetRelativeRotation (Variables|Default|GetCameraTop)))
  (Default|SetRotationMask _bp_looktocomponenttop false true false))

(event EventTick
  (params (DeltaSeconds :type Float%20%28single-precision%29))
  (bind _asbp_player_character (CallFunction|GetCurrentMikeCharacter))
  (bind _bdisabled (Config|IsDisabled))
  (bind _aicontroller_npc (Variables|Stats|GetAIController_NPC))
  (bind _aicontroller_npc_2 (Variables|Stats|GetAIController_NPC))
  (bind _bp_looktocomponenttop (Variables|Default|GetBP_LookToComponentTop))
  (bind _bp_looktocomponentbot (Variables|Default|GetBP_LookToComponentBot))
  (bind _bp_looktocomponenttop_2 (Variables|Default|GetBP_LookToComponentTop))
  (bind _waypointscamera (Variables|Config|Stats|GetWaypointsCamera))
  (bind _returnvalue (Utilities|Array|Length _waypointscamera))
  (bind _target (Default|GetTarget _aicontroller_npc))
  (bind _target_2 (Default|GetTarget _aicontroller_npc_2))
  (bind _sprint (Variables|/Game/Mike27/Core/Characters/Player/BP_PlayerCharacter.BP_PlayerCharacter_C|GetSprint _asbp_player_character))
  (bind _returnvalue_2 (> _returnvalue 0))
  (bind _rootcomponent (Variables|/Script/Engine.Actor|GetRootComponent _target_2))
  ;[1 1 1] Update
  (Config|UpdatePositionController)
  (Default|SetDisabledVision (Variables|Stats|GetAIController_NPC) _bdisabled)
  (Components|Activation|SetActive (Variables|Default|GetPS_DisabledShock) _bdisabled false)
  (switch Utilities|FlowControl|Switch|SwitchonEGuardState (Default|GetGuardState (Variables|Stats|GetAIController_NPC))
    (:NewEnumerator1
      (Utilities|FlowControl|Sequence
        (:then_0
          (Utilities|FlowControl|DoOnce false
            (:Completed
              (CallFunction|ResetPrintChaseDebug)
              (Default|SetOwnerComponent _bp_looktocomponenttop_2 (select _returnvalue_2 (Variables|Default|GetCameraTop) 0))
              (Default|SetTarget _bp_looktocomponenttop_2)
              (Default|SetOwnerComponent _bp_looktocomponentbot (select _returnvalue_2 (Variables|Default|GetCameraBottom) 0))
              (Default|SetTarget _bp_looktocomponentbot)
              (if (Variables|Config|Debug|GetbEnableDebug)
                (CallFunction|CustomPrintString (Utilities|String|Append (Utilities|GetDisplayName self) " lost sight of target!") true true "(R=0.000000,G=0.000000,B=1.000000,A=1.000000)" (Variables|Config|Debug|GetDebugDuration))))))
        (:then_1
          (CallFunction|Patrol DeltaSeconds)
          (Utilities|FlowControl|DoOnce false
            (:Completed
              (Config|ClearFocusTargettoAIs)
              (Variables|Stats|SetNormalizedValue 0.0)
              (Utilities|IsValid _asbp_player_character
                (:Is%20Valid
                  (Variables|/Script/Engine.CharacterMovementComponent|SetMaxAcceleration (Variables|/Script/Engine.Character|GetCharacterMovement _asbp_player_character) (.MaxAcceleration (Class|SprintComponent|GetSavedMovementStats _sprint)))
                  (Class|SprintComponent|SetEnabled _sprint true))))))))
    (:NewEnumerator2
      (Utilities|FlowControl|Sequence
        (:then_0
          (CallFunction|ResetPatrol)
          (Config|AlertOtherAIs)
          (Utilities|IsValid _target_2
            (:Is%20Valid
              (Default|SetTarget (Variables|Default|GetBP_LookToComponentBot) _rootcomponent)
              (Default|SetOwnerComponent (Variables|Default|GetBP_LookToComponentBot) (Variables|Default|GetCameraBottom))
              (Default|SetTarget _bp_looktocomponenttop _rootcomponent)
              (Default|SetOwnerComponent _bp_looktocomponenttop (Variables|Default|GetCameraTop))
              (Variables|Stats|SetNormalizedValue (/ (+ DeltaSeconds (Variables|Stats|GetNormalizedValue)) 2.0))
              (bind _asbp_player_character_2 (Utilities|Casting|CastToBP_PlayerCharacter _target_2))
              (Class|SprintComponent|SetEnabled (Variables|/Game/Mike27/Core/Characters/Player/BP_PlayerCharacter.BP_PlayerCharacter_C|GetSprint _asbp_player_character_2) false)
              (Variables|/Script/Engine.CharacterMovementComponent|SetMaxAcceleration (Variables|/Script/Engine.Character|GetCharacterMovement _asbp_player_character_2) (Math|Float|Lerp (Class|CharacterMovementComponent|GetMaxAcceleration (Variables|/Script/Engine.Character|GetCharacterMovement _asbp_player_character_2)) (Variables|Config|Stats|GetMinAcceleration) (Math|Float|Clamp(Float) (Variables|Stats|GetNormalizedValue)))))
            (:Is%20Not%20Valid
              (Default|SetOwnerComponent (Variables|Default|GetBP_LookToComponentBot))
              (Default|SetOwnerComponent (Variables|Default|GetBP_LookToComponentTop)))))
        (:then_1
          (Utilities|FlowControl|DoOnce false
            (:Completed
              (CallFunction|ResetPrintPatrolDebug)
              (if (Variables|Config|Debug|GetbEnableDebug)
                (CallFunction|CustomPrintString (Utilities|String|Append (Utilities|GetDisplayName self) " found target! " (select (Utilities|IsValid _target) (Utilities|GetDisplayName _target) " NULL ACTOR")) true true "(R=0.000000,G=0.000000,B=1.000000,A=1.000000)" (Variables|Config|Debug|GetDebugDuration))))))))))

(fn ConstructionScript
  (bind _conelight (Variables|Default|GetConeLight))
  (bind _returnvalue (Rendering|Material|CreateDynamicMaterialInstance _conelight 0 (Rendering|Material|GetMaterial _conelight 0) "None" :!class /Script/Engine.PrimitiveComponent))
  (Rendering|Material|SetVectorParameterValue _returnvalue "Color" (Variables|Config|Light|GetColorLight) :!class /Script/Engine.MaterialInstanceDynamic))

(fn InitializationControllerSettings
  (params (AIController :type Controller%20Object%20Reference))
  (bind _asaic_camera (Utilities|Casting|CastToAIC_Camera AIController)
    (:then
      (bind _output_get (Variables|Stats|SetAIController_NPC _asaic_camera))
      (Default|SetAttackRange _output_get 0.0)
      (Default|SetChaseRange _output_get 5e+02)
      (Default|SetShrinkDetectionRange _output_get 0.0 1.0)
      (return))
    (:CastFailed
      (CallFunction|CustomPrintString "Cast failed" true true "(R=0.000000,G=0.000000,B=1.000000,A=1.000000)" 2.0))))

(fn SetAISensing
  (bind _asmike_aiperception_component (Utilities|Casting|CastToMikeAIPerceptionComponent (Class|AIController|GetAIPerceptionComponent (AI|GetAIController self)))
    (:then
      (bind _output_get (LocalVariables|SetAISensingComponent _asmike_aiperception_component))
      (Class|MikeAIPerceptionComponent|SetSightRange _output_get (Variables|Config|Stats|GetSightRadius))
      (Class|MikeAIPerceptionComponent|SetPeripheralAngleVision (LocalVariables|GetAISensingComponent) (Variables|Config|Stats|GetPeripheralAngleVision))
      (Class|MikeAIPerceptionComponent|SetHearRange (LocalVariables|GetAISensingComponent) 0.0)
      (return))
    (:CastFailed
      (CallFunction|CustomPrintString "Cast failed" true true "(R=0.000000,G=0.000000,B=1.000000,A=1.000000)" 2.0))))

(fn AlertOtherAIs
  (bind _aicontroller_npc (Variables|Stats|GetAIController_NPC))
  (bind _output_get (LocalVariables|SetFocusTarget (Default|GetTarget _aicontroller_npc)))
  (Utilities|IsValid _output_get
    (:Is%20Valid
      (LocalVariables|SetLocation (Transformation|GetActorLocation _output_get)))
    (:Is%20Not%20Valid
      (LocalVariables|SetLocation (Default|GetLastSeenLocation _aicontroller_npc))))
  (for _array_element (Variables|Config|Stats|GetAIToAlertPredetermined)
    (bind _asaic_guard (Utilities|Casting|CastToAIC_Guard (AI|GetAIController _array_element)))
    (Utilities|IsValid (LocalVariables|GetFocusTarget)
      (:Is%20Valid
        (Default|SetSecondaryTarget _asaic_guard (LocalVariables|GetFocusTarget)))
      (:Is%20Not%20Valid
        (switch Utilities|FlowControl|Switch|SwitchonEGuardState (Default|GetGuardState _asaic_guard)
          (:NewEnumerator0
            _)
          (:NewEnumerator1
            _)
          (:NewEnumerator3
            _))
        (Default|SetLastSeenLocation _asaic_guard (LocalVariables|GetLocation) (Utilities|Enum|NotEqual(Enum) (Default|GetGuardState _asaic_guard) "NewEnumerator3")))))
  (return))

(fn UpdatePositionController
  (AI|SetFocalPoint (AI|GetAIController self) (+ (Transformation|GetWorldLocation (Variables|Default|GetCameraBottom)) (* (Math|Vector|GetForwardVector (Variables|Default|GetCameraBottom)) 1e+02))))

(fn ClearFocusTargettoAIs
  (for _array_element (Variables|Config|Stats|GetAIToAlertPredetermined)
    (bind _asaic_guard (Utilities|Casting|CastToAIC_Guard (AI|GetAIController _array_element)))
    (Default|SetSecondaryTarget _asaic_guard))
  (return))

(fn GetLastIndex
  (return (Utilities|Array|LastIndex (Variables|Config|Stats|GetWaypointsCamera))))

(fn IsDisabled
  (bind _disablers (Variables|Stats|GetDisablers))
  (if (== (Utilities|Array|Length _disablers) 0)
    (return false)
    (else
      (bind (_array_element _array_index) (Utilities|Array|ForEachLoopwithBreak _disablers :!label _label)
        (:LoopBody
          (Utilities|IsValid _array_element
            (:Is%20Valid
              (bind (_disablercollision _attachedtocomponent _bactivedisabler) (Class|BPIAiDisabler|GetDisablerInfo(Message) _array_element))
              (Utilities|IsValid _attachedtocomponent
                (:Is%20Valid
                  (if (== (Components|GetOwner _attachedtocomponent) self)
                    ;[1 1 1] Da gestire se posizione disabler è tale da poter disabilitare camera. Al primo disabler valido breakare (non c'è motivo di controllare gli altri)
                    (bind _output_get (LocalVariables|SetbIsDisabled _bactivedisabler))
                    (if _output_get
                      (goto _label Break))
                    (else
                      (Utilities|Array|Add (LocalVariables|GetIndexesToRemove) _array_index :!label _label_2))))
                (:Is%20Not%20Valid
                  (goto _label_2))))
            (:Is%20Not%20Valid
              (goto _label_2))))
        (:Completed
          (bind _arrayelement (Utilities|Array|ReverseforEachLoop (LocalVariables|GetIndexesToRemove))
            (:LoopBody
              (Utilities|Array|RemoveIndex (Variables|Stats|GetDisablers) _arrayelement))
            (:Completed
              (return (LocalVariables|GetbIsDisabled)))))))))

(fn SetNextPingPongWaypoint
  (bind _returnvalue (Config|GetLastIndex))
  (if (Variables|Config|Stats|GetbReversePatrol)
    (bind _output_get (LocalVariables|SetValue (- (Config|GetCurrentWaypoint) 1)))
    (Config|SetCurrentWaypoint _output_get)
    (if (< _output_get 0)
      (Config|SetCurrentWaypoint (Math|Integer|Clamp(Integer) 1 0 (Config|GetLastIndex)))
      (Variables|Config|Stats|SetbReversePatrol false)
      (return))
    (else
      (bind _output_get_2 (LocalVariables|SetValue (+ (Config|GetCurrentWaypoint) 1)))
      (Config|SetCurrentWaypoint _output_get_2)
      (if (> _output_get_2 _returnvalue)
        (Config|SetCurrentWaypoint (Math|Integer|Clamp(Integer) (- _returnvalue 1) 0 _returnvalue))
        (Variables|Config|Stats|SetbReversePatrol true)
        (return)))))

(fn SetNextCircularWaypoint
  (bind _currentwaypoint (Config|GetCurrentWaypoint))
  (Config|SetCurrentWaypoint (Class|MikeBlueprintFunctionLibrary|CircularClamp (select (Variables|Config|Stats|GetbReversePatrol) (- _currentwaypoint 1) (+ _currentwaypoint 1)) 0 (Config|GetLastIndex)))
  (return))

(fn SetCurrentWaypoint
  (params (CurrentWaypoint :type Integer))
  (bind _currentwaypoint (Config|GetCurrentWaypoint))
  (bind _output_get (LocalVariables|SetToSet (Math|Integer|Clamp(Integer) CurrentWaypoint 0 (Config|GetLastIndex))))
  (if (!= _output_get _currentwaypoint)
    (bind _output_get_2 (Variables|Stats|SetCurrentWaypoint _output_get))
    (Default|SetTargetLocation (Variables|Default|GetBP_LookToComponentBot) (Transformation|GetActorLocation (Utilities|Array|Get(acopy) (Variables|Config|Stats|GetWaypointsCamera) _output_get_2)) false)
    (Default|SetTargetLocation (Variables|Default|GetBP_LookToComponentTop) (Transformation|GetActorLocation (Utilities|Array|Get(acopy) (Variables|Config|Stats|GetWaypointsCamera) _output_get_2)) false)
    (return _output_get_2)
    (else
      (return _currentwaypoint))))

(fn GetCurrentWaypoint
  (return (Variables|Stats|GetCurrentWaypoint)))
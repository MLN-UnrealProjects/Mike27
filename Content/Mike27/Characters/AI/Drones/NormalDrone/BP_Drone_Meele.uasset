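; Melee drone pawn driven by an AIC_Guard controller, to which it passes perception, range and flight settings on possession.
; Tick polls guard state to update speed, spotlight and logo colour, look-at and hovering, and triggers attacks during Chase or Attack.
; After a wind-up, attacks proceed only if still in Attack state with a valid target.
; They fire arc lightning at it and apply timed radial damage ticks, gated by a cooldown.
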(event Custom|Attack
  (if (Variables|Config|Attack|GetbCanAttack)
    (Utilities|FlowControl|DoOnce false
      (:Completed
        (CallFunction|SetParticleSystem (Variables|Config|Particles|GetPrepareAttackEffect) true)
        (Utilities|Time|ClearandInvalidateTimerbyHandle (Variables|Stats|GetPreAttackDelayTimer))
        (bind _returnvalue (Utilities|Time|SetTimerbyEvent (delegate Custom|CheckAttackValidity) (Variables|Config|Attack|Stats|GetAttackDelay)))
        (Variables|Stats|SetPreAttackDelayTimer _returnvalue)
        (CallFunction|CustomPrintString "Attack commenced" true true "(R=0.000000,G=0.000000,B=1.000000,A=1.000000)" 2.0)))
    (else
      (CallFunction|ResetPreAttack))))

(event Custom|EnableAttack
  (CallFunction|ResetPreAttack)
  (Utilities|FlowControl|Gate false) ; enters at Open
)

(event Custom|OnCollisionsCheck
  (Config|AttackCollisionCheck))

(event Custom|OnStopAttack
  (Utilities|Time|ClearandInvalidateTimerbyHandle (Variables|Stats|GetAttackLifeHandle))
  (Utilities|Time|ClearandInvalidateTimerbyHandle (Variables|Stats|GetAttackCollisionCheckHandle))
  (Components|Activation|SetActive (Variables|Default|GetParticleSystem) false false))

(event Custom|StartArcing
  (params (Target :type Actor%20Object%20Reference) (bSuccessfull :type Boolean))
  (Default|SetDestinationActor (Variables|Default|GetBP_ArcLightningGenerator) Target)
  (Default|StartArcing (Variables|Default|GetBP_ArcLightningGenerator)))

(event Custom|DisableAttack
  (Utilities|FlowControl|Gate false) ; enters at Close
)

(event Custom|PerformAttack
  (Utilities|FlowControl|Gate false
    (:Exit
      (CallFunction|SetParticleSystem (Variables|Config|Particles|GetAttackEffect) true)
      (Config|Attack|RestartAttackCooldown "EnableAttack")
      (CallFunction|AttackLogic)
      (Default|CallOnAttack (Default|GetTarget (Variables|Stats|GetAiController)) true)
      (CallFunction|CustomPrintString "Attack performed" true true "(R=0.000000,G=0.000000,B=1.000000,A=1.000000)" 2.0))))

(event Custom|ResetPreAttack
  (CallFunction|OnStopAttack)
  (Utilities|Time|ClearandInvalidateTimerbyHandle (Variables|Stats|GetPreAttackDelayTimer))
  (CallFunction|ResetAttack)
  (CallFunction|CustomPrintString "Attack resetted" true true "(R=0.000000,G=0.000000,B=1.000000,A=1.000000)" 2.0))

(event Custom|ResetAttack
  (Utilities|FlowControl|DoOnce false) ; enters at Reset
)

(event Custom|CheckAttackValidity
  (if (Utilities|IsValid (Default|GetTarget (Variables|Stats|GetAiController)))
    (if (Utilities|Enum|Equal(Enum) "NewEnumerator4" (Default|GetGuardState (Variables|Stats|GetAiController)))
      (CallFunction|PerformAttack)
      (else
        (CallFunction|ResetPreAttack :!label _label)))
    (else
      (goto _label))))

(event Custom|AttackLogic
  (Utilities|Time|ClearandInvalidateTimerbyHandle (Variables|Stats|GetAttackCollisionCheckHandle))
  (bind _returnvalue (Utilities|Time|SetTimerbyEvent (delegate Custom|OnCollisionsCheck) (Variables|Config|Attack|Stats|GetAttackCollisionCheckIntervall) true))
  (Variables|Stats|SetAttackCollisionCheckHandle _returnvalue)
  (Utilities|Time|ClearandInvalidateTimerbyHandle (Variables|Stats|GetAttackLifeHandle))
  (bind _returnvalue_2 (Utilities|Time|SetTimerbyEvent (delegate Custom|OnStopAttack) (Variables|Config|Attack|Stats|GetAttackDuration)))
  (Variables|Stats|SetAttackLifeHandle _returnvalue_2))

(event Custom|SetParticleSystem
  (params (System :type Particle%20System%20Object%20Reference) (bEnable :type Boolean))
  (bind _particlesystem (Variables|Default|GetParticleSystem))
  (Components|Activation|SetActive _particlesystem false false)
  (Effects|Components|ParticleSystem|SetTemplate _particlesystem System)
  (Components|Activation|SetActive _particlesystem bEnable false))

(event EventUnpossessed
  (params (OldController :type Controller%20Object%20Reference))
  (Variables|Stats|SetAiController 0))

(event EventPossessed
  (params (NewController :type Controller%20Object%20Reference))
  ;[1 1 1] ConeLight for visual reference of the AI perception sight
  (bind _asaic_guard (Utilities|Casting|CastToAIC_Guard NewController)
    (:then
      (Variables|Stats|SetAiController _asaic_guard)
      (CallFunction|Possessed)
      (Rendering|Components|Light|SetLightColor (Variables|Default|GetSpotLight) (Variables|Config|Light|GetPatrolColor) true))
    (:CastFailed
      (CallFunction|CustomPrintString (Utilities|String|Append (Utilities|GetDisplayName self) " is not possessed by a valid controller") true true "(R=0.000000,G=0.000000,B=1.000000,A=1.000000)" 2.0))))

(event EventTick
  (params (DeltaSeconds :type Float%20%28single-precision%29))
  (bind _returnvalue (Transformation|GetVelocity))
  (bind _chasing_attackingcolor (Variables|Config|Light|GetChasing/AttackingColor))
  (bind _patrolcolor (Variables|Config|Light|GetPatrolColor))
  (bind _aicontroller (Variables|Stats|GetAiController))
  (bind _patrolspeed (Variables|Config|Stats|GetPatrolSpeed))
  (bind _aicontroller_2 (Variables|Stats|GetAiController))
  (bind _bp_looktocomponent (Variables|Default|GetBP_LookToComponent))
  (bind _midlogo (Variables|Stats|GetMIDLogo))
  (bind _state (Default|GetGuardState _aicontroller_2))
  (bind _state_2 (Default|GetGuardState _aicontroller))
  (bind _target (Default|GetTarget _aicontroller_2))
  ;[1 1 1] Light changing by perception Update
  (if (Utilities|Enum|NotEqual(Enum) _state_2 (Variables|Stats|GetPreviousGuardState))
    (Default|CallOnStateChange (Variables|Stats|GetPreviousGuardState) _state_2)
    (if (Variables|Config|Debug|GetbEnableDebug)
      (Config|Debug|ChangeStatePrint (Variables|Stats|GetPreviousGuardState) _state_2))
    (bind _output_get (Variables|Stats|SetPreviousGuardState _state_2))
    (if (Utilities|Enum|Equal(Enum) _output_get "NewEnumerator4")
      (CallFunction|Attack))
    (Variables|/Script/Engine.FloatingPawnMovement|SetMaxSpeed (Variables|Default|GetFloatingPawnMovement) (Utilities|Select :Index _output_get :NewEnumerator0 _patrolspeed :NewEnumerator1 _patrolspeed :NewEnumerator2 (Variables|Config|Stats|GetChaseSpeed) :NewEnumerator3 (Variables|Config|Stats|GetSuspicionSpeed) :NewEnumerator4 (Variables|Config|Stats|GetAttackSpeed)))
    (Utilities|IsValid _midlogo
      (:Is%20Valid
        (Rendering|Material|SetVectorParameterValue _midlogo "EmissiveColor" (Utilities|Select :Index _output_get :NewEnumerator0 _patrolcolor :NewEnumerator1 _patrolcolor :NewEnumerator2 _chasing_attackingcolor :NewEnumerator3 (Variables|Config|Light|GetSuspicionColor) :NewEnumerator4 _chasing_attackingcolor) :!class /Script/Engine.MaterialInstanceDynamic))
      (:Is%20Not%20Valid
        _))
    (Rendering|Components|Light|SetLightColor (Variables|Default|GetSpotLight) (Utilities|Select :Index _output_get :NewEnumerator0 _patrolcolor :NewEnumerator1 _patrolcolor :NewEnumerator2 _chasing_attackingcolor :NewEnumerator3 (Variables|Config|Light|GetSuspicionColor) :NewEnumerator4 _chasing_attackingcolor) true)
    (else
      (switch Utilities|FlowControl|Switch|SwitchonEGuardState _state
        (:NewEnumerator0
          (Default|SetTargetLocation _bp_looktocomponent (Math|Vector|MakeVector (.x _returnvalue) (.y _returnvalue) (select (Utilities|Enum|Equal(Enum) _state "NewEnumerator3") (.z _returnvalue) 0.0)) true :!label _label)
          (Default|SetSceneComponent (Variables|Default|GetBP_HoverComponent) (Variables|Default|GetStaticMesh)))
        (:NewEnumerator1
          (goto _label))
        (:NewEnumerator2
          (Utilities|IsValid _target :!label _label_2
            (:Is%20Valid
              (Default|SetTarget _bp_looktocomponent (Variables|/Script/Engine.Actor|GetRootComponent _target)))
            (:Is%20Not%20Valid
              _))
          (Default|SetSceneComponent (Variables|Default|GetBP_HoverComponent))
          (CallFunction|Attack))
        (:NewEnumerator3
          (goto _label))
        (:NewEnumerator4
          (goto _label_2))))))

(event EventBeginPlay
  (bind _bp_looktocomponent (Variables|Default|GetBP_LookToComponent))
  (Default|SetRotationMask _bp_looktocomponent false true true)
  (Default|SetData _bp_looktocomponent (Transformation|GetVelocity) 0 (Variables|Default|GetStaticMesh) true)
  (Default|SetSceneComponent (Variables|Default|GetBP_HoverComponent) (Variables|Default|GetStaticMesh))
  (Config|RemoveInvalidWaypoints)
  (EventDispatchers|BindEventtoOnAttack (delegate Custom|StartArcing)))

(event Custom|Possessed
  (bind _aicontroller (Variables|Stats|GetAiController))
  (bind _aicontroller_2 (Variables|Stats|GetAiController))
  (bind _mikeperception (Variables|/Script/Project.GuardAIController|GetMikePerception _aicontroller))
  ;[1 1 1] Set the SightRadius of the AI Sense SIght
  (Default|SetCanFly _aicontroller_2 (Variables|Config|GetbCanFly))
  (Default|SetShrinkDetectionRange _aicontroller_2 (Variables|Config|Perception|GetMinShrinkDetection) (Variables|Config|Perception|GetMaxShrinkDetection))
  (Default|SetAttackRange _aicontroller_2 (Variables|Config|Attack|GetAttackRange))
  (Default|SetChaseRange _aicontroller_2 (Variables|Config|Perception|GetChaseRange))
  (Default|SetNavigationData _aicontroller_2 (Variables|Config|Perception|GetNavigationData))
  (Class|MikeAIPerceptionComponent|SetSightRange _mikeperception (Variables|Config|Perception|GetSightRadius))
  (Class|MikeAIPerceptionComponent|SetHearRange _mikeperception (Variables|Config|Perception|GetHearRange))
  (Class|MikeAIPerceptionComponent|SetPeripheralAngleVision _mikeperception (Variables|Config|Perception|GetAngleVisionAI)))

(fn ConstructionScript
  (bind _returnvalue (Rendering|Material|CreateDynamicMaterialInstance (Variables|Default|GetStaticMesh) 1 "/Game/Mike27/Characters/AI/Drones/NormalDrone/MI_CommonDrone_Logo.MI_CommonDrone_Logo" "None" :!class /Script/Engine.PrimitiveComponent))
  (Variables|Stats|SetMIDLogo _returnvalue))

(fn RestartAttackCooldown
  (params (EnableAttack :type String))
  (CallFunction|DisableAttack)
  (Utilities|Time|ClearandInvalidateTimerbyHandle (Variables|Stats|GetAttackTimerHandle))
  (bind _returnvalue (Utilities|Time|SetTimerbyFunctionName self EnableAttack (Variables|Config|Attack|Stats|GetAttackCooldown)))
  (Variables|Stats|SetAttackTimerHandle _returnvalue)
  (return))

(fn ChangeStatePrint
  (params (PreviousState :type EGuardState%20Enum :default "NewEnumerator0") (NewState :type EGuardState%20Enum :default "NewEnumerator0"))
  (bind _returnvalue (Math|DateTime|Now))
  (CallFunction|CustomPrintString (Utilities|String|Append "AI instance: " (Utilities|GetDisplayName self) " changed its state from " (Utilities|String|EnumtoString PreviousState) " to " (Utilities|String|EnumtoString NewState) " at time: " (Utilities|String|Append (Utilities|String|ToString(Integer) (.hour _returnvalue)) ":" (Utilities|String|ToString(Integer) (.minute _returnvalue)) ":" (Utilities|String|ToString(Integer) (.second _returnvalue)) ":" (Utilities|String|ToString(Integer) (.millisecond _returnvalue)))) true true "(R=0.000000,G=0.000000,B=1.000000,A=1.000000)" (Variables|Config|Debug|GetDebugDuration))
  (return))

(fn IsPlayerVisible
  (return (Default|IsPlayerVisible (Variables|Stats|GetAiController))))

(fn GetGuardState
  (bind _aicontroller (Variables|Stats|GetAiController))
  (Utilities|IsValid _aicontroller
    (:Is%20Valid
      (return (Default|GetGuardState _aicontroller)))
    (:Is%20Not%20Valid
      (return "NewEnumerator0"))))

(fn GetCurrentController
  (return (Variables|Stats|GetAiController)))

(fn RemoveInvalidWaypoints
  (bind (_arrayindex _arrayelement) (Utilities|Array|ReverseforEachLoop (Variables|Config|Patrol|GetWaypoints))
    (:LoopBody
      (Utilities|IsValid _arrayelement
        (:Is%20Not%20Valid
          (Utilities|Array|Add (LocalVariables|GetIndexes) _arrayindex))))
    (:Completed
      (for _array_element (LocalVariables|GetIndexes)
        (Utilities|Array|RemoveIndex (Variables|Config|Patrol|GetWaypoints) _array_element))
      (return))))

(fn AttackCollisionCheck
  (Game|Damage|ApplyRadialDamage (* (Variables|Config|Attack|Stats|GetAttackCollisionCheckIntervall) (Variables|Config|Attack|Stats|GetAttackDamage)) (Transformation|GetWorldLocation (Variables|Default|GetParticleSystem)) (Variables|Config|Attack|GetAttackRange) (Variables|Config|Attack|Stats|GetDamageType) 0 self (Config|GetCurrentController) true "ECC_Camera")
  (return))

(fn GetRotationtoTarget
  (params (WorldStart :type Vector))
  (bind _controller (Config|GetCurrentController))
  (bind _target (Default|GetTarget _controller))
  (bind (_center _extents _returnvalue) (Class|MikeBlueprintFunctionLibrary|GetActorBoundsCenter _target true))
  (Utilities|IsValid _controller
    (:Is%20Valid
      (Utilities|IsValid _target
        (:Is%20Valid
          (if _returnvalue
            (return (Math|Rotator|FindLookatRotation WorldStart _center) true)
            (else
              _)))
        (:Is%20Not%20Valid
          _)))
    (:Is%20Not%20Valid
      _))
  (return "0, 0, 0" false))

(fn GetWaypointData
  (params (bRemoveInvalidWaypoints :type Boolean))
  (if bRemoveInvalidWaypoints
    (Config|RemoveInvalidWaypoints))
  (return (Variables|Config|Patrol|GetbSelectRandomWaypoints) (Variables|Config|Patrol|GetbForceRandomWaypoints) (Variables|Config|Patrol|GetStartingWaypoint) (Variables|Config|Patrol|GetWaypoints)))
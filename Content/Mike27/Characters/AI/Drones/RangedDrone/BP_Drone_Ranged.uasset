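; Ranged AI drone, a child Blueprint that fires its gun component when told to attack and able to.
; Tick calls reload whenever the gun reports a particular state.
; Focus rotation points from the mesh toward the target.
; Hover audio starts on BeginPlay and, once the first sound's duration has passed, switches a LoopSound parameter to avoid a pop when looping.
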(event OnAudioPlaybackPercent(HoverAudio)
  (params (PlayingSoundWave :type Sound%20Wave%20Object%20Reference) (PlaybackPercent :type Float%20%28single-precision%29))
  ;[1 1 1] Change sound to play for avoid pop sound on loop
  (Utilities|FlowControl|DoOnce false
    (:Completed
      (Utilities|FlowControl|Delay (Variables|/Script/Engine.SoundBase|GetDuration PlayingSoundWave))
      (Effects|Components|ParticleSystem|SetIntParameter (Variables|Default|GetHoverAudio) "LoopSound" 1))))

(event EventAttack
  (if (Variables|Default|GetbCanAttack)
    (Default|Fire (Variables|Default|GetBP_GunComponent))))

(event EventBeginPlay
  (|CallParentFunction)
  (Config|SetAudioInit))

(event EventTick
  (params (DeltaSeconds :type Float%20%28single-precision%29))
  (|CallParentFunction DeltaSeconds)
  (if (Utilities|Enum|Equal(Enum) (Default|GetCurrentState (Variables|Default|GetBP_GunComponent)) "NewEnumerator0")
    (Default|Reload (Variables|Default|GetBP_GunComponent))))

(fn ConstructionScript)

(fn GetFocusLocation
  (return (.Rotation (CallFunction|GetRotationtoTarget (Transformation|GetWorldLocation (Variables|Default|GetStaticMesh))))))

(fn SetAudioInit
  (bind _hoveraudio (Variables|Default|GetHoverAudio))
  (Components|Activation|SetActive _hoveraudio true false)
  (Effects|Components|ParticleSystem|SetIntParameter _hoveraudio "LoopSound" 0)
  (return))